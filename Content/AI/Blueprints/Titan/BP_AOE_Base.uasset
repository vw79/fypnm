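; BP_AOE_Base is an area-of-effect base Blueprint that reports pawns within a radius when triggered.
; Trigger runs a sphere overlap, optionally ignoring the instigator, then fires the OnAOEOverlapActor dispatcher and prints the name of each hit.
; The center looks up the BP_Titan RightFoot bone name but queries it on its own DefaultSceneRoot rather than the Titan's mesh.
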(event Custom|Spawn%20Sphere
  ;[1 1 1] Spawn and Draw Debug Sphere
  (bind _returnvalue (Actor|GetActorOfClass "/Game/AI/Blueprints/Titan/BP_Titan.BP_Titan_C"))
  (bind _outactors (Collision|SphereOverlapActors (Transformation|GetSocketLocation (Variables|Default|GetDefaultSceneRoot) (Class|SkinnedMeshComponent|GetSocketBoneName (Variables|/Script/Engine.Character|GetMesh _returnvalue) "RightFoot")) (Variables|Default|GetRadius) (Utilities|Array|MakeArray "ObjectTypeQuery3") 0 (select (Variables|Default|GetIgnore%20Instigator) (Utilities|Array|MakeArray (Game|GetInstigator)) 0)))
  (for _array_element _outactors
    (Default|CallOnAOEOverlapActor _array_element)
    (Development|PrintString (Utilities|GetDisplayName _array_element))))

(event Custom|Trigger
  (CallFunction|SpawnSphere))

(fn ConstructionScript)