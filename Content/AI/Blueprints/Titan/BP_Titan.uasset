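; BP_Titan is a boss enemy character with stomp and lightning strike attacks, delegated to its attacks component.
; Damage events from BPC_DamageSystem reveal and update the HUD boss health bar, and the first hit switches the AI controller to attacking the player.
; Death stops movement and AI logic, plays a montage, then after a delay hides the bar and destroys the actor.
; It also supplies movement speeds and ideal combat ranges.
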(event OnDamageResponse(BPC_DamageSystem)
  (params (DamageResponse :type E_DamageResponse%20Enum :default "NewEnumerator0"))
  (bind _bpc_damagesystem (Variables|Default|GetBPC_DamageSystem))
  ;[0.8194 1 0] - Titan's Health UI spawns when taking damage
  ; - Titan's Health is updated when taking damage
  (Utilities|FlowControl|Sequence
    (:then_0
      (Utilities|FlowControl|DoOnce false
        (:Completed
          (bind _asbp_mccontroller (Utilities|Casting|CastToBP_MCController (Game|GetPlayerController 0)))
          (Widget|SetVisibility (Variables|/Game/Widgets/AWB/AWB_HUD.AWB_HUD_C|GetWBP_BossHealth (Variables|/Game/Blueprints/BP_MCController.BP_MCController_C|GetHUDRef _asbp_mccontroller)) "Visible"))))
    (:then_1
      (Utilities|FlowControl|DoOnce false
        (:Completed
          (Default|SetStateasAttacking (Variables|Default|GetAIC%20Demon%20REF) (Game|GetPlayerCharacter 0)))))
    (:then_2
      (Default|UpdateHealthPercentage (Variables|/Game/Widgets/AWB/AWB_HUD.AWB_HUD_C|GetWBP_BossHealth (Variables|/Game/Blueprints/BP_MCController.BP_MCController_C|GetHUDRef _asbp_mccontroller)) (Variables|/Game/Blueprints/Health_Damage_System/BPC_DamageSystem.BPC_DamageSystem_C|GetHealth _bpc_damagesystem) (Variables|/Game/Blueprints/Health_Damage_System/BPC_DamageSystem.BPC_DamageSystem_C|GetMaxHealth _bpc_damagesystem)))))

(event OnDeath(BPC_DamageSystem)
  (bind _aic_demon_ref (Variables|Default|GetAIC%20Demon%20REF))
  ;[1 0 0.01116] - Titan Death
  ; - Health UI Disappears after Titan is Dead
  (Components|Movement|StopMovementImmediately (Variables|Character|GetCharacterMovement))
  (AI|Logic|StopLogic (Variables|/Script/AIModule.AIController|GetBrainComponent (Variables|Default|GetAIC%20Demon%20REF)) "Titan is Dead")
  (Default|SetStateasDead _aic_demon_ref)
  (Animation|Montage|PlayMontage (Variables|Character|GetMesh) "/Game/AI/Animations/Animation_Sequence/Titan/AM_TitanDeath.AM_TitanDeath"
    (:then
      (AI|ClearFocus _aic_demon_ref)
      (Utilities|FlowControl|Delay 9.0)
      (Widget|SetVisibility (Variables|/Game/Widgets/AWB/AWB_HUD.AWB_HUD_C|GetWBP_BossHealth (Variables|/Game/Blueprints/BP_MCController.BP_MCController_C|GetHUDRef (stale OnDamageResponse(BPC_DamageSystem) _asbp_mccontroller))) "Hidden")
      (Actor|DestroyActor))))

(event Custom|Stomp%20Attack
  (params (Attack%20Target :type Actor%20Object%20Reference))
  ;[1 0.2583 0] Titan Attacks
  (Default|StompAttack (Variables|Default|GetBPC_Attacks) (Utilities|Struct|MakeS_Attacks Attack%20Target "/Game/AI/Animations/Animation_Sequence/Titan/AM_Stomp.AM_Stomp" (Utilities|Struct|MakeS_DamageInfo 5e+01 "NewEnumerator1")) 1e+03))

(event Custom|Lightning%20Attack
  (params (Attack%20Target :type Actor%20Object%20Reference))
  ;[1 0.2583 0] Titan Attacks
  (Default|LightningStrike (Variables|Default|GetBPC_Attacks) Attack%20Target (Utilities|Struct|MakeS_Attacks Attack%20Target "/Game/AI/Animations/Animation_Sequence/Titan/AM_StrikeAttack.AM_StrikeAttack" "(Amount_2_1FD5280940A6D4C7899955B13C36E603=0.000000,DamageType_6_5ABD1F97450C100370FFCAB5D12B1BCA=NewEnumerator0,DamageResponse_9_BF76B78A43CE988448F2FCABF3B7B743=NewEnumerator0,IsInvincible_12_7DD98CA94A5CE9290CD73CA4265F1305=False,CanBeBlocked_14_79893AD94C36AE707485B9AF094DD051=False,CanBeParried_16_DF632D014328871EDFAB65A3016FECDB=False,ShouldForceInterrupt_18_A8663EA240844DEDFA020C8875502910=False)")))

(event EventBeginPlay
  (|CallParentFunction)
  (UserInterface|SetWidget (Variables|Default|GetHealth%20Bar%20Widget) 0))

(event Collision|EventActorBeginOverlap
  (params (OtherActor :type Actor%20Object%20Reference)))

(event EventTick
  (params (DeltaSeconds :type Float%20%28single-precision%29)))

(fn ConstructionScript
  (|CallParentFunction))

(fn SetMovementSpeed
  (params (Speed :type E_MovementSpeed%20Enum :default "NewEnumerator0"))
  (bind _output_get (Variables|/Script/Engine.CharacterMovementComponent|SetMaxWalkSpeed (Variables|Character|GetCharacterMovement) (Utilities|Select :Index Speed :NewEnumerator0 0.0 :NewEnumerator1 6e+02 :NewEnumerator3 0.0 :NewEnumerator2 0.0)))
  (return _output_get))

(fn GetIdealRange
  (return 1.5e+03 1e+03))

(fn GetMaxHealth
  (return 0.0))

(fn GetCurrentHealth
  (return 0.0))