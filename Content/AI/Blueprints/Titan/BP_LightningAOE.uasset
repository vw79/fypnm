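; BP_LightningAOE is a Titan AI area attack that calls down a delayed lightning strike at its target's ground position.
; On BeginPlay it snaps below AttackTarget with a downward visibility trace, whose end multiplies the target's Z by -1000 rather than offsetting it.
; It shows an indicator decal, waits briefly, then calls Trigger.
; If the decal is still valid, it removes it and plays lightning particles and a zap sound.
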(event Custom|Move%20to%20Ground
  (bind _attack_target (Variables|Default|GetAttack%20Target)
    (:then
      (bind (_outhit _returnvalue) (Collision|LineTraceByChannel (Transformation|GetActorLocation _attack_target) (* (Transformation|GetActorLocation _attack_target) "1.000000,1.000000,-1000.000000") "TraceTypeQuery1" false (Utilities|Array|MakeArray _attack_target) "None"))
      (if _returnvalue
        (Transformation|SetActorLocation (.Location (Collision|BreakHitResult _outhit)) false false)))
    (:else)))

(event EventBeginPlay
  (bind _returnvalue (Transformation|GetActorLocation))
  (|CallParentFunction)
  (CallFunction|MovetoGround)
  (bind _returnvalue_2 (Rendering|Decal|SpawnDecalatLocation "/Game/AI/Vefects/M_IndicatorDecal.M_IndicatorDecal" "25.000000,256.000000,256.000000" (Transformation|GetActorLocation) "-90.000000,0.000000,0.000000" 0.0))
  (Utilities|FlowControl|Delay 3.0)
  (CallFunction|Trigger)
  (Utilities|IsValid _returnvalue_2
    (:Is%20Valid
      (Components|DestroyComponent _returnvalue_2)
      (Effects|SpawnEmitteratLocation "/Game/AI/Vefects/FXVarietyPack/Particles/P_ky_lightning3.P_ky_lightning3" _returnvalue)
      (Audio|PlaySoundatLocation "/Game/AI/Vefects/Zap_VFX/Audio/SFX_Vefects_Zap_Big_01.SFX_Vefects_Zap_Big_01" _returnvalue "0, 0, 0" 1.0 1.0 0.0 0 0 0 0))))

(event Collision|EventActorBeginOverlap
  (params (OtherActor :type Actor%20Object%20Reference)))

(event EventTick
  (params (DeltaSeconds :type Float%20%28single-precision%29)))

(fn ConstructionScript
  (|CallParentFunction))