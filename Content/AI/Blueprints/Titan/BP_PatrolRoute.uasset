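; BP_PatrolRoute is a spline-based patrol route that supplies waypoints for AI movement.
; IncrementRoute steps RouteIndex by Direction along the PatrolRoute spline points, flipping Direction at the last and first points so the route runs back and forth rather than looping.
; GetSplinePointAsWorldPos returns the world position of the spline point at the current RouteIndex.
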(event Custom|IncrementRoute
  ;[1 1 1] -Increment the patrol route value
  ; - Condition Check to see if AI has reached the end
  ; - Patrol Route index will be reset and AI will move to route again
  (bind _output_get (Variables|Default|SetRouteIndex (+ (Variables|Default|GetRouteIndex) (Variables|Default|GetDirection))))
  (if (== _output_get (- (Spline|GetNumberOfSplinePoints (Variables|Default|GetPatrolRoute)) 1))
    (Variables|Default|SetDirection -1)
    (elif (== (Variables|Default|GetRouteIndex) 0)
      (Variables|Default|SetDirection 1))))

(fn ConstructionScript)

(fn GetSplinePointasWorldPos
  (return (Spline|GetLocationatSplinePoint (Variables|Default|GetPatrolRoute) (Variables|Default|GetRouteIndex) "World")))