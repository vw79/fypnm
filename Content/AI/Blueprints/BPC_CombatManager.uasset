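; BPC_CombatManager is a combat manager component that limits how many attackers can engage an AttackTarget at once.
; On BeginPlay it caches the maximum attacker count by querying the target through a GAS-named message.
; HandleAttackRequest ignores requests from the target itself, adding others to Attackers while slots remain or to WaitingAttackers otherwise.
; Each requester then receives an attack or wait message carrying the target.
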(event EventBeginPlay
  (bind _value (Class|BPIGAS|GASGetMaxAttackersCount(Message) (Variables|Default|GetAttackTarget)))
  (Variables|Default|SetMax%20Attackers%20Count _value))

(fn HandleAttackRequest
  (params (Attacker :type Actor%20Object%20Reference))
  (bind _attacktarget (Variables|Default|GetAttackTarget))
  (if (!= Attacker (Variables|Default|GetAttackTarget))
    (if (< (Utilities|Array|Length (Variables|Default|GetAttackers)) (Variables|Default|GetMax%20Attackers%20Count))
      (Utilities|Array|AddUnique (Variables|Default|GetAttackers) Attacker)
      (Class|BPIDemon|Attack(Message) Attacker _attacktarget)
      (else
        (Utilities|Array|AddUnique (Variables|Default|GetWaitingAttackers) Attacker)
        (Class|BPIDemon|Wait(Message) Attacker _attacktarget)))))