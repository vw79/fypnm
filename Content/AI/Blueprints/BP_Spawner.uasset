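; BP_Spawner spawns AI demons at random points around the player character.
; BeginPlay starts a looping timer, its interval randomized once, that calls AdvancedSpawn to pick among three DemonClass entries through chained random-integer checks, re-rolled per branch, so some ticks spawn nothing.
; A spawn counter pauses spawning for a cooldown at its limit, then resets.
; An older timer-and-destroy spawn system remains disconnected, with SpawnEnemies left empty.
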(event Custom|Spawn%20Enemies
  ;[1 1 1] Spawn System 2
  ;
  ; - Demons spawn by a Timer
  ; - Timer Stops when Demon Amount reached limit
)

(event Custom|Advanced%20Spawn
  (bind _returnvalue (Math|Random|RandomIntegerinRange 0 100))
  (bind _returnvalue_2 (Game|GetPlayerCharacter 0))
  (bind _returnvalue_3 (Transformation|GetActorLocation _returnvalue_2))
  ;[1 1 1] Spawn System 2
  ;
  ; - Enemies Spawn on a timer
  ; - Spawner spawns different enemies based on random integer
  ; - Spawner has a cooldown when it reaches certain amount, then resets the amount
  (if (Variables|Default|GetcanSpawn)
    (bind _output_get (Variables|Default|SetSpawn%20Location (Math|Vector|MakeVector (+ (.x _returnvalue_3) (Math|Random|RandomFloatinRange -5e+02 5e+02)) (+ (.y _returnvalue_3) (Math|Random|RandomFloatinRange -5e+02 5e+02)) (.z _returnvalue_3))))
    (if (< _returnvalue 50)
      (AI|SpawnAIFromClass (Utilities|Array|Get(acopy) (Variables|Default|GetDemon%20Class)) 0 _output_get "0, 0, 0" false 0)
      (bind _output_get_2 (Variables|Default|SetDemon%20Amount (+ (Variables|Default|GetDemon%20Amount) 1) :!label _label))
      (if (== _output_get_2 10)
        (Variables|Default|SetcanSpawn false)
        (Utilities|FlowControl|Delay 5e+01)
        (Variables|Default|SetcanSpawn true)
        (Variables|Default|SetDemon%20Amount 0))
      (elif (and (>= _returnvalue 50) (< _returnvalue 75))
        (AI|SpawnAIFromClass (Utilities|Array|Get(acopy) (Variables|Default|GetDemon%20Class) 1) 0 _output_get "0, 0, 0" false 0)
        (goto _label)
        (elif (>= _returnvalue 75)
          (AI|SpawnAIFromClass (Utilities|Array|Get(acopy) (Variables|Default|GetDemon%20Class) 2) 0 _output_get "0, 0, 0" false 0)
          (goto _label))))))

(event EventBeginPlay
  ;[1 1 1] Spawn System 2
  ;
  ; - Enemies Spawn on a timer
  ; - Spawner spawns different enemies based on random integer
  ; - Spawner has a cooldown when it reaches certain amount, then resets the amount
  (Utilities|Time|SetTimerbyEvent (delegate Custom|Advanced%20Spawn) (Math|Random|RandomFloatinRange 2.0 5.0) true))

(fn ConstructionScript)