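; Spawn manager component that feeds queued demons into the world around the player.
; SpawnDemons starts a looping timer, its interval randomized once, that calls AdvancedSpawn.
; Each tick spawns the first class in GS_MCGameState's DemonList at a random reachable point near the player, then removes it, clearing CanSpawn once the list is empty.
; An unconnected older branch spawns fixed melee and shielder batches.
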(event Custom|Spawn%20Demons
  (Utilities|Time|SetTimerbyEvent (delegate Custom|Advanced%20Spawn) (Math|Random|RandomFloatinRange 1.0 3.0) true))

(event Custom|Advanced%20Spawn
  (bind _returnvalue (Game|GetPlayerCharacter 0))
  (bind _returnvalue_2 (Transformation|GetActorLocation _returnvalue))
  (bind _randomlocation (AI|Navigation|GetRandomReachablePointinRadius _returnvalue_2 5e+02 0 0))
  (if (Variables|Default|GetCan%20Spawn)
    (bind _output_get (Variables|Default|SetSpawn%20Location (Math|Vector|MakeVector (.x _randomlocation) (.y _randomlocation) (.z _randomlocation))))
    (bind _asgs_mcgame_state (Utilities|Casting|CastToGS_MCGameState (Game|GetGameState)))
    (if (> (Utilities|Array|Length (Variables|/Game/GAS/GS_MCGameState.GS_MCGameState_C|GetDemon%20List _asgs_mcgame_state)) 0)
      (Game|SpawnActorfromClass (Utilities|Array|Get(acopy) (Variables|/Game/GAS/GS_MCGameState.GS_MCGameState_C|GetDemon%20List _asgs_mcgame_state)) (Math|Transform|MakeTransform _output_get "0, 0, 0" "1.000000,1.000000,1.000000") "Undefined" "MultiplyWithRoot" 0 0)
      (Utilities|Array|RemoveIndex (Variables|/Game/GAS/GS_MCGameState.GS_MCGameState_C|GetDemon%20List _asgs_mcgame_state))
      (else
        (Variables|Default|SetCan%20Spawn false)))))