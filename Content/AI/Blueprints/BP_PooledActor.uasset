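; BP_PooledActor is an actor built for object pooling, toggled between in-use and dormant states instead of being spawned and destroyed.
; SetInUse switches collision, visibility and tick together, and BeginPlay starts the actor dormant.
; Activation clears any previous timer and starts a new one for SpawnTime, after which ReturnToPool calls SetInUse(false) to deactivate it again.
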(event Custom|Set%20In%20Use
  (params (InUse :type Boolean))
  (Variables|Default|SetInUse InUse)
  (Collision|SetActorEnableCollision InUse)
  (Rendering|SetActorHiddenInGame (not InUse))
  (Actor|Tick|SetActorTickEnabled InUse)
  (Utilities|Time|ClearandInvalidateTimerbyHandle (Variables|Default|GetTimer%20Value))
  (if InUse
    (bind _returnvalue (Utilities|Time|SetTimerbyEvent (delegate Custom|Return%20to%20Pool) (Variables|Default|GetSpawn%20Time)))
    (Variables|Default|SetTimer%20Value _returnvalue)))

(event Custom|Return%20to%20Pool
  (CallFunction|SetinUse false))

(event EventBeginPlay
  (CallFunction|SetinUse false))

(fn ConstructionScript)