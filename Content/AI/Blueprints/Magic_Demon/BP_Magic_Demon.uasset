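; Magic Demon AI enemy that attacks at range with magic projectiles.
; Attack plays a montage whose notify calls the BPCAttacks magic attack from the right-hand socket, then signals FinishAttacking on completion.
; A separate MagicAttack event spawns BP_Projectile with the demon as owner.
; It supplies per-state movement speeds and attack/defend radii, and delegates incoming damage to BPCDamageSystem.
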(event Custom|Magic%20Attack
  (params (Spawn%20Transform :type Transform) (Damage%20Info :type S%20Damage%20Info%20Structure))
  (Game|SpawnActorfromClass "/Game/AI/Blueprints/Magic_Demon/BP_Projectile.BP_Projectile_C" Spawn%20Transform "Undefined" "MultiplyWithRoot" self 0))

(event EventBeginPlay
  (|CallParentFunction) ; This node is disabled and will not be called.\nDrag off pins to build functionality.
)

(event Collision|EventActorBeginOverlap
  (params (OtherActor :type Actor%20Object%20Reference)))

(event EventTick
  (params (DeltaSeconds :type Float%20%28single-precision%29)))

(event EventAttack
  (params (Attack%20Target :type Actor%20Object%20Reference))
  (bind _notifyname (Animation|Montage|PlayMontage (Variables|Character|GetMesh) (Variables|Default|GetAttack_Animation))
    (:OnCompleted
      (CallFunction|FinishAttacking Attack%20Target))
    (:OnNotifyBegin
      (switch name _notifyname
        (:Cast
          (Default|MagicAttack :self (Variables|Default|GetBPC_Attacks) :Spawn%20Transform (Math|Transform|MakeTransform (Transformation|GetSocketLocation (Variables|Character|GetMesh) "RightHand") "0, 0, 0" "1.000000,1.000000,1.000000") :Target Attack%20Target))))))

(fn ConstructionScript
  (|CallParentFunction))

(fn SetMovementSpeed
  (params (Speed :type E_MovementSpeed%20Enum :default "NewEnumerator0"))
  (return (Utilities|Select :Index Speed :NewEnumerator0 0.0 :NewEnumerator1 1.5e+02 :NewEnumerator3 2.5e+02 :NewEnumerator2 5e+02)))

(fn GetIdealRange
  (return 5e+02 7e+02))

(fn TakeDamage
  (params (DamageInfo :type S%20Damage%20Info%20Structure))
  (bind _wasdamaged (Default|TakeDamage (Variables|Default|GetBPC_DamageSystem) DamageInfo))
  (return _wasdamaged))