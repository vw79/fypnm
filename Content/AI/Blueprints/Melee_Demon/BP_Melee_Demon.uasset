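; Melee demon enemy character that registers with the combat manager on spawn and fights with claw slash, dual slash and 360 attacks.
; Attack, damage and token logic go through components, while the AI controller receives attack, wait, stun and dead states.
; Hits play directional montages or hold it airborne for air combos, flagging it executable at low health.
; Death ragdolls it, returns reserved tokens, updates player lock-on, then dissolves and destroys it.
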(event Custom|360%20Attack
  (params (Attack%20Target :type Actor%20Object%20Reference))
  ;[0 0.0585 1] AI Attack System
  (Default|360Attack (Variables|Default|GetBPC_Attacks) (Utilities|Struct|MakeS_Attacks Attack%20Target 0 (Utilities|Struct|MakeS_DamageInfo 1e+01 "NewEnumerator1"))))

(event Custom|Claw%20Slash
  (params (Attack%20Target :type Actor%20Object%20Reference))
  ;[0 0.0585 1] AI Attack System
  (Default|ClawSlash (Variables|Default|GetBPC_Attacks) (Utilities|Struct|MakeS_Attacks Attack%20Target "/Game/Animation/MeleeDemon/AM_Claw_Slash.AM_Claw_Slash" (Utilities|Struct|MakeS_DamageInfo 1e+01 "NewEnumerator1"))))

(event Custom|DamageResponse
  (params (DamageResponse :type E_DamageResponse%20Enum :default "NewEnumerator0") (HitDirectiob :type E_DirectionalHit%20Enum :default "NewEnumerator0"))
  (bind _playercontrollerref (Variables|Default|GetPlayerControllerRef))
  ;[1 0.8259 0] - AI Has a Hit Reaction to Damage
  (Utilities|FlowControl|Sequence
    (:then_0
      (Utilities|FlowControl|DoOnce false
        (:Completed
          (bind _returnvalue (Actor|GetActorOfClass "/Game/AI/Blueprints/Titan/BP_Titan.BP_Titan_C"))
          (if (or (Collision|IsOverlappingActor (Variables|Default|GetCapsuleComponent) _returnvalue :!class /Script/Engine.PrimitiveComponent) (Collision|IsOverlappingActor (Variables|Character|GetMesh) _returnvalue :!class /Script/Engine.PrimitiveComponent))
            (Transformation|AddActorWorldOffset (Math|Vector|MakeVector 0.0 0.0 (+ (.z (Transformation|GetActorLocation)) 1e+02)))))))
    (:then_1
      _))
  (Niagara|SpawnSystematLocation "/Game/Roi/VFX/NS_EnemyBloodSplat.NS_EnemyBloodSplat" (Transformation|GetWorldLocation (Variables|Default|GetLock)))
  (Audio|PlaySound2D "/Game/SFX/SoundCue/SC_SlashHit.SC_SlashHit" 1.0 1.0 0.0 0 0)
  (if (> (Variables|/Game/Blueprints/Health_Damage_System/BPC_DamageSystem.BPC_DamageSystem_C|GetHealth (Variables|Default|GetBPC_DamageSystem)) 2e+01)
    _
    (else
      (Default|SetIndicationColor (Variables|Default|GetWbpLockOnRef) (Utilities|Struct|MakeSlateColor "(R=1.000000,G=0.006772,B=0.000000,A=1.000000)"))
      (Variables|/Game/Blueprints/Health_Damage_System/BPC_DamageSystem.BPC_DamageSystem_C|SetisExecutable (Variables|Default|GetBPC_DamageSystem) true)))
  (Components|Movement|StopMovementImmediately (Variables|Character|GetCharacterMovement))
  (Default|SetStateasStunned (Variables|Default|GetAIC%20Demon%20REF))
  (bind _aswbp_health_bar (Utilities|Casting|CastToWBP_HealthBar (UserInterface|GetWidget (Variables|Default|GetHealth%20Bar%20Widget))))
  (Default|DamageGlitch _aswbp_health_bar)
  (if (not (AI|Components|NavMovement|IsFalling (Variables|Character|GetCharacterMovement)))
    (Utilities|DirectionalHitAnimation HitDirectiob
      (:OnCompleted
        _)
      (:OnInterrupted
        _))
    (Utilities|FlowControl|Delay 2.0)
    (Default|SetStateasAttacking (Variables|Default|GetAIC%20Demon%20REF) (Game|GetPlayerCharacter 0))
    (else
      ;;[1 1 1] Air Attack Hit Reaction
      (Variables|Default|SetisStayAir true)
      (if (not (Variables|/Game/Blueprints/BP_MCController.BP_MCController_C|GetisSlam _playercontrollerref))
        (Transformation|SetRelativeLocation (Variables|Default|GetCapsuleComponent) (Transformation|GetWorldLocation (Variables|/Game/ThirdPerson/Blueprints/Player/BP_MC.BP_MC_C|GetAirAttack (Variables|/Game/Blueprints/BP_MCController.BP_MCController_C|GetPlayerCharacterRef _playercontrollerref))) false false)))))

(event Custom|Death
  (bind _mesh (Variables|Character|GetMesh))
  ;[1 0 0] AI Death Logic
  (Variables|Default|SetisStayAir false)
  (CallFunction|HandleDeathTargeting)
  (Physics|SetSimulatePhysics _mesh true)
  (Collision|SetCollisionEnabled _mesh "QueryAndPhysics")
  (AI|Logic|StopLogic (Variables|/Script/AIModule.AIController|GetBrainComponent (Variables|Default|GetAIC%20Demon%20REF)) "")
  (Default|SetStateasDead (Variables|Default|GetAIC%20Demon%20REF))
  (Utilities|FlowControl|Sequence
    (:then_0
      (Utilities|Array|Add (Variables|/Game/GAS/GS_MCGameState.GS_MCGameState_C|GetDemon%20List (Variables|Default|GetGameStateRef)) "BP_Melee_Demon_C")
      (Components|Activation|Deactivate (Variables|Default|GetHeavyIndicator))
      (Components|Activation|Deactivate (Variables|Default|GetParryIndicator)))
    (:then_1
      (bind _keys (Utilities|Map|Keys (Variables|Default|GetReserved%20Attack%20Tokens)))
      (for _array_element _keys
        (Class|BPIDamagable|ReturnAttackToken(Message) _array_element (.Value (Utilities|Map|Find (Variables|Default|GetReserved%20Attack%20Tokens) _array_element)))
        (Default|HandleDeath (Variables|Default|GetCombat%20Manager) self)))
    (:then_2
      (Utilities|Time|SetTimerbyEvent (delegate Custom|Dissolve%20Enemy) 2.0))))

(event Custom|Dissolve%20Enemy
  (bind _dissolve_particles (Variables|Default|GetDissolve%20Particles))
  ;[1 0 0] AI Death Logic
  (Audio|PlaySoundatLocation "/Game/SFX/Enemy/DemonDead.DemonDead" (Transformation|GetWorldLocation (Variables|Character|GetMesh)) "0, 0, 0" 1.0 1.0 0.0 "/Game/SFX/SoundCue/SA_Demon.SA_Demon" 0 0 0)
  (Components|Activation|Activate _dissolve_particles false)
  (bind _dissolve_amount (Timeline|Dissolve%20Timeline PlayFromStart)
    (:Update
      (Niagara|SetNiagaraVariable(Float) _dissolve_particles "Mask" _dissolve_amount)
      (Rendering|Material|SetScalarParameterValueonMaterials (Variables|Character|GetMesh) "Mask" _dissolve_amount))
    (:Finished
      (Components|Activation|Deactivate _dissolve_particles)
      (Audio|PlaySound2D "/Game/SFX/Enemy/DemonDead.DemonDead" 1.0 1.0 0.0 0 0)
      (Pawn|UnPossess (AI|GetAIController 0))
      (Actor|DestroyActor))))

(event Custom|Dual%20Claw%20Slash
  (params (Attack%20Target :type Actor%20Object%20Reference))
  ;[0 0.0585 1] AI Attack System
  (Default|DualClawSlash (Variables|Default|GetBPC_Attacks) (Utilities|Struct|MakeS_Attacks Attack%20Target "/Game/Animation/MeleeDemon/AM_Dual_Claw_Slash.AM_Dual_Claw_Slash" (Utilities|Struct|MakeS_DamageInfo 12.0 "NewEnumerator1"))))

(event Custom|Spawn%20Orb
  ;[1 0 0] AI Death Logic
  (Default|SpawnfromPool (Variables|Default|GetBPC_ObjectPool) (Math|Transform|MakeTransform (Transformation|GetActorLocation) "0, 0, 0" "1.000000,1.000000,1.000000")))

(event EventReturnAttackToken
  (params (Amount :type Integer))
  ;[0 0.0585 1] AI Attack System
  (Default|ReturnAttackToken (Variables|Default|GetBPC_DamageSystem) Amount))

(event EventOnLanded
  (params (Hit :type Hit%20Result%20Structure%20%28by%20ref%29))
  ;[1 1 1] Air Attack
  ;;[1 1 1] Reset Stay in Air
  (Variables|Default|SetisStayAir false)
  (Default|SetStateasAttacking (Variables|Default|GetAIC%20Demon%20REF) (Game|GetPlayerCharacter 0)))

(event EventSetIsInterruptible
  (params (Value :type Boolean))
  ;[1 0.8259 0] - AI Has a Hit Reaction to Damage
  (Variables|/Game/Blueprints/Health_Damage_System/BPC_DamageSystem.BPC_DamageSystem_C|SetisInterruptible (Variables|Default|GetBPC_DamageSystem) Value))

(event EventAATKLaunchEnemy
  (params (LaunchVelocity :type Vector :default "0, 0, 0") (XYOverride :type Boolean) (ZOverride :type Boolean))
  ;[1 1 1] Air Attack
  ;;[1 1 1] Interfaces
  (Character|LaunchCharacter LaunchVelocity XYOverride ZOverride)
  (Animation|PlayAnimMontage "/Game/Animation/MeleeDemon/AM_StayAir.AM_StayAir" 1.0 "None")
  (Variables|Default|SetisStayAir true)
  (Default|SetStateasStunned (Variables|Default|GetAIC%20Demon%20REF)))

(event EventWait
  (params (Attack%20Target :type Actor%20Object%20Reference))
  (Default|SetStateasWaiting (Variables|Default|GetAIC%20Demon%20REF) Attack%20Target))

(event EventBeginPlay
  (bind _zap_vfx (Variables|Default|GetZap%20VFX))
  (Utilities|FlowControl|Sequence
    (:then_0
      (|CallParentFunction))
    (:then_1
      (Components|Activation|Activate _zap_vfx false)
      (Audio|PlaySoundatLocation "/Game/AI/Vefects/Zap_VFX/Audio/SFX_Vefects_Zap_Big_02.SFX_Vefects_Zap_Big_02" (Transformation|GetActorLocation) "0, 0, 0" 1.0 1.0 0.0 0 0 0 0)
      (Utilities|FlowControl|Delay 1.0)
      (Components|Activation|Deactivate _zap_vfx))
    (:then_2
      (bind _returnvalue (Actor|GetActorOfClass "/Game/AI/Blueprints/BP_CombatManager.BP_CombatManager_C"))
      (bind _output_get (Variables|Default|SetCombat%20Manager _returnvalue))
      (Default|HandleAttackRequest _returnvalue self))))

(event EventActivateParryIndicator
  (params (IndicatorDuration :type Float%20%28double-precision%29))
  (bind _parryindicator (Variables|Default|GetParryIndicator))
  ;[1 1 1] Parry Indication
  (if (not (Variables|/Game/Blueprints/Health_Damage_System/BPC_DamageSystem.BPC_DamageSystem_C|GetisDead (Variables|Default|GetBPC_DamageSystem)))
    (Niagara|SetNiagaraVariable(Float) _parryindicator "Lifetime" IndicatorDuration)
    (Components|Activation|Activate _parryindicator false)))

(event EventAttack
  (params (Attack%20Target :type Actor%20Object%20Reference))
  (Default|SetStateasAttacking (Variables|Default|GetAIC%20Demon%20REF) Attack%20Target))

(event EventActivateHeavyIndicator
  (params (IndicatorDuration :type Float%20%28double-precision%29))
  (bind _heavyindicator (Variables|Default|GetHeavyIndicator))
  ;[1 1 1] Heavy Indication
  (if (not (Variables|/Game/Blueprints/Health_Damage_System/BPC_DamageSystem.BPC_DamageSystem_C|GetisDead (Variables|Default|GetBPC_DamageSystem)))
    (Niagara|SetNiagaraVariable(Float) _heavyindicator "Lifetime" IndicatorDuration)
    (Components|Activation|Activate _heavyindicator false)))

(fn ConstructionScript
  (bind _bpc_damagesystem (Variables|Default|GetBPC_DamageSystem))
  (EventDispatchers|BindEventtoOnDeath _bpc_damagesystem (EventDispatchers|CreateEvent :!event Custom|Death))
  (EventDispatchers|BindEventtoOnDamageResponse _bpc_damagesystem (EventDispatchers|CreateEvent :!event Custom|DamageResponse)))

(fn Heal
  (params (HealAmount :type Float%20%28double-precision%29))
  (return 0.0))

(fn ReserveAttackToken
  (params (Amount :type Integer))
  (bind _success (Default|ReserveAttackToken (Variables|Default|GetBPC_DamageSystem) Amount))
  (return _success))

(fn GetIdealRange
  (return 1e+02 5e+02))

(fn GetMaxHealth
  (return (Variables|/Game/Blueprints/Health_Damage_System/BPC_DamageSystem.BPC_DamageSystem_C|GetMaxHealth (Variables|Default|GetBPC_DamageSystem))))

(fn AATKGetEnemyCapsule
  (return (Variables|Default|GetCapsuleComponent)))

(fn GetEnemyCharacterMovement
  (return (Variables|Character|GetCharacterMovement)))

(fn HandleDeathTargeting
  (bind _playercontrollerref (Variables|Default|GetPlayerControllerRef))
  (bind _targetingsystemref (Variables|/Game/Blueprints/BP_MCController.BP_MCController_C|GetTargetingSystemRef _playercontrollerref))
  (Rendering|SetVisibility (Variables|Default|GetLock) false false)
  (if (Variables|/Game/Blueprints/Component/BPC_TargetingSystem.BPC_TargetingSystem_C|GetisHardLock _targetingsystemref)
    (Default|EndHardTarget _targetingsystemref)
    (Collision|SetCollisionResponsetoChannel (Variables|Default|GetCapsuleComponent) "ECC_Visibility" "ECR_Ignore" :!label _label)
    (Default|HardLockonTarget _targetingsystemref)
    (elif (Variables|/Game/Blueprints/Component/BPC_TargetingSystem.BPC_TargetingSystem_C|GetisSoftLock _targetingsystemref)
      (Default|EndSoftTarget _targetingsystemref)
      (goto _label))))

(fn GetCurrentHealth
  (return (Variables|/Game/Blueprints/Health_Damage_System/BPC_DamageSystem.BPC_DamageSystem_C|GetHealth (Variables|Default|GetBPC_DamageSystem))))

(fn SetMovementSpeed
  (params (Speed :type E_MovementSpeed%20Enum :default "NewEnumerator0"))
  (bind _output_get (Variables|/Script/Engine.CharacterMovementComponent|SetMaxWalkSpeed (Variables|Character|GetCharacterMovement) (Utilities|Select :Index Speed :NewEnumerator0 0.0 :NewEnumerator1 1.7e+02 :NewEnumerator3 1.7e+02 :NewEnumerator2 5e+02)))
  (return _output_get))

(fn GetDemonRef
  (return self (Variables|Default|GetBPC_DamageSystem)))

(fn GetTeamNumber
  (return (Variables|Default|GetTeam%20Number)))