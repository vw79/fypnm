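; Shielder demon enemy character driven by a behavior tree, with montage-based melee attacks and a launched-arc jump toward targets.
; The attack's Swing notify sphere-traces forward to deal damage.
; Damage component events stun it with a hit reaction, then resume attacking, or ragdoll and destroy it on death.
; At low health it roars once, pausing its AI to heal with ripple VFX while temporarily invincible.
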(event OnDamageResponse(BPC_DamageSystem)
  (params (DamageResponse :type E_DamageResponse%20Enum :default "NewEnumerator0"))
  (bind _bpc_damagesystem (Variables|Default|GetBPC_DamageSystem))
  (bind _bpc_damagesystem_2 (Variables|Default|GetBPC_DamageSystem))
  (bind _ripple_vfx (Variables|Default|GetRipple%20VFX))
  ;[1 0.8259 0] - AI Has a Hit Reaction to Damage
  ; - AI Heals when Health is below 30
  ; - Invincible for 2 seconds when healing then can take damage again
  (Components|Movement|StopMovementImmediately (Variables|Character|GetCharacterMovement))
  (Default|SetStateasStunned (Variables|Default|GetAIC%20Demon%20REF))
  (Animation|Montage|PlayMontage (Variables|Character|GetMesh) "/Game/AI/Animations/Animation_Sequence/Mutant/AM_Shielder_Hit.AM_Shielder_Hit"
    (:OnCompleted
      _)
    (:OnInterrupted
      _))
  (Default|SetStateasAttacking (Variables|Default|GetAIC%20Demon%20REF) (Game|GetPlayerCharacter 0))
  (if (<= (Variables|/Game/Blueprints/Health_Damage_System/BPC_DamageSystem.BPC_DamageSystem_C|GetHealth _bpc_damagesystem_2) 3e+01)
    (Variables|/Game/Blueprints/Health_Damage_System/BPC_DamageSystem.BPC_DamageSystem_C|SetisInterruptible _bpc_damagesystem_2 false)
    (Utilities|FlowControl|DoOnce false
      (:Completed
        (Animation|Montage|PlayMontage (Variables|Character|GetMesh) "/Game/AI/Animations/Animation_Sequence/Mutant/AM_Shielder_Roar.AM_Shielder_Roar"
          (:then
            (AI|Logic|StopLogic (Variables|/Script/AIModule.AIController|GetBrainComponent (Variables|Default|GetAIC%20Demon%20REF)) "")
            (Variables|/Game/Blueprints/Health_Damage_System/BPC_DamageSystem.BPC_DamageSystem_C|SetisInvincible _bpc_damagesystem true)
            (Utilities|FlowControl|Delay 1.4)
            (Components|Activation|Activate _ripple_vfx false)
            (bind _newhealth (Default|Heal _bpc_damagesystem_2 1e+02))
            (Variables|/Game/Blueprints/Health_Damage_System/BPC_DamageSystem.BPC_DamageSystem_C|SetHealth _bpc_damagesystem_2 _newhealth))
          (:OnCompleted
            (Components|Activation|Deactivate _ripple_vfx)
            (Variables|/Game/Blueprints/Health_Damage_System/BPC_DamageSystem.BPC_DamageSystem_C|SetisInvincible _bpc_damagesystem false)
            (Variables|/Game/Blueprints/Health_Damage_System/BPC_DamageSystem.BPC_DamageSystem_C|SetisInterruptible _bpc_damagesystem true)
            (AI|RunBehaviorTree (Variables|Default|GetAIC%20Demon%20REF) (Variables|Default|GetBehaviorTree))))))))

(event OnDeath(BPC_DamageSystem)
  (bind _mesh (Variables|Character|GetMesh))
  ;[1 0 0] AI Death Logic
  (Physics|SetSimulatePhysics _mesh true)
  (Collision|SetCollisionEnabled _mesh "QueryAndPhysics")
  (AI|Logic|StopLogic (Variables|/Script/AIModule.AIController|GetBrainComponent (Variables|Default|GetAIC%20Demon%20REF)) "")
  (Default|SetStateasDead (Variables|Default|GetAIC%20Demon%20REF))
  (Utilities|FlowControl|Delay 2.0)
  (Actor|DestroyActor))

(event Custom|Attack
  (bind _returnvalue (Transformation|GetActorLocation))
  ;[0 0.0585 1] - AI Attack Animation
  ; - Attack Deals Damage to Player
  (bind _notifyname (Animation|Montage|PlayMontage (Variables|Character|GetMesh) (Variables|Default|GetAttack_Animation))
    (:OnCompleted
      (Default|CallOnAttackEnd :!label _label))
    (:OnInterrupted
      (goto _label))
    (:OnNotifyBegin
      (switch name _notifyname
        (:Swing
          (bind (_outhit _returnvalue_2) (Collision|SphereTraceForObjects _returnvalue (+ _returnvalue (* (Transformation|GetActorForwardVector) 1e+02)) 2e+01 (Utilities|Array|MakeArray "ObjectTypeQuery3") false 0 "ForDuration"))
          (if _returnvalue_2
            (Class|BPIDamagable|TakeDamage(Message) (.HitActor (Collision|BreakHitResult _outhit)) (Utilities|Struct|MakeS_DamageInfo 4e+01 "NewEnumerator1"))))))))

(event Custom|Jump%20to%20target
  (params (Attack%20Target :type Actor%20Object%20Reference))
  (bind _returnvalue (Transformation|GetActorLocation Attack%20Target))
  ;[0 0.0585 1] - AI Attack Animation
  ; - Attack Deals Damage to Player
  (bind _outlaunchvelocity (Game|SuggestProjectileVelocityCustomArc (Transformation|GetActorLocation) (Math|Vector|MakeVector (.x _returnvalue) (.y _returnvalue) (+ (.z _returnvalue) 1e+02)) 0.0 0.5))
  (Character|LaunchCharacter _outlaunchvelocity true true))

(event EventBeginPlay
  (bind _bpc_damagesystem (Variables|Default|GetBPC_DamageSystem))
  (Utilities|FlowControl|Sequence
    (:then_0
      (|CallParentFunction))
    (:then_1
      (bind _output_get (Variables|/Game/Blueprints/Health_Damage_System/BPC_DamageSystem.BPC_DamageSystem_C|SetMaxHealth _bpc_damagesystem 2e+02))
      (Variables|/Game/Blueprints/Health_Damage_System/BPC_DamageSystem.BPC_DamageSystem_C|SetHealth _bpc_damagesystem _output_get))))

(fn ConstructionScript
  (|CallParentFunction))

(fn GetIdealRange
  (return 1.5e+02 4e+02))