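; BPC_ObjectPool is a Blueprint component that pre-spawns and reuses actors of a configurable pooled class.
; On BeginPlay it spawns a small random number of them, ignoring its PoolSize variable, and marks each not in use.
; SpawnFromPool takes the first free actor, moves it to the requested transform and flags it in use.
; An exhausted pool only prints a failure message and does not grow.
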(event Custom|Initialize%20Pool
  (for _index (range 0 (Math|Random|RandomIntegerinRange 1 3))
    (bind _returnvalue (Game|SpawnActorfromClass (Variables|Default|GetPooledActorClass) (Math|Transform|MakeTransform "0, 0, 0" "0, 0, 0" "1.000000,1.000000,1.000000") "Undefined" "MultiplyWithRoot" 0 5.0 0))
    (Utilities|Array|AddUnique (Variables|Default|GetObjectPool) _returnvalue)
    (Default|SetinUse _returnvalue false)))

(event EventBeginPlay
  (CallFunction|InitializePool))

(fn FindFirstAvailableActor
  (for _array_element (Variables|Default|GetObjectPool)
    (if (not (Variables|/Game/AI/Blueprints/BP_PooledActor.BP_PooledActor_C|GetInUse _array_element))
      (return _array_element))))

(fn SpawnfromPool
  (params (Spawn%20Transform :type Transform))
  (bind _pooledactor (CallFunction|FindFirstAvailableActor))
  (Utilities|IsValid _pooledactor
    (:Is%20Valid
      (Transformation|SetActorTransform _pooledactor Spawn%20Transform)
      (Default|SetinUse _pooledactor true)
      (return _pooledactor))
    (:Is%20Not%20Valid
      (Development|PrintString "Failed to Find Object from Pool!"))))