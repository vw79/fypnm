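; AI controller for the Titan enemy that runs its behavior tree and triggers a demon spawn when it sees something.
; On possession it waits briefly, starts the pawn's tree in a patrolling state and writes the pawn's attack and defend radii to the Blackboard.
; Perception updates are filtered for successful sight stimuli, and a DoOnce lets only the first one call the spawn manager with the Titan reference.
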(event OnPerceptionUpdated(DemonPerception)
  (params (UpdatedActors :type Array%20of%20Actor%20Object%20References))
  (for _array_element UpdatedActors
    (bind _sensed (CallFunction|CanSenseActor _array_element "NewEnumerator1"))
    (if _sensed
      (Utilities|FlowControl|DoOnce false
        (:Completed
          (Default|SpawnDemons (Variables|Default|GetBPC_SpawnManager) (Variables|Default|GetTitan%20REF)))))))

(event EventPossess
  (params (PossessedPawn :type Pawn%20Object%20Reference))
  (bind _blackboard (Variables|Default|GetBlackboard))
  (bind _asbp_titan (Utilities|Casting|CastToBP_Titan PossessedPawn))
  (Variables|Default|SetTitan%20REF _asbp_titan)
  (Utilities|FlowControl|Delay 0.2)
  (AI|RunBehaviorTree (Variables|/Game/AI/Blueprints/BP_Demon_Base.BP_Demon_Base_C|GetBehaviorTree _asbp_titan))
  (CallFunction|SetStateasPatrolling)
  (bind (_attackradius _defendradius) (Class|BPIDemon|GetIdealRange(Message) PossessedPawn))
  (AI|Components|Blackboard|SetValueasFloat _blackboard (Variables|Default|GetAttack%20Radius%20Key) _attackradius)
  (AI|Components|Blackboard|SetValueasFloat _blackboard (Variables|Default|GetDefend%20Radius%20Key) _defendradius))

(fn ConstructionScript
  (|CallParentFunction))

(fn CanSenseActor
  (params (Actor :type Actor%20Object%20Reference) (Sense :type E_AISense%20Enum :default "NewEnumerator0"))
  (bind _info (Class|AIPerceptionComponent|GetActorsPerception (Variables|Default|GetDemon%20Perception) Actor))
  (for _array_element (.LastSensedStimuli (Utilities|Struct|BreakActorPerceptionBlueprintInfo _info))
    (bind _returnvalue (Class|AIPerceptionSystem|GetSenseClassforStimulus _array_element))
    (if (== _returnvalue (Utilities|Select :Index Sense :NewEnumerator0 0 :NewEnumerator1 "/Script/AIModule.AISense_Sight" :NewEnumerator2 0))
      (return (.bSuccessfullySensed (Utilities|Struct|BreakAIStimulus _array_element)) _array_element))))