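; AI controller for demon enemies that runs the pawn's behavior tree and manages its blackboard state.
; On possess, it briefly delays, starts the tree, sets Attacking on player 0 and stores the pawn's attack and defend radii.
; AI perception filters sight and damage stimuli: sight only prints a message, while damage switches Passive or Investigate demons to Attacking.
; State setters cover attacking, patrolling, waiting, stunned and dead, which also unpossesses.
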(event OnPerceptionUpdated(DemonPerception)
  (params (UpdatedActors :type Array%20of%20Actor%20Object%20References))
  (for _array_element UpdatedActors
    (Utilities|FlowControl|Sequence
      (:then_0
        (bind _sensed (CallFunction|SenseActor _array_element "NewEnumerator1"))
        (if _sensed
          (CallFunction|HandleSensedSight)))
      (:then_1
        (bind _sensed_2 (CallFunction|SenseActor 0 "NewEnumerator2"))
        (if _sensed_2
          (CallFunction|HandleSensedDamage _array_element))))))

(event EventPossess
  (params (PossessedPawn :type Pawn%20Object%20Reference))
  (bind _blackboard (Variables|Default|GetBlackboard))
  (bind _asbp_demon_base (Utilities|Casting|CastToBP_Demon_Base PossessedPawn))
  (Utilities|FlowControl|Delay 0.2)
  (AI|RunBehaviorTree (Variables|/Game/AI/Blueprints/BP_Demon_Base.BP_Demon_Base_C|GetBehaviorTree _asbp_demon_base))
  (CallFunction|SetStateasAttacking (Game|GetPlayerCharacter 0))
  (bind (_attackradius _defendradius) (Class|BPIDemon|GetIdealRange(Message) PossessedPawn))
  (AI|Components|Blackboard|SetValueasFloat _blackboard (Variables|Keys|GetAttackRadiusKey) _attackradius)
  (AI|Components|Blackboard|SetValueasFloat _blackboard (Variables|Keys|GetDefendRadiusKey) _defendradius))

(fn ConstructionScript)

(fn SetStateasAttacking
  (params (PlayerTarget :type Actor%20Object%20Reference))
  (bind _blackboard (Variables|Default|GetBlackboard))
  (AI|Components|Blackboard|SetValueasObject _blackboard (Variables|Keys|GetPlayer%20Key) PlayerTarget)
  (AI|Components|Blackboard|SetValueasEnum _blackboard (Variables|Keys|GetState%20Key) (Utilities|Enum|LiteralenumE_States "NewEnumerator0"))
  (Variables|Default|SetPlayer%20Target PlayerTarget))

(fn SetStateasPatrolling
  (AI|Components|Blackboard|SetValueasEnum (Variables|Default|GetBlackboard) (Variables|Keys|GetState%20Key) (Utilities|Enum|LiteralenumE_States "NewEnumerator1")))

(fn SetStateasDead
  (AI|Components|Blackboard|SetValueasEnum (Variables|Default|GetBlackboard) (Variables|Keys|GetState%20Key) (Utilities|Enum|LiteralenumE_States "NewEnumerator5"))
  (Pawn|UnPossess))

(fn SetStateasStunned
  (AI|Components|Blackboard|SetValueasEnum (Variables|Default|GetBlackboard) (Variables|Keys|GetState%20Key) (Utilities|Enum|LiteralenumE_States "NewEnumerator2")))

(fn SetStateasWaiting
  (params (PlayerTarget :type Actor%20Object%20Reference))
  (bind _blackboard (Variables|Default|GetBlackboard))
  (AI|Components|Blackboard|SetValueasObject _blackboard (Variables|Keys|GetPlayer%20Key) PlayerTarget)
  (AI|Components|Blackboard|SetValueasEnum _blackboard (Variables|Keys|GetState%20Key) (Utilities|Enum|LiteralenumE_States "NewEnumerator4"))
  (Variables|Default|SetPlayer%20Target PlayerTarget))

(fn SenseActor
  (params (Actor :type Actor%20Object%20Reference) (Sense :type E_AISense%20Enum :default "NewEnumerator0"))
  (bind _info (Class|AIPerceptionComponent|GetActorsPerception (Variables|Default|GetDemon%20Perception) Actor))
  (for _array_element (.LastSensedStimuli (Utilities|Struct|BreakActorPerceptionBlueprintInfo _info))
    (bind _returnvalue (Class|AIPerceptionSystem|GetSenseClassforStimulus _array_element))
    (if (== _returnvalue (Utilities|Select :Index Sense :NewEnumerator0 0 :NewEnumerator1 "/Script/AIModule.AISense_Sight" :NewEnumerator2 "/Script/AIModule.AISense_Damage"))
      (return (.bSuccessfullySensed (Utilities|Struct|BreakAIStimulus _array_element)) _array_element))))

(fn HandleSensedDamage
  (params (Actor :type Actor%20Object%20Reference))
  (bind _state (CallFunction|GetCurrentState))
  (switch Utilities|FlowControl|Switch|SwitchonE_States _state
    (:NewEnumerator4
      _)
    (:NewEnumerator3
      _))
  (CallFunction|SetStateasAttacking Actor))

(fn GetCurrentState
  (return (Utilities|Enum|ByteToEnumE_States (Class|BlackboardComponent|GetValueasEnum (Variables|Default|GetBlackboard) (Variables|Keys|GetState%20Key)))))

(fn HandleSensedSight
  (params (Actor :type Actor%20Object%20Reference))
  (Development|PrintString "Player Seen!"))