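; Shielder demon enemy character that attacks, blocks with a shield, leaps at targets and self-heals.
; Swing and heavy attacks go through BPCAttacks, while BPCDamageSystem handles health, blocking and attack tokens.
; Hits stun it via the AI controller, play directional reactions or air-juggle it, flag executable at low health and trigger a one-time invincible heal.
; Death ragdolls it, stops AI, clears player lock-on, then dissolves it and spawns a pooled orb.
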(event OnDamageResponse(BPC_DamageSystem)
  (params (DamageResponse :type E_DamageResponse%20Enum :default "NewEnumerator0") (HitDirection :type E_DirectionalHit%20Enum :default "NewEnumerator0"))
  (bind _bpc_damagesystem (Variables|Default|GetBPC_DamageSystem))
  (bind _bpc_damagesystem_2 (Variables|Default|GetBPC_DamageSystem))
  (bind _playercontrollerref (Variables|Default|GetPlayerControllerRef))
  ;[1 0.8259 0] - AI Has a Hit Reaction to Damage
  ; - AI Heals when Health is below 30
  ; - Invincible for 2 seconds when healing then can take damage again
  (if (> (Variables|/Game/Blueprints/Health_Damage_System/BPC_DamageSystem.BPC_DamageSystem_C|GetHealth (Variables|Default|GetBPC_DamageSystem)) 2e+01)
    _
    (else
      (Default|SetIndicationColor (Variables|Default|GetWbpLockOnRef) (Utilities|Struct|MakeSlateColor "(R=1.000000,G=0.006772,B=0.000000,A=1.000000)"))
      (Variables|/Game/Blueprints/Health_Damage_System/BPC_DamageSystem.BPC_DamageSystem_C|SetisExecutable (Variables|Default|GetBPC_DamageSystem) true)))
  (Components|Movement|StopMovementImmediately (Variables|Character|GetCharacterMovement))
  (Default|SetStateasStunned (Variables|Default|GetAIC%20Demon%20REF))
  (bind _aswbp_health_bar (Utilities|Casting|CastToWBP_HealthBar (UserInterface|GetWidget (Variables|Default|GetHealth%20Bar%20Widget))))
  (Default|DamageGlitch _aswbp_health_bar)
  (if (not (AI|Components|NavMovement|IsFalling (Variables|Character|GetCharacterMovement)))
    (Utilities|DirectionalHitAnimation HitDirection
      (:then
        (Default|SetStateasAttacking (Variables|Default|GetAIC%20Demon%20REF) (Game|GetPlayerCharacter 0)))
      (:OnCompleted
        _)
      (:OnInterrupted
        _))
    (if (<= (Variables|/Game/Blueprints/Health_Damage_System/BPC_DamageSystem.BPC_DamageSystem_C|GetHealth _bpc_damagesystem_2) 3e+01)
      (Class|BPIDamagable|SetIsInterruptible(Message) _bpc_damagesystem_2 false)
      (Utilities|FlowControl|DoOnce false
        (:Completed
          (Animation|Montage|PlayMontage (Variables|Character|GetMesh) "/Game/Animation/MeleeDemon/AM_Heal.AM_Heal"
            (:then
              (AI|Logic|StopLogic (Variables|/Script/AIModule.AIController|GetBrainComponent (Variables|Default|GetAIC%20Demon%20REF)) "")
              (Variables|/Game/Blueprints/Health_Damage_System/BPC_DamageSystem.BPC_DamageSystem_C|SetisInvincible _bpc_damagesystem true)
              (bind _newhealth (Default|Heal _bpc_damagesystem_2 1e+02))
              (Variables|/Game/Blueprints/Health_Damage_System/BPC_DamageSystem.BPC_DamageSystem_C|SetHealth _bpc_damagesystem_2 _newhealth))
            (:OnCompleted
              (Variables|/Game/Blueprints/Health_Damage_System/BPC_DamageSystem.BPC_DamageSystem_C|SetisInvincible _bpc_damagesystem false)
              (Class|BPIDamagable|SetIsInterruptible(Message) _bpc_damagesystem_2 true)
              (AI|RunBehaviorTree (Variables|Default|GetAIC%20Demon%20REF) (Variables|Default|GetBehaviorTree)))))))
    (else
      ;;[1 1 1] Air Attack Hit Reaction
      (Variables|Default|SetisStayAir true)
      (if (not (Variables|/Game/Blueprints/BP_MCController.BP_MCController_C|GetisSlam _playercontrollerref))
        (Transformation|SetRelativeLocation (Variables|Default|GetCapsuleComponent) (Transformation|GetWorldLocation (Variables|/Game/ThirdPerson/Blueprints/Player/BP_MC.BP_MC_C|GetAirAttack (Variables|/Game/Blueprints/BP_MCController.BP_MCController_C|GetPlayerCharacterRef _playercontrollerref))) false false)))))

(event OnDeath(BPC_DamageSystem)
  (bind _mesh (Variables|Character|GetMesh))
  (Variables|Default|SetisStayAir false)
  (CallFunction|HandleDeathTargeting)
  ;[1 0 0] AI Death Logic
  (Physics|SetSimulatePhysics _mesh true)
  (Collision|SetCollisionEnabled _mesh "QueryAndPhysics")
  (AI|Logic|StopLogic (Variables|/Script/AIModule.AIController|GetBrainComponent (Variables|Default|GetAIC%20Demon%20REF)) "")
  (Default|SetStateasDead (Variables|Default|GetAIC%20Demon%20REF))
  (Utilities|Time|SetTimerbyEvent (delegate Custom|Dissolve%20Enemy) 4.0))

(event Custom|Swing%20Attack
  (params (Attack%20Target :type Actor%20Object%20Reference))
  ;[0 0.0585 1] - AI Attack Animation
  ; - Attack Deals Damage to Player
  ; - Attack Blocking
  (Default|SwingAttack (Variables|Default|GetBPC_Attacks) (Utilities|Struct|MakeS_Attacks Attack%20Target "/Game/Animation/MeleeDemon/AM_Swing.AM_Swing" (Utilities|Struct|MakeS_DamageInfo 2e+01 "NewEnumerator1"))))

(event Custom|Dissolve%20Enemy
  (bind _dissolve_particles (Variables|Default|GetDissolve%20Particles))
  ;[1 0 0] AI Death Logic
  (Components|Activation|Activate _dissolve_particles false)
  (bind _dissolve_amount (Timeline|Timeline PlayFromStart)
    (:Update
      (Niagara|SetNiagaraVariable(Float) _dissolve_particles "Mask" _dissolve_amount)
      (Rendering|Material|SetScalarParameterValueonMaterials (Variables|Character|GetMesh) "Mask" _dissolve_amount))
    (:Finished
      (Components|Activation|Deactivate _dissolve_particles)
      (CallFunction|SpawnOrb)
      (Actor|DestroyActor))))

(event Custom|Jump%20to%20target
  (params (Attack%20Target :type Actor%20Object%20Reference))
  (bind _returnvalue (Transformation|GetActorLocation Attack%20Target))
  ;[0 0.0585 1] - AI Attack Animation
  ; - Attack Deals Damage to Player
  ; - Attack Blocking
  (bind _outlaunchvelocity (Game|SuggestProjectileVelocityCustomArc (Transformation|GetActorLocation) (Math|Vector|MakeVector (.x _returnvalue) (.y _returnvalue) (+ (.z _returnvalue) 1e+02)) 0.0 0.5))
  (Character|LaunchCharacter _outlaunchvelocity true true))

(event Custom|Spawn%20Orb
  ;[1 0 0] AI Death Logic
  (Default|SpawnfromPool (Variables|Default|GetBPC_ObjectPool) (Math|Transform|MakeTransform (Transformation|GetActorLocation) "0, 0, 0" "1.000000,1.000000,1.000000")))

(event Custom|Block%20Attacks
  ;[0 0.0585 1] - AI Attack Animation
  ; - Attack Deals Damage to Player
  ; - Attack Blocking
  (Variables|/Game/Blueprints/Health_Damage_System/BPC_DamageSystem.BPC_DamageSystem_C|SetisBlocking (Variables|Default|GetBPC_DamageSystem) true)
  (Animation|Montage|PlayMontage (Variables|Character|GetMesh) "/Game/Animation/MeleeDemon/AM_Block.AM_Block"
    (:then
      (Components|Activation|Activate (Variables|Default|GetShield%20VFX) false))
    (:OnCompleted
      (CallFunction|EndBlock :!label _label))
    (:OnInterrupted
      (goto _label))))

(event Custom|End%20Block
  ;[0 0.0585 1] - AI Attack Animation
  ; - Attack Deals Damage to Player
  ; - Attack Blocking
  (Utilities|FlowControl|Delay 2.0)
  (Variables|/Game/Blueprints/Health_Damage_System/BPC_DamageSystem.BPC_DamageSystem_C|SetisBlocking (Variables|Default|GetBPC_DamageSystem) false)
  (Components|Activation|Deactivate (Variables|Default|GetShield%20VFX))
  (Default|CallOnBlockEnd))

(event Custom|Heavy%20Attack
  (params (Attack%20Target :type Actor%20Object%20Reference))
  ;[0 0.0585 1] - AI Attack Animation
  ; - Attack Deals Damage to Player
  ; - Attack Blocking
  (Default|HeavyAttack (Variables|Default|GetBPC_Attacks) (Utilities|Struct|MakeS_Attacks Attack%20Target "/Game/Animation/MeleeDemon/AM_Heavy.AM_Heavy" (Utilities|Struct|MakeS_DamageInfo 4e+01 "NewEnumerator1"))))

(event EventBeginPlay
  (bind _bpc_damagesystem (Variables|Default|GetBPC_DamageSystem))
  (Utilities|FlowControl|Sequence
    (:then_0
      (|CallParentFunction))
    (:then_1
      (bind _output_get (Variables|/Game/Blueprints/Health_Damage_System/BPC_DamageSystem.BPC_DamageSystem_C|SetMaxHealth _bpc_damagesystem 2e+02))
      (Variables|/Game/Blueprints/Health_Damage_System/BPC_DamageSystem.BPC_DamageSystem_C|SetHealth _bpc_damagesystem _output_get))))

(event EventOnLanded
  (params (Hit :type Hit%20Result%20Structure%20%28by%20ref%29))
  ;[1 1 1] Air Attack
  ;;[1 1 1] Reset Stay in Air
  (Variables|Default|SetisStayAir false)
  (Default|SetStateasAttacking (Variables|Default|GetAIC%20Demon%20REF) (Game|GetPlayerCharacter 0)))

(event EventReturnAttackToken
  (params (Amount :type Integer))
  ;[0 0.0585 1] - AI Attack Animation
  ; - Attack Deals Damage to Player
  ; - Attack Blocking
  (Default|ReturnAttackToken (Variables|Default|GetBPC_DamageSystem) Amount))

(event EventAATKLaunchEnemy
  (params (LaunchVelocity :type Vector :default "0, 0, 0") (XYOverride :type Boolean) (ZOverride :type Boolean))
  ;[1 1 1] Air Attack
  ;;[1 1 1] Interfaces
  (Character|LaunchCharacter LaunchVelocity XYOverride ZOverride)
  (Default|SetStateasStunned (Variables|Default|GetAIC%20Demon%20REF)))

(event EventLaunchEnemy
  (params (Velocity :type Vector :default "0, 0, 0") (XY :type Boolean) (Z :type Boolean))
  ;[1 1 1] Air Attack
  ;;[1 1 1] Slam Enemy Down
  (Character|LaunchCharacter Velocity XY Z))

(event EventActivateParryIndicator
  (params (IndicatorDuration :type Float%20%28double-precision%29))
  (bind _parryindicator (Variables|Default|GetParryIndicator))
  ;[1 1 1] Parry Indication
  (if (not (Variables|/Game/Blueprints/Health_Damage_System/BPC_DamageSystem.BPC_DamageSystem_C|GetisDead (Variables|Default|GetBPC_DamageSystem)))
    (Niagara|SetNiagaraVariable(Float) _parryindicator "Lifetime" IndicatorDuration)
    (Components|Activation|Activate _parryindicator false)))

(fn ConstructionScript
  (|CallParentFunction))

(fn GetIdealRange
  (return 1.3e+02 4e+02))

(fn ReserveAttackToken
  (params (Amount :type Integer))
  (bind _success (Default|ReserveAttackToken (Variables|Default|GetBPC_DamageSystem) Amount))
  (return _success))

(fn IsAttacking
  (return (Variables|Default|GetAttacking)))

(fn GetDemonRef
  (return self (Variables|Default|GetBPC_DamageSystem)))

(fn HandleDeathTargeting
  (bind _playercontrollerref (Variables|Default|GetPlayerControllerRef))
  (bind _targetingsystemref (Variables|/Game/Blueprints/BP_MCController.BP_MCController_C|GetTargetingSystemRef _playercontrollerref))
  (Rendering|SetVisibility (Variables|Default|GetLock) false false)
  (if (Variables|/Game/Blueprints/Component/BPC_TargetingSystem.BPC_TargetingSystem_C|GetisHardLock _targetingsystemref)
    (Default|EndHardTarget _targetingsystemref)
    (Collision|SetCollisionResponsetoChannel (Variables|Default|GetCapsuleComponent) "ECC_Visibility" "ECR_Ignore" :!label _label)
    (elif (Variables|/Game/Blueprints/Component/BPC_TargetingSystem.BPC_TargetingSystem_C|GetisSoftLock _targetingsystemref)
      (Default|EndSoftTarget _targetingsystemref)
      (goto _label))))