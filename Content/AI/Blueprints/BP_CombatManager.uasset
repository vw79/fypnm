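; BP_CombatManager limits how many AI attackers engage one target at once, defaulting to the player character.
; At BeginPlay it gets the attacker cap from the target via a GAS message.
; Attack requests receive an Attack message while slots are free; overflow is queued with a Wait message.
; An attacker's death promotes the first waiter, while the target's death sets everyone to wait and clears both lists.
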(event EventBeginPlay
  (Variables|Default|GetAttack%20Target
    (:then
      _)
    (:else
      (Variables|Default|SetAttack%20Target (Game|GetPlayerCharacter 0))))
  (bind _value (Class|BPIGAS|GASGetMaxAttackersCount(Message) (Variables|Default|GetAttack%20Target)))
  (Variables|Default|SetMax%20Attackers%20Count _value))

(fn ConstructionScript)

(fn HandleAttackRequest
  (params (Attacker :type Actor%20Object%20Reference))
  (bind _attack_target (Variables|Default|GetAttack%20Target))
  (if (!= Attacker (Variables|Default|GetAttack%20Target))
    (if (< (Utilities|Array|Length (Variables|Default|GetAttackers)) (Variables|Default|GetMax%20Attackers%20Count))
      (Utilities|Array|AddUnique (Variables|Default|GetAttackers) Attacker)
      (Class|BPIDemon|Attack(Message) Attacker _attack_target)
      (else
        (Utilities|Array|AddUnique (Variables|Default|GetWaitingAttackers) Attacker)
        (Class|BPIDemon|Wait(Message) Attacker _attack_target)))))

(fn HandleDeath
  (params (Actor%20Ref :type Actor%20Object%20Reference))
  (bind _attack_target (Variables|Default|GetAttack%20Target))
  (bind _attackers (Variables|Default|GetAttackers))
  (if (== Actor%20Ref _attack_target)
    (Utilities|Array|AppendArray _attackers (Variables|Default|GetWaitingAttackers))
    (for _array_element _attackers
      (Class|BPIDemon|Wait(Message) _array_element _attack_target))
    (Utilities|Array|Clear (Variables|Default|GetWaitingAttackers))
    (Utilities|Array|Clear (Variables|Default|GetAttackers))
    (elif (Utilities|Array|ContainsItem (Variables|Default|GetAttackers) Actor%20Ref)
      (Utilities|Array|RemoveItem (Variables|Default|GetAttackers) Actor%20Ref)
      (CallFunction|EngageWaitingAttacker)
      (elif (Utilities|Array|ContainsItem (Variables|Default|GetWaitingAttackers) Actor%20Ref)
        (Utilities|Array|RemoveItem (Variables|Default|GetWaitingAttackers) Actor%20Ref)))))

(fn EngageWaitingAttacker
  (bind _waitingattackers (Variables|Default|GetWaitingAttackers))
  (bind _output (Utilities|Array|Get(acopy) _waitingattackers))
  (Utilities|IsValid _output
    (:Is%20Valid
      (bind _output_get (Variables|Default|SetWaiting%20Attacker _output))
      (Utilities|Array|RemoveItem (Variables|Default|GetWaitingAttackers) _output_get)
      (Utilities|Array|AddUnique (Variables|Default|GetAttackers) _output_get)
      (Class|BPIDemon|Attack(Message) _output_get (Variables|Default|GetAttack%20Target)))))