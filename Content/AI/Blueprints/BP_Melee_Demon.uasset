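; Melee demon enemy character that attacks with an animation montage, reacts to hits and reports its death to the game mode.
; A montage notify triggers a short forward sphere trace that applies damage.
; BPCDamageSystem handles attack tokens and drives damage and death events: hits stun the AI, then resume attacking the player.
; Death ragdolls the mesh, stops AI logic, updates the remaining-demon count and destroys the actor after a delay.
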(event Custom|DamageResponse
  (params (DamageResponse :type E_DamageResponse%20Enum :default "NewEnumerator0"))
  ;[1 0.8259 0] - AI Has a Hit Reaction to Damage
  (Components|Movement|StopMovementImmediately (Variables|Character|GetCharacterMovement))
  (Default|SetStateasStunned (Variables|Default|GetAIC%20Demon%20REF))
  (Animation|Montage|PlayMontage (Variables|Character|GetMesh) "/Game/AI/Animations/Animation_Sequence/Manny/AM_Hit_Reaction.AM_Hit_Reaction"
    (:OnCompleted
      _)
    (:OnInterrupted
      _))
  (Default|SetStateasAttacking (Variables|Default|GetAIC%20Demon%20REF) (Game|GetPlayerCharacter 0)))

(event Custom|Death
  (bind _mesh (Variables|Character|GetMesh))
  ;[1 0 0] AI Death Logic
  (Physics|SetSimulatePhysics _mesh true)
  (Collision|SetCollisionEnabled _mesh "QueryAndPhysics")
  (AI|Logic|StopLogic (Variables|/Script/AIModule.AIController|GetBrainComponent (Variables|Default|GetAIC%20Demon%20REF)) "")
  (Default|SetStateasDead (Variables|Default|GetAIC%20Demon%20REF))
  (bind _asbp_third_person_game_mode (Utilities|Casting|CastToBP_ThirdPersonGameMode (Game|GetGameMode)))
  (Math|Integer|DecrementInt (Variables|/Game/ThirdPerson/Blueprints/BP_ThirdPersonGameMode.BP_ThirdPersonGameMode_C|GetDemons%20Remaining _asbp_third_person_game_mode)
    (:%20%20
      (Default|CheckRemainingDemons _asbp_third_person_game_mode)
      (Utilities|FlowControl|Delay 2.0)
      (Actor|DestroyActor))))

(event EventReturnAttackToken
  (params (Amount :type Integer))
  ;[0 0.0585 1] AI Attack System
  (Default|ReturnAttackToken (Variables|Default|GetBPC_DamageSystem) Amount))

(event EventAttack
  (params (Attack%20Target :type Actor%20Object%20Reference))
  (bind _returnvalue (Transformation|GetActorLocation))
  ;[0 0.0585 1] AI Attack System
  (|CallParentFunction Attack%20Target)
  (bind _notifyname (Animation|Montage|PlayMontage (Variables|Character|GetMesh) (Variables|Default|GetAttack_Animation) 1.4)
    (:OnCompleted
      (CallFunction|FinishAttacking Attack%20Target :!label _label))
    (:OnInterrupted
      (goto _label))
    (:OnNotifyBegin
      (switch name _notifyname
        (:Punch
          (bind (_outhit _returnvalue_2) (Collision|SphereTraceForObjects _returnvalue (+ _returnvalue (* (Transformation|GetActorForwardVector) 1e+02)) 2e+01 (Utilities|Array|MakeArray "ObjectTypeQuery3") false 0 "None"))
          (if _returnvalue_2
            (Class|BPIDamagable|TakeDamage(Message) (.HitActor (Collision|BreakHitResult _outhit)) (Utilities|Struct|MakeS_DamageInfo 1e+01 "NewEnumerator1"))))))))

(fn ConstructionScript
  (bind _bpc_damagesystem (Variables|Default|GetBPC_DamageSystem))
  (EventDispatchers|BindEventtoOnDeath _bpc_damagesystem (EventDispatchers|CreateEvent :!event Custom|Death))
  (EventDispatchers|BindEventtoOnDamageResponse _bpc_damagesystem (EventDispatchers|CreateEvent :!event Custom|DamageResponse)))

(fn Heal
  (params (HealAmount :type Float%20%28double-precision%29))
  (return 0.0))

(fn ReserveAttackToken
  (params (Amount :type Integer))
  (bind _success (Default|ReserveAttackToken (Variables|Default|GetBPC_DamageSystem) Amount))
  (return _success))