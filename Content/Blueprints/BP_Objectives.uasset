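; BP_Objectives is a level objective manager that tracks the mission stage and decides win or lose through a box trigger.
; BeginPlay counts BP_Titan actors, and each TitanDeath decrements the count until Objective2 switches the GameState string to stopping Dr Draxxon.
; Box overlap switches on that string: during the first objective a Titan kills BP_MC once and others are warned back, while afterwards any overlap prints a win.
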(event OnComponentBeginOverlap(Box)
  (params (OverlappedComponent :type Primitive%20Component%20Object%20Reference) (OtherActor :type Actor%20Object%20Reference) (OtherComp :type Primitive%20Component%20Object%20Reference) (OtherBodyIndex :type Integer) (bFromSweep :type Boolean) (SweepResult :type Hit%20Result%20Structure%20%28by%20ref%29))
  (switch string (Variables|Default|GetGame%20State)
    (:Defeat%20the%203%20Titans
      (if (Actor|ActorHasTag OtherActor "Titan")
        (Utilities|FlowControl|DoOnce false
          (:Completed
            (Development|PrintString "You Lose Monkey!")
            (bind _returnvalue (Actor|GetActorOfClass "/Game/ThirdPerson/Blueprints/Player/BP_MC.BP_MC_C"))
            (Default|Dead _returnvalue)))
        (else
          (Development|PrintString "Turn Around!")
          (Actor|GetActorOfClass "/Game/ThirdPerson/Blueprints/Player/BP_MC.BP_MC_C"))))
    (:Stop%20Dr%20Draxxon%20top%20of%20Merdeka%20Tower
      (Development|PrintString "You Win!"))))

(event Custom|Titan%20Death
  (Variables|Default|SetTitan%20Count (- (Variables|Default|GetTitan%20Count) 1))
  (if (<= (Variables|Default|GetTitan%20Count) 0)
    (CallFunction|Objective2)))

(event Custom|Objective%202
  (bind _output_get (Variables|Default|SetGame%20State "Stop Dr Draxxon top of Merdeka Tower"))
  (Development|PrintString _output_get))

(event EventBeginPlay
  (bind _outactors (Actor|GetAllActorsOfClass "/Game/AI/Blueprints/Titan/BP_Titan.BP_Titan_C"))
  (Development|PrintString (Utilities|String|ToString(Integer) (Utilities|Array|Length _outactors)))
  (Variables|Default|SetTitan%20Count (Utilities|Array|Length _outactors))
  (Variables|Default|SetGame%20State "Defeat the 3 Titans"))

(fn ConstructionScript)