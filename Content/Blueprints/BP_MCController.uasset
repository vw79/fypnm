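; Player controller for the BP_MC character in a melee action game, handling combat input, targeting and the base UI with pause menu and prompts.
; Attack and dash inputs activate GAS abilities by tag based on ground state, combo tags and lock-on, with timelines turning the character toward hard or soft targets.
; Sphere-trace weapon hits apply damage, trigger parries with hit stop and keep air attackers aloft.
; It also handles weapon switching and slow-motion free look.
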(event Custom|OnPromptCanceled_Event
  (params (PromptIndex :type UI_PromptIndex%20Enum :default "NewEnumerator0") (PromptToStack :type UI_PromptToStack%20Enum :default "NewEnumerator0"))
  ;[1 1 1] Prompt
  ;;[1 1 1] Bindings
  (switch Utilities|FlowControl|Switch|SwitchonUI_PromptToStack PromptToStack
    (:NewEnumerator0
      _)
    (:NewEnumerator1
      _))
  (Class|BPIPromptInterface|PromptCanceled(Message) (Class|CommonActivatableWidgetContainerBase|GetActiveWidget (Variables|/Game/Widgets/AWB/AWB_BaseUILayout.AWB_BaseUILayout_C|GetMenuStack (Variables|UI|GetBaseUIWidget))) PromptIndex))

(event Custom|OnPromptConfirmed_Event
  (params (PromptIndex :type UI_PromptIndex%20Enum :default "NewEnumerator0") (PromptToStack :type UI_PromptToStack%20Enum :default "NewEnumerator0"))
  ;[1 1 1] Prompt
  ;;[1 1 1] Bindings
  (switch Utilities|FlowControl|Switch|SwitchonUI_PromptToStack PromptToStack
    (:NewEnumerator0
      _)
    (:NewEnumerator1
      _))
  (Class|BPIPromptInterface|PromptConfirmed(Message) (Class|CommonActivatableWidgetContainerBase|GetActiveWidget (Variables|/Game/Widgets/AWB/AWB_BaseUILayout.AWB_BaseUILayout_C|GetMenuStack (Variables|UI|GetBaseUIWidget))) PromptIndex))

(event Custom|Bindings
  (bind _masterbinderui (Variables|UI|GetMasterBinderUI))
  ;[1 1 1] Prompt
  ;;[1 1 1] Bindings
  (EventDispatchers|BindEventtoOnPromptConfirmed _masterbinderui (delegate Custom|OnPromptConfirmed_Event))
  (EventDispatchers|BindEventtoOnPromptCanceled _masterbinderui (delegate Custom|OnPromptCanceled_Event)))

(event Input|EnhancedActionEvents|EnhancedInputActionIA_Dash
  (params (ActionValue :type Boolean) (ElapsedSeconds :type Float%20%28double-precision%29) (TriggeredSeconds :type Float%20%28double-precision%29) (InputAction :type Input%20Action%20Object%20Reference :default "/Game/Input/IA_Dash.IA_Dash"))
  (bind _returnvalue (Dash|GetDesireRotation))
  ;[1 1 1] Dash
  (if (Utilities|Operators|NotEqual(!=) :A _returnvalue)
    (Transformation|SetActorRotation (Variables|Ref|GetPlayerCharacterRef) _returnvalue))
  (if (CallFunction|IsonGround)
    (Abilities|TryActivateAbilitiesbyTag (Variables|Ref|GetGASRef) (Variables|GasTag|Move|GetDashAbilityTag) true)
    (else
      (Abilities|TryActivateAbilitiesbyTag (Variables|Ref|GetGASRef) (Variables|GasTag|Move|GetAirDashAbilityTag) true))))

(event EventBeginPlay
  (bind _self self)
  ;[1 1 1] Event Begin Setup
  (bind _returnvalue (Actor|GetActorOfClass "/Game/ThirdPerson/Blueprints/Player/BP_MC.BP_MC_C"))
  (bind _output_get (Variables|Ref|SetPlayerCharacterRef _returnvalue))
  (Variables|Ref|SetGASRef (Variables|/Game/ThirdPerson/Blueprints/Player/BP_MC.BP_MC_C|GetAbilitySystem _output_get))
  (Variables|Ref|SetTargetingSystemRef (Variables|/Game/ThirdPerson/Blueprints/Player/BP_MC.BP_MC_C|GetBPC_TargetingSystem _output_get))
  (bind _returnvalue_2 (UserInterface|CreateWidget "/Game/Widgets/AWB/AWB_BaseUILayout.AWB_BaseUILayout_C" self))
  (bind _output_get_2 (Variables|UI|SetBaseUIWidget _returnvalue_2))
  (UserInterface|Viewport|AddtoViewport _output_get_2 0)
  (Input|SetInputModeGameOnly _self false)
  (Variables|/Script/Engine.PlayerController|SetbShowMouseCursor _self false)
  (bind _hudref (Default|PushHUDMenu (Variables|UI|GetBaseUIWidget)))
  (Variables|Ref|SetHUDRef _hudref)
  (bind _returnvalue_3 (Actor|GetActorOfClass "/Game/Blueprints/BP_MasterBinderUI.BP_MasterBinderUI_C"))
  (Variables|UI|SetMasterBinderUI _returnvalue_3)
  (CallFunction|Bindings))

(event EventPCWMPushMenuPrompt
  (params (PromptText :type Text) (PromptIndex :type UI_PromptIndex%20Enum :default "NewEnumerator0") (PromptToStack :type UI_PromptToStack%20Enum :default "NewEnumerator0"))
  ;[1 1 1] Prompt
  ;;[1 1 1] Menu Prompt With Custom Prompt (Quit)
  (Default|PushMenuPrompt (Variables|UI|GetBaseUIWidget) PromptIndex PromptToStack PromptText))

(event EventPCWMPushMenu
  (params (ActivatableWidget :type Common%20Activatable%20Widget%20Class%20Reference))
  ;[1 1 1] Push Any AWB Menu
  (Default|PushMenu (Variables|UI|GetBaseUIWidget) ActivatableWidget))

(event Input|KeyboardEvents|DebugKeyCapsLock
  (params (Key :type Key%20Structure) (ActionValue :type Input%20Action%20Value%20Structure))
  (bind _returnvalue (Dash|GetDesireRotation))
  ;[1 1 1] Dash
  (:Pressed
    (if (Utilities|Operators|NotEqual(!=) :A _returnvalue)
      (Transformation|SetActorRotation (Variables|Ref|GetPlayerCharacterRef) _returnvalue))
    (if (CallFunction|IsonGround)
      (Abilities|TryActivateAbilitiesbyTag (Variables|Ref|GetGASRef) (Variables|GasTag|Move|GetDashAbilityTag) true)
      (else
        (Abilities|TryActivateAbilitiesbyTag (Variables|Ref|GetGASRef) (Variables|GasTag|Move|GetAirDashAbilityTag) true)))))

(event Input|KeyboardEvents|DebugKeyO
  (params (Key :type Key%20Structure) (ActionValue :type Input%20Action%20Value%20Structure))
  (bind _self self)
  (bind (_sizex _sizey) (HUD|GetViewportSize _self))
  ;[1 1 1] Pause Menu
  (:Pressed
    (if (not (Game|IsGamePaused))
      (CallFunction|PCWMPushMenu "/Game/Widgets/AWB/AWB_Pause.AWB_Pause_C")
      (Game|SetGamePaused true)
      (Input|SetInputModeUIOnly self 0 "DoNotLock" false)
      (Variables|Default|SetbShowMouseCursor true)
      (Class|PlayerController|SetMouseLocation (/ _sizex 2) (/ _sizey 3)))))

(event Input|KeyboardEvents|DebugKeyT
  (params (Key :type Key%20Structure) (ActionValue :type Input%20Action%20Value%20Structure))
  (:Pressed
    (Utilities|FlowControl|FlipFlop
      (:A
        ;[1 1 1] Free Look
        (bind _newtrack_0 (Timeline|SlowMo Play)
          (:Update
            (Utilities|Time|SetGlobalTimeDilation _newtrack_0))))
      (:B
        (Timeline|SlowMo Reverse)))))

(event Input|KeyboardEvents|Escape
  (params (Key :type Key%20Structure))
  ;[1 1 1] Pause Menu
)

(event Input|KeyboardEvents|LeftAlt
  (params (Key :type Key%20Structure))
  (bind _playercharacterref (Variables|Ref|GetPlayerCharacterRef))
  ;[1 1 1] Free Look
  (:Pressed
    (Variables|/Game/ThirdPerson/Blueprints/Player/BP_MC.BP_MC_C|SetIsFreeLook? _playercharacterref true)
    (bind _newtrack_0 (Timeline|SlowMo Play)
      (:Update
        (Utilities|Time|SetGlobalTimeDilation _newtrack_0))))
  (:Released
    (Variables|/Game/ThirdPerson/Blueprints/Player/BP_MC.BP_MC_C|SetIsFreeLook? _playercharacterref false)
    (Timeline|SlowMo Reverse)))

(event Custom|RotateToTarget
  (bind _playercharacterref (Variables|Ref|GetPlayerCharacterRef))
  (bind _playercharacterref_2 (Variables|Ref|GetPlayerCharacterRef))
  (bind _targetingsystemref (Variables|Ref|GetTargetingSystemRef))
  (bind _returnvalue (Transformation|GetActorRotation _playercharacterref_2))
  (bind _returnvalue_2 (Transformation|GetActorRotation _playercharacterref))
  (bind _softlockedonactor (Variables|/Game/Blueprints/Component/BPC_TargetingSystem.BPC_TargetingSystem_C|GetSoftLockedOnActor _targetingsystemref))
  ;[1 1 1] Player Rotation
  (if (Utilities|IsValid (Variables|/Game/Blueprints/Component/BPC_TargetingSystem.BPC_TargetingSystem_C|GetHardLockedOnActor (Variables|Ref|GetTargetingSystemRef)))
    ;;[1 0.4039 0] Rotate Towards Hard Target
    (Audio|Components|Audio|Stop (Variables|Default|GetRotationToHardTargetTimeline))
    (bind _hardtargetrotation (Timeline|RotationToHardTargetTimeline PlayFromStart)
      (:Update
        (if (Utilities|IsValid (Variables|/Game/Blueprints/Component/BPC_TargetingSystem.BPC_TargetingSystem_C|GetHardLockedOnActor (Variables|Ref|GetTargetingSystemRef)))
          (Transformation|SetActorRotation (Variables|Ref|GetPlayerCharacterRef) (Math|Rotator|Lerp(Rotator) (Transformation|GetActorRotation (Variables|Ref|GetPlayerCharacterRef)) (Math|Rotator|MakeRotator (.roll _returnvalue) (.pitch _returnvalue) (.yaw (Math|Rotator|FindLookatRotation (Transformation|GetActorLocation (Variables|Ref|GetPlayerCharacterRef)) (Transformation|GetActorLocation (Variables|/Game/Blueprints/Component/BPC_TargetingSystem.BPC_TargetingSystem_C|GetHardLockedOnActor (Variables|Ref|GetTargetingSystemRef)))))) _hardtargetrotation))
          (else
            (Audio|Components|Audio|Stop (Variables|Default|GetRotationToHardTargetTimeline))))))
    (else
      ;;[0.1559 1 0] Rotate Towards Soft Target
      (if (Utilities|IsValid _softlockedonactor)
        (bind _dmgsyscomponent (Class|BPIDamagable|DmgGetDmgSysComponent(Message) _softlockedonactor))
        (if (not (Variables|/Game/Blueprints/Health_Damage_System/BPC_DamageSystem.BPC_DamageSystem_C|GetisDead _dmgsyscomponent))
          (Variables|Target|SetSoftTargetEnemy _softlockedonactor)
          (Audio|Components|Audio|Stop (Variables|Default|GetRotationToSoftTargetTimeline))
          (bind _softtargetrotation (Timeline|RotationToSoftTargetTimeline PlayFromStart)
            (:Update
              (if (Utilities|IsValid (Variables|/Game/Blueprints/Component/BPC_TargetingSystem.BPC_TargetingSystem_C|GetSoftLockedOnActor (Variables|Ref|GetTargetingSystemRef)))
                (bind _dmgsyscomponent_2 (Class|BPIDamagable|DmgGetDmgSysComponent(Message) (Variables|Target|GetSoftTargetEnemy)))
                (if (Variables|/Game/Blueprints/Health_Damage_System/BPC_DamageSystem.BPC_DamageSystem_C|GetisDead _dmgsyscomponent_2)
                  (Audio|Components|Audio|Stop (Variables|Default|GetRotationToSoftTargetTimeline) :!label _label)
                  (Variables|Target|SetSoftTargetEnemy 0)
                  (else
                    (Transformation|SetActorRotation (Variables|Ref|GetPlayerCharacterRef) (Math|Rotator|Lerp(Rotator) (Transformation|GetActorRotation (Variables|Ref|GetPlayerCharacterRef)) (Math|Rotator|MakeRotator (.roll _returnvalue_2) (.pitch _returnvalue_2) (.yaw (Math|Rotator|FindLookatRotation (Transformation|GetActorLocation (Variables|Ref|GetPlayerCharacterRef)) (Transformation|GetActorLocation (Variables|/Game/Blueprints/Component/BPC_TargetingSystem.BPC_TargetingSystem_C|GetSoftLockedOnActor (Variables|Ref|GetTargetingSystemRef)))))) _softtargetrotation))))
                (else
                  (goto _label))))))))))

(event Input|EnhancedActionEvents|EnhancedInputActionIA_Targeting
  (params (ActionValue :type Boolean) (ElapsedSeconds :type Float%20%28double-precision%29) (TriggeredSeconds :type Float%20%28double-precision%29) (InputAction :type Input%20Action%20Object%20Reference :default "/Game/Input/IA_Targeting.IA_Targeting"))
  (bind _targetingsystemref (Variables|Ref|GetTargetingSystemRef))
  ;[1 0.402 0] Hard Lock Target Enemy
  (:Started
    (if (not (Variables|/Game/Blueprints/Component/BPC_TargetingSystem.BPC_TargetingSystem_C|GetisHardLock _targetingsystemref))
      (Default|HardLockonTarget _targetingsystemref)
      (else
        (Default|EndHardTarget _targetingsystemref)))))

(event Input|EnhancedActionEvents|EnhancedInputActionIA_Move
  (params (ActionValue :type Vector%202D%20Structure) (ElapsedSeconds :type Float%20%28double-precision%29) (TriggeredSeconds :type Float%20%28double-precision%29) (InputAction :type Input%20Action%20Object%20Reference :default "/Game/Input/IA_Move.IA_Move"))
  ;[0.1559 1 0] Cancel Soft Lock if Move
  (if (not (GameplayTags|HasMatchingGameplayTag (Variables|Ref|GetGASRef) "(TagName=\"Attack\")"))
    (Default|EndSoftTarget (Variables|Ref|GetTargetingSystemRef))))

(event Input|EnhancedActionEvents|EnhancedInputActionIA_SwitchTargetRight
  (params (ActionValue :type Boolean) (ElapsedSeconds :type Float%20%28double-precision%29) (TriggeredSeconds :type Float%20%28double-precision%29) (InputAction :type Input%20Action%20Object%20Reference :default "/Game/Input/IA_SwitchTargetRight.IA_SwitchTargetRight"))
  (bind _targetingsystemref (Variables|Ref|GetTargetingSystemRef))
  ;[1 0.402 0] Switch Target (Right)
  (:Started
    (if (Variables|/Game/Blueprints/Component/BPC_TargetingSystem.BPC_TargetingSystem_C|GetisHardLock _targetingsystemref)
      (Default|LockonTarget(Right) _targetingsystemref))))

(event Input|EnhancedActionEvents|EnhancedInputActionIA_Look
  (params (ActionValue :type Vector%202D%20Structure) (ElapsedSeconds :type Float%20%28double-precision%29) (TriggeredSeconds :type Float%20%28double-precision%29) (InputAction :type Input%20Action%20Object%20Reference :default "/Game/Input/IA_Look.IA_Look"))
  (bind _targetingsystemref (Variables|Ref|GetTargetingSystemRef))
  (:Started
    (if (Target|IsController (.x ActionValue))
      (if (Target|ThumbStickRight (.x ActionValue) (.y ActionValue))
        ;[1 0.402 0] Switch Target (Right)
        (if (Variables|/Game/Blueprints/Component/BPC_TargetingSystem.BPC_TargetingSystem_C|GetisHardLock _targetingsystemref)
          (Default|LockonTarget(Right) _targetingsystemref))))))

(event Input|EnhancedActionEvents|EnhancedInputActionIA_Look
  (params (ActionValue :type Vector%202D%20Structure) (ElapsedSeconds :type Float%20%28double-precision%29) (TriggeredSeconds :type Float%20%28double-precision%29) (InputAction :type Input%20Action%20Object%20Reference :default "/Game/Input/IA_Look.IA_Look"))
  (bind _targetingsystemref (Variables|Ref|GetTargetingSystemRef))
  (:Started
    (if (Target|IsController (.x ActionValue))
      (if (Target|ThumbStickLeft (.x ActionValue) (.y ActionValue))
        ;[1 0.402 0] Switch Target (Left)
        (if (Variables|/Game/Blueprints/Component/BPC_TargetingSystem.BPC_TargetingSystem_C|GetisHardLock _targetingsystemref)
          (Default|LockonTarget(Left) _targetingsystemref))))))

(event Input|EnhancedActionEvents|EnhancedInputActionIA_SwitchTargetLeft
  (params (ActionValue :type Boolean) (ElapsedSeconds :type Float%20%28double-precision%29) (TriggeredSeconds :type Float%20%28double-precision%29) (InputAction :type Input%20Action%20Object%20Reference :default "/Game/Input/IA_SwitchTargetLeft.IA_SwitchTargetLeft"))
  (bind _targetingsystemref (Variables|Ref|GetTargetingSystemRef))
  ;[1 0.402 0] Switch Target (Left)
  (:Started
    (if (Variables|/Game/Blueprints/Component/BPC_TargetingSystem.BPC_TargetingSystem_C|GetisHardLock _targetingsystemref)
      (Default|LockonTarget(Left) _targetingsystemref))))

(event Custom|StayInAir
  (bind _playercharacterref (Variables|Ref|GetPlayerCharacterRef))
  (bind _returnvalue (Transformation|GetActorLocation _playercharacterref))
  (bind (_x _y _z) (Math|Vector|BreakVector _returnvalue))
  ;[1 1 1] Stay in Air if hit Enemy
  (bind _returnvalue_2 (Class|KismetSystemLibrary|LineTraceMultiforObjects _returnvalue (Math|Vector|MakeVector _x _y (- _z 1.2e+03)) (Utilities|Array|MakeArray "ObjectTypeQuery1" "ObjectTypeQuery2") false (Utilities|Array|MakeArray _playercharacterref) "None" true))
  (if _returnvalue_2
    (Character|LaunchCharacter (Variables|Ref|GetPlayerCharacterRef) "0.000000,0.000000,300.000000" true true)))

(event Custom|Hit%20Stop%20Zawarudo
  (params (Dilation :type Float%20%28double-precision%29) (Delay :type Float%20%28double-precision%29))
  ;[1 1 1] HitStop
  (Utilities|Time|SetGlobalTimeDilation Dilation)
  (Utilities|FlowControl|Delay Delay)
  (Utilities|Time|SetGlobalTimeDilation 1.0))

(event Input|EnhancedActionEvents|EnhancedInputActionIA_SwitchWeapon
  (params (ActionValue :type Boolean) (ElapsedSeconds :type Float%20%28double-precision%29) (TriggeredSeconds :type Float%20%28double-precision%29) (InputAction :type Input%20Action%20Object%20Reference :default "/Game/Input/IA_SwitchWeapon.IA_SwitchWeapon"))
  ;[1 1 1] Switch Weapon
  (|ToggleWeaponMode))

(event Input|EnhancedActionEvents|EnhancedInputActionIA_LightAtk
  (params (ActionValue :type Boolean) (ElapsedSeconds :type Float%20%28double-precision%29) (TriggeredSeconds :type Float%20%28double-precision%29) (InputAction :type Input%20Action%20Object%20Reference :default "/Game/Input/IA_LightAtk.IA_LightAtk"))
  ;[0 1 0.05978] Light Attack
  (:Started
    (if (CallFunction|IsonGround)
      ;;[1 1 1] Launch Requirement
      (if (and (Variables|/Game/Blueprints/Component/BPC_TargetingSystem.BPC_TargetingSystem_C|GetisHardLock (Variables|Ref|GetTargetingSystemRef)) (< (.y (Input|EnhancedActionValues|GetIA_Move)) 0.0))
        ;;[1 1 1] Launch Enemy
        (bind _returnvalue (Abilities|TryActivateAbilitiesbyTag (Variables|Ref|GetGASRef) (Variables|GasTag|Air|GetLaunchTag) true))
        (if _returnvalue
          (Target|ApplyTargetRotation))
        (else
          ;;[1 1 1] Chain Combo Requirement
          (if (GameplayTags|HasMatchingGameplayTag (Variables|Ref|GetGASRef) "(TagName=\"Attack.Combo.CW\")")
            ;;[1 1 1] Chain Attack
            (bind _returnvalue_2 (Abilities|TryActivateAbilitiesbyTag (Variables|Ref|GetGASRef) (Variables|GasTag|Chain|GetComboChainTag) true))
            (if _returnvalue_2
              (Target|ApplyTargetRotation))
            (else
              ;;[1 1 1] Basic Light Combo
              (bind _returnvalue_3 (Abilities|TryActivateAbilitiesbyTag (Variables|Ref|GetGASRef) (Variables|GasTag|Ground|GetGroundLAtkTag) true))
              (if _returnvalue_3
                (Target|ApplyTargetRotation))))))
      (else
        ;;[1 1 1] Air Attack
        (bind _returnvalue_4 (Abilities|TryActivateAbilitiesbyTag (Variables|Ref|GetGASRef) (Variables|GasTag|Air|GetAirLAtkTag) true))
        (if _returnvalue_4
          (Target|ApplyTargetRotation))))))

(event Input|EnhancedActionEvents|EnhancedInputActionIA_HeavyAtk
  (params (ActionValue :type Boolean) (ElapsedSeconds :type Float%20%28double-precision%29) (TriggeredSeconds :type Float%20%28double-precision%29) (InputAction :type Input%20Action%20Object%20Reference :default "/Game/Input/IA_HeavyAtk.IA_HeavyAtk"))
  ;[1 0.04575 0] Heavy
  (:Started
    (if (CallFunction|IsonGround)
      ;;[1 1 1] Chain Combo Requirement
      (if (GameplayTags|HasMatchingGameplayTag (Variables|Ref|GetGASRef) "(TagName=\"Attack.Combo.CW\")")
        ;;[1 1 1] Chain Attack
        (bind _returnvalue (Abilities|TryActivateAbilitiesbyTag (Variables|Ref|GetGASRef) (Variables|GasTag|Chain|GetComboChainTag) true))
        (if _returnvalue
          (Target|ApplyTargetRotation))
        (else
          ;;[1 1 1] Basic Heavy Combo
          (bind _returnvalue_2 (Abilities|TryActivateAbilitiesbyTag (Variables|Ref|GetGASRef) (Variables|GasTag|Ground|GetGroundHAtkTag) true))
          (if _returnvalue_2
            (Target|ApplyTargetRotation))))
      (else
        ;;[1 1 1] Slam Down
        (bind _returnvalue_3 (Abilities|TryActivateAbilitiesbyTag (Variables|Ref|GetGASRef) (Variables|GasTag|Air|GetSlamTag) true))
        (if _returnvalue_3
          (Target|ApplyTargetRotation))))))

(event EventGASSetIsSlam
  (params (isSlam :type Boolean))
  ;[1 0.04575 0] Heavy
  ;;[1 1 1] Slam Down
  (Variables|Default|SetisSlam isSlam))

(event EventGASSetLAttackIndex
  (params (LAtkIndex :type Integer))
  ;[0 0.03429 1] Interfaces
  (Variables|Default|SetCurrentLAtkStage LAtkIndex))

(event EventGASWeaponCollision
  (params (End :type Float%20%28double-precision%29) (Radius :type Float%20%28double-precision%29) (DamageAmount :type Float%20%28double-precision%29))
  ;[0 0.03429 1] Interfaces
  ;;[1 1 1] Collision
  (Attack|WeaponCollision Radius End DamageAmount))

(event EventGASSetHAttackIndex
  (params (HAtkIndex :type Integer))
  ;[0 0.03429 1] Interfaces
  (Variables|Default|SetCurrentHAtkStage HAtkIndex))

(event Input|KeyboardEvents|DebugKeyEquals
  (params (Key :type Key%20Structure :default "None") (ActionValue :type Input%20Action%20Value%20Structure))
  ;[0 1 0.06027] GAS Debug
  (:Pressed
    (Utilities|FlowControl|FlipFlop
      (:A
        (Development|ExecuteConsoleCommand "ShowDebug AbilitySystem" 0))
      (:B
        (Development|ExecuteConsoleCommand "ShowDebug None" 0)))))

(fn ConstructionScript)

(fn IsonGround
  (return (not (AI|Components|NavMovement|IsFalling (Variables|/Script/Engine.Character|GetCharacterMovement (Variables|Ref|GetPlayerCharacterRef))))))

(fn SetState
  (params (CurrentState :type E_MCState%20Enum :default "NewEnumerator0"))
  (if (Utilities|Enum|NotEqual(Enum) CurrentState (Variables|FSM|GeteMcState))
    (Variables|FSM|SeteMcState CurrentState)))

(fn GetState
  (return (Variables|FSM|GeteMcState)))

(fn IsCurrentStateEqualtoAny
  (params (States%20to%20Check :type Array%20of%20E_MCState%20Enums :default "NewEnumerator0"))
  (return (Utilities|Array|ContainsItem States%20to%20Check (Variables|FSM|GeteMcState))))

(fn CanAttack
  (return (and (not (FSM|IsCurrentStateEqualtoAny (Utilities|Array|MakeArray "NewEnumerator1" "NewEnumerator2" "NewEnumerator3" "NewEnumerator4"))) (CallFunction|IsonGround))))

(fn GetDesireRotation
  (bind _playercharacterref (Variables|Ref|GetPlayerCharacterRef))
  (bind _charactermovement (Variables|/Script/Engine.Character|GetCharacterMovement _playercharacterref))
  (bind _returnvalue (Pawn|Components|PawnMovement|GetLastInputVector _charactermovement))
  (return (Math|Rotator|SelectRotator (Math|Conversions|RotationFromXVector _returnvalue) "0, 0, 0" (Utilities|Operators|NotEqual(!=) :A _returnvalue))))

(fn WeaponCollision
  (params (Radius :type Float%20%28single-precision%29) (End :type Float%20%28single-precision%29) (DamageAmount :type Float%20%28double-precision%29))
  (bind _playercharacterref (Variables|Ref|GetPlayerCharacterRef))
  (bind _targetingsystemref (Variables|Ref|GetTargetingSystemRef))
  (bind _returnvalue (Transformation|GetActorLocation _playercharacterref))
  (LocalVariables|SetDmgDealt DamageAmount)
  (Utilities|Array|Clear (Variables|Attack|GetHitEnemy))
  (bind (_outhits _returnvalue_2) (Collision|MultiSphereTraceForObjects _returnvalue (+ (* (Transformation|GetActorForwardVector _playercharacterref) End) _returnvalue) Radius (Utilities|Array|MakeArray "ObjectTypeQuery3") true 0 "None"))
  (if _returnvalue_2
    (for _array_element _outhits
      (if (not (Utilities|Array|ContainsItem (Variables|Attack|GetHitEnemy) (.HitActor (Collision|BreakHitResult _array_element))))
        (if (Utilities|ClassIsChildOf (Utilities|GetClass (.HitActor (Collision|BreakHitResult _array_element))) "/Game/AI/Blueprints/BP_Demon_Base.BP_Demon_Base_C")
          (bind _dmgsyscomponent (Class|BPIDamagable|DmgGetDmgSysComponent(Message) (.HitActor (Collision|BreakHitResult _array_element))))
          (if (not (Variables|/Game/Blueprints/Health_Damage_System/BPC_DamageSystem.BPC_DamageSystem_C|GetisDead _dmgsyscomponent))
            (Utilities|Array|AddUnique (Variables|Attack|GetHitEnemy) (.HitActor (Collision|BreakHitResult _array_element)))
            (Default|DamageEnemy (Variables|Ref|GetPlayerCharacterRef) (.HitActor (Collision|BreakHitResult _array_element)) (LocalVariables|GetDmgDealt))
            (if (GameplayTags|HasMatchingGameplayTag (Ability|GetAbilitySystemComponent (.HitActor (Collision|BreakHitResult _array_element))) "(TagName=\"Attack.Enemy.Parryable\")")
              (Abilities|TryActivateAbilitiesbyTag (Variables|Ref|GetGASRef) (Variables|GasTag|GetParryTag) true)
              (Default|DamageEnemy (Variables|Ref|GetPlayerCharacterRef) (.HitActor (Collision|BreakHitResult _array_element)) (* (LocalVariables|GetDmgDealt) 2.0))
              (Camera|PlayWorldCameraShake "/Game/GAS/CamShake.CamShake_C" (Transformation|GetActorLocation (Variables|Ref|GetPlayerCharacterRef)) 5e+02 1e+03)
              (CallFunction|HitStopZawarudo 0.2 0.1))
            (if (Variables|/Game/Blueprints/Component/BPC_TargetingSystem.BPC_TargetingSystem_C|GetisHardLock _targetingsystemref)
              (if (CallFunction|IsonGround)
                (Variables|Default|SetlaunchedHit true)
                (elif (GameplayTags|HasMatchingGameplayTag (Variables|Ref|GetGASRef) "(TagName=\"Attack.Air.Slam\")")
                  (Variables|Default|SetisSlam true)
                  (else
                    (CallFunction|StayinAir))))
              (elif (Variables|/Game/Blueprints/Component/BPC_TargetingSystem.BPC_TargetingSystem_C|GetisSoftLock _targetingsystemref)
                (Class|BPIDemon|ToggleLockVisual(Message) (Variables|/Game/Blueprints/Component/BPC_TargetingSystem.BPC_TargetingSystem_C|GetSoftLockedOnActor (Variables|Ref|GetTargetingSystemRef)) true (Utilities|Struct|MakeSlateColor "(R=1.000000,G=1.000000,B=0.223228,A=1.000000)"))))))))))

(fn ApplyTargetRotation
  (bind _targetingsystemref (Variables|Ref|GetTargetingSystemRef))
  (if (Variables|/Game/Blueprints/Component/BPC_TargetingSystem.BPC_TargetingSystem_C|GetisHardLock _targetingsystemref)
    (CallFunction|RotatetoTarget)
    (else
      (Default|SoftLockonTarget (Variables|Ref|GetTargetingSystemRef))
      (if (Variables|/Game/Blueprints/Component/BPC_TargetingSystem.BPC_TargetingSystem_C|GetisSoftLock _targetingsystemref)
        (CallFunction|RotatetoTarget)))))

(fn IsController
  (params (XAxisInput :type Float%20%28double-precision%29))
  (return (and (Utilities|Enum|Equal(Enum) (.PrimaryDeviceType (Utilities|Struct|BreakHardwareDeviceIdentifier (Class|InputDeviceSubsystem|GetInputDeviceHardwareIdentifier (|InputDeviceSubsystem)))) "Gamepad") (> (Math|Float|Absolute(Float) XAxisInput) 0.1))))

(fn ThumbStickRight
  (params (X :type Float%20%28double-precision%29) (Y :type Float%20%28double-precision%29))
  (bind _returnvalue (Class|KismetMathLibrary|DegAtan2 Y X))
  (return (and (> _returnvalue -45.0) (< _returnvalue 45.0))))

(fn ThumbStickLeft
  (params (X :type Float%20%28double-precision%29) (Y :type Float%20%28double-precision%29))
  (bind _returnvalue (Class|KismetMathLibrary|DegAtan2 Y X))
  (return (or (> _returnvalue 135.0) (< _returnvalue -135.0))))

(fn GASGetIsFalling
  (return false))

(fn GASGetIsSlam
  (return (Variables|Default|GetisSlam)))

(fn GASGetMcRef
  (return 0))

(fn GASGetTargetingSystem
  (return 0))

(fn MCCGetHUDRef
  (return (Variables|Ref|GetHUDRef)))

(fn MCCStateCheck
  (return (FSM|IsCurrentStateEqualtoAny (Utilities|Array|MakeArray "NewEnumerator0"))))

(fn PCWMGetBaseUIWidget
  (return (Variables|UI|GetBaseUIWidget)))