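; Game instance that holds the player's save game, background music and sound volume settings for the game.
; Loading reads the SG_SaveGame slot, or creates a new, not yet written save object if none exists.
; GI-prefixed events and getters expose the save, volume array and audio controls.
; Music plays as a stored 2D sound, optionally persisting across levels; stopping calls Stop immediately after starting the fade-out.
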(event Custom|LoadPlayerSaveGame
  (bind _slotname (Variables|Save|GetSlotName))
  ;[1 1 1] Load Player save, if not exist create new save
  (bind _returnvalue (SaveGame|DoesSaveGameExist _slotname))
  (if _returnvalue
    (bind _returnvalue_2 (SaveGame|LoadGamefromSlot _slotname))
    (bind _assg_save_game (Utilities|Casting|CastToSG_SaveGame _returnvalue_2))
    (Variables|Save|SetSaveGame _assg_save_game)
    (Development|PrintString "Save Loaded")
    (else
      (bind _returnvalue_3 (SaveGame|CreateSaveGameObject "/Game/SaveGame/SG_SaveGame.SG_SaveGame_C"))
      (Variables|Save|SetSaveGame _returnvalue_3)
      (Development|PrintString "Create New Save"))))

(event EventGIPlayStartSFX
  ;[1 1 1] Volume
  (CallFunction|GameStartSFX))

(event EventGIStopAudio
  ;[1 1 1] Volume
  (CallFunction|StopBGM))

(event EventGISetVolumeArray
  (params (Volume :type Array%20of%20Floats%20%28double-precision%29))
  ;[1 1 1] Volume
  (Variables|Sound|SetSoundVolume Volume))

(event EventGIPlayAudio
  (params (Audio :type Sound%20Base%20Object%20Reference) (Volume :type Float%20%28double-precision%29) (Persist :type Boolean))
  ;[1 1 1] Volume
  (CallFunction|PlayBGM Audio Volume Persist))

(fn PlayBGM
  (params (Audio :type Sound%20Base%20Object%20Reference) (Volume :type Float%20%28double-precision%29) (bPersistAcrossLevelTransition :type Boolean))
  (bind _returnvalue (Audio|CreateSound2D Audio Volume 1.0 0.0 0 bPersistAcrossLevelTransition))
  (bind _output_get (Variables|Default|SetAudio _returnvalue))
  (Audio|Components|Audio|FadeIn _output_get 1.0 1.0 0.0 "Linear" :!class /Script/Engine.AudioComponent)
  (Audio|Components|Audio|Play _output_get 0.0))

(fn StopBGM
  (bind _audio (Variables|Default|GetAudio))
  (Audio|Components|Audio|FadeOut _audio 1.0 0.0 "Linear" :!class /Script/Engine.AudioComponent)
  (Audio|Components|Audio|Stop _audio))

(fn GameStartSFX
  (bind _returnvalue (Audio|CreateSound2D 0 1.0 1.0 0.0 0))
  (Audio|Components|Audio|FadeIn _returnvalue 1.0 1.0 0.0 "Linear" :!class /Script/Engine.AudioComponent)
  (Audio|Components|Audio|Play _returnvalue 0.0)
  (Audio|Components|Audio|FadeOut _returnvalue 4.0 0.0 "Linear" :!class /Script/Engine.AudioComponent))

(fn GIGetSaveGame
  (return (Variables|Save|GetSaveGame)))

(fn GIGetVolumeArray
  (return (Variables|Sound|GetSoundVolume)))