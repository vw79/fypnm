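; Actor component holding enemy attack routines for mage, melee, shielder and Titan characters, dealing damage through TakeDamage messages.
; Melee attacks play the supplied montage, sphere-trace for Player-tagged pawns on a notify, and message the owner about attack state and interruptibility.
; Magic attacks bind projectile impacts, while Titan lightning, stomp and beam attacks spawn warning or AOE actors and bind their overlaps to damage, with stomp adding launch and camera shake.
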(event Custom|Sphere%20Trace%20Damage
  (params (DamageInfo :type S%20Damage%20Info%20Structure))
  (bind _returnvalue (Components|GetOwner))
  (bind _player (Variables|Default|Getplayer))
  (bind _returnvalue_2 (Transformation|GetActorLocation _returnvalue))
  ;[1 1 1] SPHERE TRACE DAMAGE
  (Utilities|Array|Clear (Variables|Default|Getplayer))
  (bind (_outhits _returnvalue_3) (Collision|MultiSphereTraceForObjects _returnvalue_2 (+ _returnvalue_2 (* (Transformation|GetActorForwardVector _returnvalue) 1e+02)) 0.0 (Utilities|Array|MakeArray "ObjectTypeQuery3") false 0 "None"))
  (if _returnvalue_3
    (for _array_element _outhits
      (if (Actor|ActorHasTag (.HitActor (Collision|BreakHitResult _array_element)) "Player")
        (Utilities|Array|AddUnique _player (.HitActor (Collision|BreakHitResult _array_element)))))
    (Class|BPIDamagable|TakeDamage(Message) (Utilities|Array|Get(acopy) _player) DamageInfo (Components|GetOwner))))

(event Custom|Hit%20Impact
  (params (Other%20Actor :type Actor%20Object%20Reference) (Hit :type Hit%20Result%20Structure))
  ;[0.2781 0 0.2343] MAGE ATTACKS
  (Class|BPIDamagable|TakeDamage(Message) Other%20Actor (stale Custom|Magic%20Attack DamageInfo))
  (Class|AISenseDamage|ReportDamageEvent Other%20Actor (Components|GetOwner) (Utilities|Struct|BreakS_DamageInfo (stale Custom|Magic%20Attack DamageInfo)) (Transformation|GetActorLocation (Components|GetOwner)) "0, 0, 0" "None")
  (Default|CallOnAttackEnded))

(event Custom|AOE%20Damage
  (params (Attack%20Target :type Actor%20Object%20Reference) (Radius :type Float%20%28single-precision%29) (DamageInfo :type S%20Damage%20Info%20Structure))
  (bind _returnvalue (Components|GetOwner))
  (bind _returnvalue_2 (Actor|GetComponentbyClass _returnvalue "/Script/Engine.SkeletalMeshComponent"))
  ;[1 1 1] Attack Notifies
  (bind _returnvalue_3 (Game|SpawnActorfromClass "/Game/AI/Blueprints/Titan/BP_AOE_Base.BP_AOE_Base_C" (Math|Transform|MakeTransform (Transformation|GetSocketLocation _returnvalue_2 (Class|SkinnedMeshComponent|GetSocketBoneName _returnvalue_2 "foot_R")) "0, 0, 0" "1.000000,1.000000,1.000000") "Undefined" "MultiplyWithRoot" 0 0))
  (Variables|/Game/AI/Blueprints/Titan/BP_AOE_Base.BP_AOE_Base_C|SetRadius _returnvalue_3 Radius)
  (EventDispatchers|BindEventtoOnAOEOverlapActor _returnvalue_3 (delegate Custom|Launch%20Player))
  (Default|Trigger _returnvalue_3)
  (Utilities|FlowControl|Delay 3.0)
  (Actor|DestroyActor _returnvalue_3))

(event Custom|Launch%20Player
  (params (Actor :type Actor%20Object%20Reference))
  ;[1 1 1] Attack Notifies
  (if (== Actor (stale Custom|AOE%20Damage Attack%20Target))
    (Character|LaunchCharacter (Game|GetPlayerCharacter 0) "0.000000,1000.000000,350.000000" true true)
    (Class|BPIDamagable|TakeDamage(Message) Actor (stale Custom|AOE%20Damage DamageInfo))))

(event Custom|Dual%20Claw%20Slash
  (params (Attack%20Info :type S%20Attacks%20Structure))
  (bind (_attacktarget _montage _damageinfo) (Utilities|Struct|BreakS_Attacks Attack%20Info))
  (bind _returnvalue (Components|GetOwner))
  (bind _returnvalue_2 (Components|GetOwner))
  ;[1 0.9804 0] MELEE ATTACKS
  (Class|BPIDemon|Attack(Message) _returnvalue_2 _attacktarget)
  (bind _notifyname (Animation|Montage|PlayMontage (Actor|GetComponentbyClass _returnvalue_2 "/Script/Engine.SkeletalMeshComponent") _montage)
    (:then
      (Class|BPIDamagable|SetIsInterruptible(Message) _returnvalue false))
    (:OnCompleted
      (Class|BPIDemon|FinishAttacking(Message) _returnvalue _attacktarget :!label _label)
      (Class|BPIDamagable|SetIsInterruptible(Message) _returnvalue true))
    (:OnInterrupted
      (goto _label))
    (:OnNotifyEnd
      (switch name _notifyname
        (:Dual%20Slash
          (CallFunction|SphereTraceDamage _damageinfo))))))

(event Custom|Heavy%20Attack
  (params (Attack%20Info :type S%20Attacks%20Structure))
  (bind (_attacktarget _montage _damageinfo) (Utilities|Struct|BreakS_Attacks Attack%20Info))
  (bind _returnvalue (Components|GetOwner))
  (bind _returnvalue_2 (Components|GetOwner))
  ;[0 1 0.9307] Shielder Attacks
  (Class|BPIDemon|Attack(Message) _returnvalue _attacktarget)
  (bind _notifyname (Animation|Montage|PlayMontage (Actor|GetComponentbyClass _returnvalue "/Script/Engine.SkeletalMeshComponent") _montage)
    (:then
      (Class|BPIDamagable|SetIsInterruptible(Message) _returnvalue_2 true))
    (:OnCompleted
      (Class|BPIDemon|FinishAttacking(Message) _returnvalue_2 _attacktarget :!label _label)
      (Class|BPIDamagable|SetIsInterruptible(Message) _returnvalue_2 true))
    (:OnInterrupted
      (goto _label))
    (:OnNotifyEnd
      (switch name _notifyname
        (:Heavy
          (CallFunction|SphereTraceDamage _damageinfo))))))

(event Custom|Beam%20Impact
  (params (Attacks :type S%20Attacks%20Structure))
  (bind _returnvalue (Components|GetOwner))
  (bind (_aspawn _bsuccess) (Utilities|Casting|CastToPawn _returnvalue))
  ;[1 1 1] TITAN ATACKS
  (bind _returnvalue_2 (Game|SpawnActorfromClass "/Game/AI/Blueprints/Titan/BP_AOE_BeamImpact.BP_AOE_BeamImpact_C" (Math|Transform|MakeTransform "0, 0, 0" "0, 0, 0" "1.000000,1.000000,1.000000") "Undefined" "MultiplyWithRoot" 0 0.1 (select _bsuccess _aspawn 0)))
  (EventDispatchers|BindEventtoOnAOEOverlapActor _returnvalue_2 (delegate Custom|Damage))
  (Default|Trigger _returnvalue_2))

(event Custom|Damage
  (params (Actor :type Actor%20Object%20Reference))
  ;[1 1 1] TITAN ATACKS
  (if (== Actor (.AttackTarget (Utilities|Struct|BreakS_Attacks (stale Custom|Beam%20Impact Attacks))))
    (Class|BPIDamagable|TakeDamage(Message) Actor (Utilities|Struct|MakeS_DamageInfo 1e+01 "NewEnumerator3") (Components|GetOwner))))

(event Custom|Stomp%20Attack
  (params (Attacks :type S%20Attacks%20Structure) (Radius :type Float%20%28single-precision%29))
  (bind (_attacktarget _montage _damageinfo) (Utilities|Struct|BreakS_Attacks Attacks))
  (bind _returnvalue (Components|GetOwner))
  (bind _returnvalue_2 (Components|GetOwner))
  ;[1 1 1] TITAN ATACKS
  ;;[0.224 0.1153 0] Stomp Attack
  (Class|BPIDemon|Attack(Message) _returnvalue_2 _attacktarget)
  (bind _notifyname (Animation|Montage|PlayMontage (Actor|GetComponentbyClass _returnvalue_2 "/Script/Engine.SkeletalMeshComponent") _montage)
    (:then
      (Class|BPIDamagable|SetIsInterruptible(Message) _returnvalue false)
      (AI|ClearFocus (AI|GetAIController _returnvalue))
      (Game|SpawnActorfromClass "/Game/AI/Blueprints/Titan/BP_StompWarning.BP_StompWarning_C" (Math|Transform|MakeTransform "0, 0, 0" "0, 0, 0" "1.000000,1.000000,1.000000") "Undefined" "MultiplyWithRoot" 0 _attacktarget 0))
    (:OnCompleted
      (Class|BPIDemon|FinishAttacking(Message) _returnvalue _attacktarget :!label _label)
      (Class|BPIDamagable|SetIsInterruptible(Message) _returnvalue true))
    (:OnInterrupted
      (goto _label))
    (:OnNotifyEnd
      (switch name _notifyname
        (:Stomp
          (CallFunction|AOEDamage _attacktarget Radius _damageinfo)
          (Camera|PlayWorldCameraShake "/Game/AI/Blueprints/Titan/BP_CameraShake.BP_CameraShake_C" (Transformation|GetActorLocation _returnvalue) 0.0 2.8e+03))))))

(event Custom|Magic%20Attack
  (params (Spawn%20Transform :type Transform) (DamageInfo :type S%20Damage%20Info%20Structure) (Target :type Actor%20Object%20Reference))
  ;[0.2781 0 0.2343] MAGE ATTACKS
  (bind _returnvalue (Game|SpawnActorfromClass "/Game/AI/Blueprints/Magic_Demon/BP_Projectile.BP_Projectile_C" Spawn%20Transform "Undefined" "MultiplyWithRoot" (Components|GetOwner) 0))
  (EventDispatchers|AssignOnProjectileImpact _returnvalue (delegate Custom|Hit%20Impact)))

(event Custom|Lightning%20Strike
  (params (Attack%20Target :type Actor%20Object%20Reference) (Attacks :type S%20Attacks%20Structure))
  (bind (_attacktarget _montage) (Utilities|Struct|BreakS_Attacks Attacks))
  (bind _returnvalue (Components|GetOwner))
  (bind _returnvalue_2 (Components|GetOwner))
  (bind _returnvalue_3 (AI|GetAIController _returnvalue))
  (bind (_aspawn _bsuccess) (Utilities|Casting|CastToPawn _returnvalue_2))
  ;[1 1 1] TITAN ATACKS
  ;;[1 0.9344 0] Lightining Strike
  (bind _notifyname (Animation|Montage|PlayMontage (Actor|GetComponentbyClass (Components|GetOwner) "/Script/Engine.SkeletalMeshComponent") _montage)
    (:then
      (AI|ClearFocus _returnvalue_3))
    (:OnCompleted
      (Class|BPIDemon|FinishAttacking(Message) _returnvalue _attacktarget :!label _label)
      (AI|SetFocus _returnvalue_3 _attacktarget))
    (:OnInterrupted
      (goto _label))
    (:OnNotifyBegin
      (switch name _notifyname
        (:Strike
          (bind _returnvalue_4 (Game|SpawnActorfromClass "/Game/AI/Blueprints/Titan/BP_StompWarning.BP_StompWarning_C" (Math|Transform|MakeTransform "0, 0, 0" "0, 0, 0" "1.000000,1.000000,1.000000") "Undefined" "MultiplyWithRoot" 0 Attack%20Target (select _bsuccess _aspawn 0)))
          (EventDispatchers|BindEventtoOnAOEOverlapActor _returnvalue_4 (delegate Custom|Damage%20Player)))))))

(event Custom|Push%20Player
  (params (Actor :type Actor%20Object%20Reference))
  (bind _returnvalue (Game|GetPlayerCharacter 0))
  ;[1 1 1] Keep This Just in Case the current Stomp Attack suddenly bugs out
  (Character|LaunchCharacter _returnvalue "0.000000,1500.000000,900.000000" true true)
  (Class|BPIDamagable|TakeDamage(Message) _returnvalue (Utilities|Struct|MakeS_DamageInfo 4e+01 "NewEnumerator1")))

(event Custom|Damage%20Player
  (params (Actor :type Actor%20Object%20Reference))
  ;[1 1 1] TITAN ATACKS
  ;;[1 0.9344 0] Lightining Strike
  (Class|BPIDamagable|TakeDamage(Message) Actor (Utilities|Struct|MakeS_DamageInfo 3e+01 "NewEnumerator3")))

(event Custom|360%20Attack
  (params (Attack%20Info :type S%20Attacks%20Structure))
  (bind (_attacktarget _montage) (Utilities|Struct|BreakS_Attacks Attack%20Info))
  (bind _returnvalue (Components|GetOwner))
  (bind _returnvalue_2 (Components|GetOwner))
  ;[1 0.9804 0] MELEE ATTACKS
  (Class|BPIDemon|Attack(Message) _returnvalue_2 _attacktarget)
  (bind _notifyname (Animation|Montage|PlayMontage (Actor|GetComponentbyClass _returnvalue_2 "/Script/Engine.SkeletalMeshComponent") _montage)
    (:then
      (Class|BPIDamagable|SetIsInterruptible(Message) _returnvalue false))
    (:OnCompleted
      (Class|BPIDemon|FinishAttacking(Message) _returnvalue _attacktarget :!label _label)
      (Class|BPIDamagable|SetIsInterruptible(Message) _returnvalue true))
    (:OnInterrupted
      (goto _label))
    (:OnNotifyBegin
      (switch name _notifyname
        (:360%20Attack
          (CallFunction|SphereTraceDamage (Utilities|Struct|MakeS_DamageInfo 1e+01 "NewEnumerator1")))))))

(event Custom|Claw%20Slash
  (params (Attack%20Info :type S%20Attacks%20Structure))
  (bind (_attacktarget _montage _damageinfo) (Utilities|Struct|BreakS_Attacks Attack%20Info))
  (bind _returnvalue (Components|GetOwner))
  (bind _returnvalue_2 (Components|GetOwner))
  ;[1 0.9804 0] MELEE ATTACKS
  (Class|BPIDemon|Attack(Message) _returnvalue_2 _attacktarget)
  (bind _notifyname (Animation|Montage|PlayMontage (Actor|GetComponentbyClass _returnvalue_2 "/Script/Engine.SkeletalMeshComponent") _montage 0.7)
    (:then
      (Class|BPIDamagable|SetIsInterruptible(Message) _returnvalue true))
    (:OnCompleted
      (Class|BPIDemon|FinishAttacking(Message) _returnvalue _attacktarget :!label _label)
      (Class|BPIDamagable|SetIsInterruptible(Message) _returnvalue true))
    (:OnInterrupted
      (goto _label))
    (:OnNotifyEnd
      (switch name _notifyname
        (:Claw%20Slash
          (CallFunction|SphereTraceDamage _damageinfo))))))

(event Custom|Swing%20Attack
  (params (Attack%20Info :type S%20Attacks%20Structure))
  (bind (_attacktarget _montage _damageinfo) (Utilities|Struct|BreakS_Attacks Attack%20Info))
  (bind _returnvalue (Components|GetOwner))
  (bind _returnvalue_2 (Components|GetOwner))
  ;[0 1 0.9307] Shielder Attacks
  (Class|BPIDemon|Attack(Message) _returnvalue _attacktarget)
  (bind _notifyname (Animation|Montage|PlayMontage (Actor|GetComponentbyClass _returnvalue "/Script/Engine.SkeletalMeshComponent") _montage)
    (:then
      (Class|BPIDamagable|SetIsInterruptible(Message) _returnvalue_2 true))
    (:OnCompleted
      (Class|BPIDemon|FinishAttacking(Message) _returnvalue_2 _attacktarget :!label _label)
      (Class|BPIDamagable|SetIsInterruptible(Message) _returnvalue_2 true))
    (:OnInterrupted
      (goto _label))
    (:OnNotifyEnd
      (switch name _notifyname
        (:Swing
          (CallFunction|SphereTraceDamage _damageinfo))))))

(fn DamageAllNonTeamMembers
  (params (Hits :type Array%20of%20Hit%20Result%20Structures) (DamageInfo :type S%20Damage%20Info%20Structure))
  (for _array_element Hits
    (bind _team_number (Class|BPIDamagable|GetTeamNumber(Message) (.HitActor (Collision|BreakHitResult _array_element))))
    (bind _team_number_2 (Class|BPIDamagable|GetTeamNumber(Message) (Components|GetOwner)))
    (if (and (!= _team_number_2 _team_number) (not (Utilities|Array|ContainsItem (LocalVariables|GetActors%20Damaged%20So%20Far) (.HitActor (Collision|BreakHitResult _array_element)))))
      (Class|BPIDamagable|TakeDamage(Message) (.HitActor (Collision|BreakHitResult _array_element)) DamageInfo (Components|GetOwner))
      (Utilities|Array|AddUnique (LocalVariables|GetActors%20Damaged%20So%20Far) (.HitActor (Collision|BreakHitResult _array_element)))))
  (return (LocalVariables|GetActors%20Damaged%20So%20Far)))