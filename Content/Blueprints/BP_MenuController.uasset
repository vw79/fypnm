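; Player controller for the main menu that creates the base UI layout widget and acts as the entry point for pushing menus and prompts onto it.
; On the Main Menu level it runs the settings widget's start logic, switches to UI-only input with a cursor and pushes the first menu.
; It binds to prompt confirm and cancel events on a level-placed binder actor, forwarding results to the active menu-stack widget.
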(event Custom|Bindings
  (bind _masterbinderui (Variables|Default|GetMasterBinderUI))
  ;[1 1 1] Prompt
  ;;[1 1 1] Bindings
  (EventDispatchers|BindEventtoOnPromptConfirmed _masterbinderui (delegate Custom|OnPromptConfirmed_Event))
  (EventDispatchers|BindEventtoOnPromptCanceled _masterbinderui (delegate Custom|OnPromptCanceled_Event)))

(event Custom|OnPromptCanceled_Event
  (params (PromptIndex :type UI_PromptIndex%20Enum :default "NewEnumerator0") (PromptToStack :type UI_PromptToStack%20Enum :default "NewEnumerator0"))
  ;[1 1 1] Prompt
  ;;[1 1 1] Bindings
  (switch Utilities|FlowControl|Switch|SwitchonUI_PromptToStack PromptToStack
    (:NewEnumerator0
      _)
    (:NewEnumerator1
      _))
  (Class|BPIPromptInterface|PromptCanceled(Message) (Class|CommonActivatableWidgetContainerBase|GetActiveWidget (Variables|/Game/Widgets/AWB/AWB_BaseUILayout.AWB_BaseUILayout_C|GetMenuStack (Variables|Default|GetBaseUIWidget))) PromptIndex))

(event Custom|OnPromptConfirmed_Event
  (params (PromptIndex :type UI_PromptIndex%20Enum :default "NewEnumerator0") (PromptToStack :type UI_PromptToStack%20Enum :default "NewEnumerator0"))
  ;[1 1 1] Prompt
  ;;[1 1 1] Bindings
  (switch Utilities|FlowControl|Switch|SwitchonUI_PromptToStack PromptToStack
    (:NewEnumerator0
      _)
    (:NewEnumerator1
      _))
  (Class|BPIPromptInterface|PromptConfirmed(Message) (Class|CommonActivatableWidgetContainerBase|GetActiveWidget (Variables|/Game/Widgets/AWB/AWB_BaseUILayout.AWB_BaseUILayout_C|GetMenuStack (Variables|Default|GetBaseUIWidget))) PromptIndex))

(event EventBeginPlay
  (bind _self self)
  ;[1 1 1] Event Begin Setup
  (bind _returnvalue (UserInterface|CreateWidget "/Game/Widgets/AWB/AWB_BaseUILayout.AWB_BaseUILayout_C" self))
  (bind _output_get (Variables|Default|SetBaseUIWidget _returnvalue))
  (UserInterface|Viewport|AddtoViewport _output_get 0)
  (bind _returnvalue_2 (Game|GetCurrentLevelName true))
  (switch string _returnvalue_2
    (:MainMenu
      (bind _returnvalue_3 (UserInterface|CreateWidget "/Game/Widgets/AWB/Settings/AWB_Settings.AWB_Settings_C" _self))
      (Default|OnGameStart _returnvalue_3)
      (Input|SetInputModeUIOnly _self 0 "DoNotLock" false)
      (Variables|/Script/Engine.PlayerController|SetbShowMouseCursor _self true)
      (Default|PushMenu (Variables|Default|GetBaseUIWidget) "/Game/Widgets/AWB/AWB_FirstMenu.AWB_FirstMenu_C")
      (bind _returnvalue_4 (Actor|GetActorOfClass "/Game/Blueprints/BP_MasterBinderUI.BP_MasterBinderUI_C"))
      (Variables|Default|SetMasterBinderUI _returnvalue_4)
      (CallFunction|Bindings))))

(event EventPCWMPushMenuPrompt
  (params (PromptText :type Text) (PromptIndex :type UI_PromptIndex%20Enum :default "NewEnumerator0") (PromptToStack :type UI_PromptToStack%20Enum :default "NewEnumerator0"))
  ;[1 1 1] Prompt
  ;;[1 1 1] Menu Prompt With Custom Prompt (Quit)
  (Default|PushMenuPrompt (Variables|Default|GetBaseUIWidget) PromptIndex PromptToStack PromptText))

(event EventPCWMPushMenu
  (params (ActivatableWidget :type Common%20Activatable%20Widget%20Class%20Reference))
  ;[1 1 1] Push Any AWB Menu
  (Default|PushMenu (Variables|Default|GetBaseUIWidget) ActivatableWidget))

(fn ConstructionScript)

(fn PCWMGetBaseUIWidget
  (return (Variables|Default|GetBaseUIWidget)))

(fn PCWMGetHudRef
  (return 0))