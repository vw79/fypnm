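; BP_FootSteps is an animation notify that plays surface-dependent footstep sounds.
; When triggered, it line-traces on the Visibility channel from the mesh owner's location down along its negative up vector.
; The hit's physical surface type selects the Road or Tiles sound, played non-spatialized with PlaySound2D.
; The branch after the trace is hard-wired true, so the trace result is not checked before the surface lookup.
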(fn ReceivedNotify
  (params (MeshComp :type Skeletal%20Mesh%20Component%20Object%20Reference) (Animation :type Anim%20Sequence%20Base%20Object%20Reference) (EventReference :type Anim%20Notify%20Event%20Reference%20Structure%20%28by%20ref%29))
  (bind _returnvalue (Components|GetOwner MeshComp))
  (bind _returnvalue_2 (Transformation|GetActorLocation _returnvalue))
  (bind _outhit (Collision|LineTraceByChannel _returnvalue_2 (+ _returnvalue_2 (* (Transformation|GetActorUpVector _returnvalue) -2e+02)) "TraceTypeQuery1" false 0 "None"))
  (if true
    (switch Utilities|FlowControl|Switch|SwitchonEPhysicalSurface (Collision|GetSurfaceType _outhit)
      (:SurfaceType1
        (Audio|PlaySound2D "/Game/SFX/SoundCue/FootSteps_Road.FootSteps_Road" 1.0 1.0 0.0 0 0))
      (:SurfaceType2
        (Audio|PlaySound2D "/Game/SFX/SoundCue/FootSteps_Tiles.FootSteps_Tiles" 1.0 1.0 0.0 0 0))))
  (return false))