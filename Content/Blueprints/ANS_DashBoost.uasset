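; ANS_DashBoost is an animation notify state that marks a dash boost timing window during an animation.
; On begin it records the start time and timing data on the game state, reached through interface messages, and each tick asks the game state to check the boost.
; On end it removes the reset gameplay tags from the main character and clears the boost data.
; Indicator FX toggles are present but unwired.
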(fn ReceivedNotifyBegin
  (params (MeshComp :type Skeletal%20Mesh%20Component%20Object%20Reference) (Animation :type Anim%20Sequence%20Base%20Object%20Reference) (TotalDuration :type Float%20%28single-precision%29) (EventReference :type Anim%20Notify%20Event%20Reference%20Structure%20%28by%20ref%29))
  (bind _returnvalue (Components|GetOwner MeshComp))
  (bind _gamestate (Class|BPIMCGameState|MCGSGetGameState(Message) (Game|GetGameState _returnvalue)))
  (bind _mc (Class|BPIGAS|GASGetMcRef(Message) _returnvalue))
  (Default|SetDashBoostData _gamestate (Utilities|Time|GetGameTimeinSeconds _returnvalue) (Variables|Default|GetDashBoostTiming))
  (return true))

(fn ReceivedNotifyEnd
  (params (MeshComp :type Skeletal%20Mesh%20Component%20Object%20Reference) (Animation :type Anim%20Sequence%20Base%20Object%20Reference) (EventReference :type Anim%20Notify%20Event%20Reference%20Structure%20%28by%20ref%29))
  (bind _returnvalue (Components|GetOwner MeshComp))
  (bind _mc (Class|BPIGAS|GASGetMcRef(Message) _returnvalue))
  (Ability|GameplayEffect|RemoveLooseGameplayTags _mc (Variables|Default|GetResetTag))
  (bind _gamestate (Class|BPIMCGameState|MCGSGetGameState(Message) (Game|GetGameState _returnvalue)))
  (Default|ResetDashBoostData _gamestate)
  (return true))

(fn ReceivedNotifyTick
  (params (MeshComp :type Skeletal%20Mesh%20Component%20Object%20Reference) (Animation :type Anim%20Sequence%20Base%20Object%20Reference) (FrameDeltaTime :type Float%20%28single-precision%29) (EventReference :type Anim%20Notify%20Event%20Reference%20Structure%20%28by%20ref%29))
  (bind _gamestate (Class|BPIMCGameState|MCGSGetGameState(Message) (Game|GetGameState (Components|GetOwner MeshComp))))
  (Default|CheckDashBoost _gamestate)
  (return true))