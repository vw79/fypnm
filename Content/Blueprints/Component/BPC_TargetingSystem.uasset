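; Player targeting component that soft-locks and hard-locks onto living BP_Demon_Base enemies found by sphere traces.
; Soft lock picks a forward target during gamepad movement, otherwise scores candidates by camera alignment and distance.
; Hard lock takes the closest or most camera-centred enemy per GameInstance setting, with left/right switching by cross-product side tests.
; A looping timer interpolates control rotation toward the hard target, releasing it when invalid or out of range.
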(event Custom|LockOnTarget%28Left%29
  (bind _potentialtargetactor (General|FindActortoLockon))
  (bind _leftsideenemy (Switch|Left|FilterLeftSideEnemy _potentialtargetactor))
  ;[1 0.402 0] Switch Target Left
  (Utilities|IsValid (Variables|HardLock|GetHardLockedOnActor)
    (:Is%20Valid
      (Utilities|IsValid _leftsideenemy
        (:Is%20Valid
          (Utilities|IsValid (Variables|HardLock|GetHardLockedOnActor)
            (:Is%20Valid
              (Class|BPIDemon|ToggleLockVisual(Message) (Variables|HardLock|GetHardLockedOnActor) false)
              (bind _output_get (Variables|HardLock|SetHardLockedOnActor _leftsideenemy))
              (Variables|HardLock|SetisHardLock true)
              (Class|BPIDemon|ToggleLockVisual(Message) _output_get true (Utilities|Struct|MakeSlateColor "(R=1.000000,G=1.000000,B=1.000000,A=1.000000)"))
              (CallFunction|StartTargetLockonTimer))))
        (:Is%20Not%20Valid
          (HardLock|EndHardTarget))))))

(event Custom|TargetLockonTimer
  (bind _returnvalue (Utilities|Time|GetWorldDeltaSeconds))
  (bind _returnvalue_2 (General|GetLockonCameraRotation))
  (bind _camrotationspeed (Variables|General|GetCamRotationSpeed))
  (bind _mccontrollerref (Variables|Reference|GetMCControllerRef))
  (bind _returnvalue_3 (Pawn|GetControlRotation _mccontrollerref :!class /Script/Engine.Controller))
  (bind _returnvalue_4 (Math|Interpolation|RInterpTo _returnvalue_3 _returnvalue_2 _returnvalue _camrotationspeed))
  ;[1 0 0.723] Target Enemy Camera
  (if (and (Variables|HardLock|GetisHardLock) (Utilities|IsValid (Variables|HardLock|GetHardLockedOnActor)))
    (if (< (Transformation|GetDistanceTo (Variables|Reference|GetMcRef) (Variables|HardLock|GetHardLockedOnActor)) (Variables|General|GetMaxTargetDistance))
      (Pawn|SetControlRotation (Variables|Reference|GetMCControllerRef) (Math|Rotator|MakeRotator (.Roll (Math|Rotator|BreakRotator _returnvalue_3)) (.pitch _returnvalue_4) (.yaw _returnvalue_4)))
      (else
        (Development|PrintString "too far")
        (HardLock|EndHardTarget)))
    (else
      (HardLock|EndHardTarget))))

(event Custom|LockOnTarget%28Right%29
  (bind _potentialtargetactor (General|FindActortoLockon))
  (bind _rightsideenemy (Switch|Right|FilterRightSideEnemy _potentialtargetactor))
  ;[1 0.402 0] Switch Target Right
  (Utilities|IsValid (Variables|HardLock|GetHardLockedOnActor)
    (:Is%20Valid
      (Utilities|IsValid _rightsideenemy
        (:Is%20Valid
          (Utilities|IsValid (Variables|HardLock|GetHardLockedOnActor)
            (:Is%20Valid
              (Class|BPIDemon|ToggleLockVisual(Message) (Variables|HardLock|GetHardLockedOnActor) false)
              (bind _output_get (Variables|HardLock|SetHardLockedOnActor _rightsideenemy))
              (Variables|HardLock|SetisHardLock true)
              (Class|BPIDemon|ToggleLockVisual(Message) _output_get true (Utilities|Struct|MakeSlateColor "(R=1.000000,G=1.000000,B=1.000000,A=1.000000)"))
              (CallFunction|StartTargetLockonTimer))))
        (:Is%20Not%20Valid
          (HardLock|EndHardTarget))))))

(event Custom|SoftLockOnTarget
  (params (moveInput :type Boolean))
  (bind _potentialtargetactor (General|FindActortoLockon))
  (bind _softlockenemy (General|FindActortoLockonDirection))
  (bind _closettarget (SoftLock|FindClosetSoftTarget _potentialtargetactor))
  ;[0.1559 1 0] Soft Lockon Target
  (if (and moveInput (CallFunction|IsController))
    (Utilities|IsValid _softlockenemy
      (:Is%20Valid
        (if (!= _softlockenemy (Variables|SoftLock|GetSoftLockedOnActor))
          (SoftLock|EndSoftTarget))
        (Variables|SoftLock|SetisSoftLock true)))
    (else
      (Utilities|IsValid _closettarget
        (:Is%20Valid
          (if (!= _closettarget (Variables|SoftLock|GetSoftLockedOnActor))
            (SoftLock|EndSoftTarget))
          (Variables|SoftLock|SetSoftLockedOnActor _closettarget)
          (Variables|SoftLock|SetisSoftLock true))))))

(event Custom|HardLockOnTarget
  (bind _closestenemy (General|FindActortoLockonController))
  (bind _potentialtargetactor (General|FindActortoLockon))
  (bind _closettarget (HardLock|FindClosetHardTarget _potentialtargetactor))
  ;[1 0.402 0] Hard Lockon Target
  (bind _lockonmode (Class|BPIGameInstance|GIGetLockonMode(Message) (Variables|Reference|GetGameInstanceRef)))
  (switch Utilities|FlowControl|Switch|SwitchonE_LockonMode _lockonmode
    (:NewEnumerator0
      ;;[1 1 1] Target Enemy Closet Enemy
      (Utilities|IsValid _closestenemy
        (:Is%20Valid
          (bind _output_get (Variables|HardLock|SetHardLockedOnActor _closestenemy))
          (SoftLock|EndSoftTarget)
          (Variables|HardLock|SetisHardLock true)
          (Class|BPIDemon|ToggleLockVisual(Message) _output_get true (Utilities|Struct|MakeSlateColor "(R=1.000000,G=1.000000,B=1.000000,A=1.000000)"))
          (CallFunction|StartTargetLockonTimer))
        (:Is%20Not%20Valid
          (HardLock|EndHardTarget))))
    (:NewEnumerator1
      ;;[1 1 1] Target Enemy at the Centre of Camera
      (Utilities|IsValid _closettarget
        (:Is%20Valid
          (bind _output_get_2 (Variables|HardLock|SetHardLockedOnActor _closettarget))
          (SoftLock|EndSoftTarget)
          (Variables|HardLock|SetisHardLock true)
          (Class|BPIDemon|ToggleLockVisual(Message) _output_get_2 true (Utilities|Struct|MakeSlateColor "(R=1.000000,G=1.000000,B=1.000000,A=1.000000)"))
          (CallFunction|StartTargetLockonTimer))
        (:Is%20Not%20Valid
          (HardLock|EndHardTarget))))))

(event Custom|StartTargetLockonTimer
  ;[1 0 0.723] Target Enemy Camera
  (CallFunction|StopTargetLockonTimer)
  (bind _returnvalue (Utilities|Time|SetTimerbyEvent (delegate Custom|TargetLockonTimer) (Utilities|Time|GetWorldDeltaSeconds) true)))

(event Custom|StopTargetLockonTimer
  ;[1 0 0.723] Target Enemy Camera
  (Utilities|Time|ClearandInvalidateTimerbyHandle (stale Custom|StartTargetLockonTimer _returnvalue)))

(event EventBeginPlay
  ;[1 1 1] On Start
  (bind _mc (Class|BPIGAS|GASGetMcRef(Message) (Components|GetOwner)))
  (Variables|Reference|SetMcRef _mc)
  (Variables|Reference|SetCameraRef (Variables|/Game/ThirdPerson/Blueprints/Player/BP_MC.BP_MC_C|GetFollowCamera _mc))
  (bind _mccontroller (Class|BPIGAS|GASGetMcControllerRef(Message) (Game|GetPlayerController 0)))
  (Variables|Reference|SetMCControllerRef _mccontroller)
  (bind _asbp_nmgame_instance (Utilities|Casting|CastToBP_NMGameInstance (Game|GetGameInstance)))
  (Variables|Reference|SetGameInstanceRef _asbp_nmgame_instance))

(fn FindActortoLockon
  (bind _mcref (Variables|Reference|GetMcRef))
  (bind _returnvalue (Transformation|GetActorLocation _mcref))
  (Utilities|Array|Clear (Variables|General|GetPotentialTargetActor))
  (bind (_outhits _returnvalue_2) (Collision|MultiSphereTraceForObjects _returnvalue _returnvalue (Variables|General|GetRadius) (Utilities|Array|MakeArray "ObjectTypeQuery7") false (Utilities|Array|MakeArray (Components|GetOwner)) "None"))
  (for _array_element _outhits
    (if (and _returnvalue_2 (Utilities|ClassIsChildOf (Utilities|GetClass (.HitActor (Collision|BreakHitResult _array_element))) "/Game/AI/Blueprints/BP_Demon_Base.BP_Demon_Base_C"))
      (bind _dmgsyscomponent (Class|BPIDamagable|DmgGetDmgSysComponent(Message) (.HitActor (Collision|BreakHitResult _array_element))))
      (if (not (Variables|/Game/Blueprints/Health_Damage_System/BPC_DamageSystem.BPC_DamageSystem_C|GetisDead _dmgsyscomponent))
        (Utilities|Array|AddUnique (Variables|General|GetPotentialTargetActor) (.HitActor (Collision|BreakHitResult _array_element))))))
  (return (Variables|General|GetPotentialTargetActor)))

(fn CheckHowCloseHardTarget
  (params (Target :type Actor%20Object%20Reference))
  (return (Math|Vector|DotProduct (Math|Vector|GetForwardVector (Variables|Reference|GetCameraRef)) (Math|Rotator|GetRotationXVector (Math|Rotator|FindLookatRotation (Transformation|GetActorLocation (Variables|Reference|GetMcRef)) (Transformation|GetActorLocation Target))))))

(fn FindClosetHardTarget
  (params (Actor :type Array%20of%20Actor%20Object%20References))
  (for _array_element Actor
    (Utilities|IsValid _array_element
      (:Is%20Valid
        (bind _returnvalue (Collision|LineTraceByChannel (Transformation|GetWorldLocation (Variables|Reference|GetCameraRef)) (Transformation|GetActorLocation _array_element) "TraceTypeQuery1" false 0 "None"))
        (if _returnvalue
          (Math|Float|CompareFloat (HardLock|CheckHowCloseHardTarget _array_element) (LocalVariables|GetCompareTarget)
            (:>
              (LocalVariables|SetCompareTarget (HardLock|CheckHowCloseHardTarget _array_element))
              (LocalVariables|SetlClosetTarget _array_element)))))))
  (return (LocalVariables|GetlClosetTarget)))

(fn CheckHowCloseSoftTarget
  (params (Target :type Actor%20Object%20Reference))
  (return (- (Math|Vector|DotProduct (Math|Vector|GetForwardVector (Variables|Reference|GetCameraRef)) (Math|Rotator|GetRotationXVector (Math|Rotator|FindLookatRotation (Transformation|GetActorLocation (Variables|Reference|GetMcRef)) (Transformation|GetActorLocation Target)))) (* 1.5 (/ (Math|Vector|Distance2D(Vector) (Transformation|GetActorLocation (Variables|Reference|GetMcRef)) (Transformation|GetActorLocation Target)) (Variables|General|GetRadius))))))

(fn FindClosetSoftTarget
  (params (Actor :type Array%20of%20Actor%20Object%20References))
  (LocalVariables|SetSoftScore 0.0)
  (LocalVariables|SetlClosetSoftTarget 0)
  (for _array_element Actor
    (Utilities|IsValid _array_element
      (:Is%20Valid
        (bind _returnvalue (Collision|LineTraceByChannel (Transformation|GetWorldLocation (Variables|Reference|GetCameraRef)) (Transformation|GetActorLocation _array_element) "TraceTypeQuery1" false 0 "None"))
        (if _returnvalue
          (Math|Float|CompareFloat (SoftLock|CheckHowCloseSoftTarget _array_element) (LocalVariables|GetSoftScore)
            (:>
              (LocalVariables|SetSoftScore (SoftLock|CheckHowCloseSoftTarget _array_element))
              (LocalVariables|SetlClosetSoftTarget _array_element)))))))
  (return (LocalVariables|GetlClosetSoftTarget)))

(fn GetLockonCameraRotation
  (bind _hardlockedonactor (Variables|HardLock|GetHardLockedOnActor))
  (bind _returnvalue (Transformation|GetActorLocation _hardlockedonactor))
  (return (Math|Rotator|FindLookatRotation (Transformation|GetWorldLocation (Variables|Reference|GetCameraRef)) (Math|Vector|MakeVector (.x _returnvalue) (.y _returnvalue) (- (.z _returnvalue) (/ (Math|Vector|Distance(Vector) (Transformation|GetActorLocation (Variables|Reference|GetMcRef)) (Transformation|GetActorLocation (Variables|HardLock|GetHardLockedOnActor))) 2.0))))))

(fn EndHardTarget
  (Variables|HardLock|SetisHardLock false)
  (Utilities|IsValid (Variables|HardLock|GetHardLockedOnActor)
    (:Is%20Valid
      (Class|BPIDemon|ToggleLockVisual(Message) (Variables|HardLock|GetHardLockedOnActor) false))
    (:Is%20Not%20Valid
      _))
  (Variables|HardLock|SetHardLockedOnActor 0)
  (CallFunction|StopTargetLockonTimer))

(fn FilterLeftSideEnemy
  (params (Actor :type Array%20of%20Actor%20Object%20References))
  (LocalVariables|SetlClosetTarget 0)
  (LocalVariables|SetclosetDistance 99999.0)
  (for _array_element Actor
    (LocalVariables|SetenemyDirection (- (Transformation|GetActorLocation _array_element) (Transformation|GetActorLocation (Variables|Reference|GetMcRef))))
    (LocalVariables|SettargetDirection (- (Transformation|GetActorLocation (Variables|HardLock|GetHardLockedOnActor)) (Transformation|GetActorLocation (Variables|Reference|GetMcRef))))
    (if (> (.z (Math|Vector|CrossProduct (LocalVariables|GetenemyDirection) (LocalVariables|GettargetDirection))) 0.0)
      (Math|Float|CompareFloat (Math|Vector|Distance(Vector) (Transformation|GetActorLocation _array_element) (Transformation|GetActorLocation (Variables|HardLock|GetHardLockedOnActor))) (LocalVariables|GetclosetDistance)
        (:<
          (LocalVariables|SetclosetDistance (Math|Vector|Distance(Vector) (Transformation|GetActorLocation _array_element) (Transformation|GetActorLocation (Variables|HardLock|GetHardLockedOnActor))))
          (LocalVariables|SetlClosetTarget _array_element)))))
  (return (LocalVariables|GetlClosetTarget)))

(fn EndSoftTarget
  (Variables|SoftLock|SetisSoftLock false)
  (Utilities|IsValid (Variables|SoftLock|GetSoftLockedOnActor)
    (:Is%20Valid
      (Class|BPIDemon|ToggleLockVisual(Message) (Variables|SoftLock|GetSoftLockedOnActor) false))
    (:Is%20Not%20Valid
      _))
  (Variables|SoftLock|SetSoftLockedOnActor 0))

(fn FilterRightSideEnemy
  (params (Actor :type Array%20of%20Actor%20Object%20References))
  (LocalVariables|SetlClosetTarget 0)
  (LocalVariables|SetclosetDistance 99999.0)
  (for _array_element Actor
    (LocalVariables|SetenemyDirection (- (Transformation|GetActorLocation _array_element) (Transformation|GetActorLocation (Variables|Reference|GetMcRef))))
    (LocalVariables|SettargetDirection (- (Transformation|GetActorLocation (Variables|HardLock|GetHardLockedOnActor)) (Transformation|GetActorLocation (Variables|Reference|GetMcRef))))
    (if (< (.z (Math|Vector|CrossProduct (LocalVariables|GetenemyDirection) (LocalVariables|GettargetDirection))) 0.0)
      (Math|Float|CompareFloat (Math|Vector|Distance(Vector) (Transformation|GetActorLocation _array_element) (Transformation|GetActorLocation (Variables|HardLock|GetHardLockedOnActor))) (LocalVariables|GetclosetDistance)
        (:<
          (LocalVariables|SetclosetDistance (Math|Vector|Distance(Vector) (Transformation|GetActorLocation _array_element) (Transformation|GetActorLocation (Variables|HardLock|GetHardLockedOnActor))))
          (LocalVariables|SetlClosetTarget _array_element)))))
  (return (LocalVariables|GetlClosetTarget)))

(fn GetHardLockEnemy
  (bind (_enemy _dmgsystem) (Class|BPIDemon|GetDemonRef(Message) (Variables|HardLock|GetHardLockedOnActor)))
  (Utilities|IsValid _enemy
    (:Is%20Valid
      (return _enemy (Variables|/Game/Blueprints/Health_Damage_System/BPC_DamageSystem.BPC_DamageSystem_C|GetisDead _dmgsystem)))))

(fn IsController
  (return (Utilities|Enum|Equal(Enum) (.PrimaryDeviceType (Utilities|Struct|BreakHardwareDeviceIdentifier (Class|InputDeviceSubsystem|GetInputDeviceHardwareIdentifier (|InputDeviceSubsystem)))) "Gamepad")))

(fn FindActortoLockonDirection
  (bind _mcref (Variables|Reference|GetMcRef))
  (LocalVariables|SetSoftScore 99999.0)
  (bind (_outhits _returnvalue) (Collision|MultiSphereTraceForObjects (Transformation|GetActorLocation _mcref) (+ (Transformation|GetActorLocation _mcref) (* (Transformation|GetActorForwardVector _mcref) (Variables|General|GetRadius))) 1e+02 (Utilities|Array|MakeArray "ObjectTypeQuery7") false (Utilities|Array|MakeArray (Components|GetOwner)) "None"))
  (for _array_element _outhits
    (if (and _returnvalue (Utilities|ClassIsChildOf (Utilities|GetClass (.HitActor (Collision|BreakHitResult _array_element))) "/Game/AI/Blueprints/BP_Demon_Base.BP_Demon_Base_C"))
      (bind _dmgsyscomponent (Class|BPIDamagable|DmgGetDmgSysComponent(Message) (.HitActor (Collision|BreakHitResult _array_element))))
      (if (and (not (Variables|/Game/Blueprints/Health_Damage_System/BPC_DamageSystem.BPC_DamageSystem_C|GetisDead _dmgsyscomponent)) (CallFunction|InfrontOf (.HitActor (Collision|BreakHitResult _array_element))))
        (Math|Float|CompareFloat (/ (Math|Vector|Distance2D(Vector) (Transformation|GetActorLocation (Variables|Reference|GetMcRef)) (Transformation|GetActorLocation (.HitActor (Collision|BreakHitResult _array_element)))) (Variables|General|GetRadius)) (LocalVariables|GetSoftScore)
          (:<
            (LocalVariables|SetSoftScore (/ (Math|Vector|Distance2D(Vector) (Transformation|GetActorLocation (Variables|Reference|GetMcRef)) (Transformation|GetActorLocation (.HitActor (Collision|BreakHitResult _array_element)))) (Variables|General|GetRadius)))
            (LocalVariables|SetTargetEnemy (.HitActor (Collision|BreakHitResult _array_element))))))))
  (return (LocalVariables|GetTargetEnemy)))

(fn FindActortoLockonController
  (bind _mcref (Variables|Reference|GetMcRef))
  (bind _returnvalue (Transformation|GetActorLocation _mcref))
  (LocalVariables|SetSoftScore 99999.0)
  (bind (_outhits _returnvalue_2) (Collision|MultiSphereTraceForObjects _returnvalue _returnvalue (Variables|General|GetRadius) (Utilities|Array|MakeArray "ObjectTypeQuery7") false (Utilities|Array|MakeArray (Components|GetOwner)) "None"))
  (for _array_element _outhits
    (if (and _returnvalue_2 (Utilities|ClassIsChildOf (Utilities|GetClass (.HitActor (Collision|BreakHitResult _array_element))) "/Game/AI/Blueprints/BP_Demon_Base.BP_Demon_Base_C"))
      (bind _dmgsyscomponent (Class|BPIDamagable|DmgGetDmgSysComponent(Message) (.HitActor (Collision|BreakHitResult _array_element))))
      (if (not (Variables|/Game/Blueprints/Health_Damage_System/BPC_DamageSystem.BPC_DamageSystem_C|GetisDead _dmgsyscomponent))
        (Math|Float|CompareFloat (/ (Math|Vector|Distance2D(Vector) (Transformation|GetActorLocation (Variables|Reference|GetMcRef)) (Transformation|GetActorLocation (.HitActor (Collision|BreakHitResult _array_element)))) (Variables|General|GetRadius)) (LocalVariables|GetSoftScore)
          (:<
            (LocalVariables|SetSoftScore (/ (Math|Vector|Distance2D(Vector) (Transformation|GetActorLocation (Variables|Reference|GetMcRef)) (Transformation|GetActorLocation (.HitActor (Collision|BreakHitResult _array_element)))) (Variables|General|GetRadius)))
            (LocalVariables|SetTargetEnemy (.HitActor (Collision|BreakHitResult _array_element))))))))
  (return (LocalVariables|GetTargetEnemy)))

(fn InfrontOf
  (params (Enemy :type Actor%20Object%20Reference))
  (bind _mcref (Variables|Reference|GetMcRef))
  (return (> (Math|Vector|DotProduct (Transformation|GetActorForwardVector _mcref) (Math|Vector|Normalize (- (Transformation|GetActorLocation Enemy) (Transformation|GetActorLocation _mcref)))) 0.7)))