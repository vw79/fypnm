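; Player weapon actor for the Megan character that switches between Katana and Blade Whip forms by toggling mesh visibility and updating the HUD image.
; On BeginPlay it starts unequipped in Katana form and registers itself with the character's ABP_Megan anim instance.
; Equip and unequip events snap the katana between the hand socket and its rest position, toggling the trail effect.
; Separate events move the sheath between character sockets.
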(event Custom|UpdateWeaponMode
  (params (WeaponMode :type E_WeaponMode%20Enum :default "NewEnumerator0") (AttackTriggered :type Boolean))
  (switch Utilities|FlowControl|Switch|SwitchonE_WeaponMode WeaponMode
    (:NewEnumerator0
      (Rendering|SetVisibility (Variables|Default|GetWhip) false false)
      (Rendering|SetVisibility (Variables|Default|GetKatana) true false)
      (Default|UpdateWeaponImage (Variables|Default|GetHUD%20Ref) (Variables|Default|GetEWeaponMode)))
    (:NewEnumerator2
      (Rendering|SetVisibility (Variables|Default|GetKatana) false false)
      (Rendering|SetVisibility (Variables|Default|GetWhip) true false)
      (Default|UpdateWeaponImage (Variables|Default|GetHUD%20Ref) (Variables|Default|GetEWeaponMode)))))

(event Custom|EquipWeapon
  (Transformation|AttachComponentToComponent (Variables|Default|GetKatana) (Variables|/Script/Engine.Character|GetMesh (Variables|Default|GetMcRef)) "weaponSocket" "SnapToTarget" "SnapToTarget" "SnapToTarget" true)
  (Components|Activation|Activate (Variables|Default|GetTrail) false)
  (Variables|Default|SetisEquip true))

(event Custom|UnequipWeapon
  (bind _katana (Variables|Default|GetKatana))
  (Transformation|DetachFromComponent _katana "KeepRelative" "KeepRelative" "KeepRelative" true)
  (Transformation|AttachComponentToComponent _katana (Variables|Default|GetOriKatanaPos) "" "SnapToTarget" "SnapToTarget" "SnapToTarget" true)
  (Components|Activation|Deactivate (Variables|Default|GetTrail))
  (Variables|Default|SetisEquip false))

(event Custom|EquipSheath
  (Transformation|AttachComponentToComponent (Variables|/Script/Engine.Character|GetMesh (Variables|Default|GetMcRef)) "sheathSocket" "SnapToTarget" "SnapToTarget" "SnapToTarget" true))

(event Custom|UnequipSheath
  (Transformation|AttachComponentToComponent (Variables|/Script/Engine.Character|GetMesh (Variables|Default|GetMcRef)) "unequipSheath" "SnapToTarget" "SnapToTarget" "SnapToTarget" true))

(event EventBeginPlay
  (CallFunction|UnequipWeapon)
  (Rendering|SetVisibility (Variables|Default|GetWhip) false false)
  (Rendering|SetVisibility (Variables|Default|GetKatana) true false)
  (bind _mc (Class|BPIGAS|GASGetMcRef(Message) (Game|GetPlayerCharacter 0)))
  (bind _output_get (Variables|Default|SetMcRef _mc))
  (bind _asabp_megan (Utilities|Casting|CastToABP_Megan (Components|SkeletalMesh|GetAnimInstance (Variables|/Script/Engine.Character|GetMesh _output_get))))
  (Variables|/Game/Characters/Megan/ABP_Megan.ABP_Megan_C|SetWeapon%20Ref _asabp_megan self))

(fn ConstructionScript)