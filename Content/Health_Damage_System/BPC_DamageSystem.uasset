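; Actor component that manages health for the damage system, handling healing, damage, blocking and death.
; TakeDamage routes a DamageInfo struct through the CanBeDamaged macro, which checks death, invincibility and blocking to choose block, damage or no damage.
; Blocked hits report parryability; damaging hits reduce Health, then either signal death or send a damage response when interruptible and force-interrupted.
; Heal adds health clamped to MaxHealth while alive.
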(event EventBeginPlay)

(event EventTick
  (params (DeltaSeconds :type Float%20%28single-precision%29)))

(fn Heal
  (params (Amount :type Float%20%28double-precision%29))
  (if (not (Variables|Default|GetisDead))
    (Variables|Default|SetHealth (Math|Float|Clamp(Float) (+ Amount (Variables|Default|GetHealth)) 0.0 (Variables|Default|GetMaxHealth)))
    (return 0.0)))

(fn TakeDamage
  (params (DamageInfo :type S%20Damage%20Info%20Structure))
  (bind (_amount _damagetype _damageresponse _isinvincible _canbeblocked _canbeparried _shouldforceinterrupt) (Utilities|Struct|BreakS_DamageInfo DamageInfo))
  (Utilities|CanbeDamaged _isinvincible _canbeblocked
    (:BlockDamage
      ;[1 1 1] Nothing for Now, but if possible can implement later
      (Default|CallOnBlocked _canbeparried)
      (return false))
    (:DoDamage
      (bind _output_get (Variables|Default|SetHealth (- (Variables|Default|GetHealth) _amount)))
      (if (<= _output_get 0.0)
        (Variables|Default|SetisDead true)
        (Default|CallOnDeath)
        (return true)
        (elif (and (Variables|Default|GetisInterruptible) _shouldforceinterrupt)
          (Default|CallOnDamageResponse _damageresponse)
          (return true))))
    (:NoDamage
      (return false))))