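; GA_Dash is a Gameplay Ability that makes the avatar dash using the AM_Dash montage.
; On activation it commits, starts the montage, messages the avatar to add movement and commits the cooldown.
; It ends on the Ability.Dash.End event or montage interruption or cancellation, then messages the avatar to stop dash movement and reset FOV.
; An unconnected step-back branch for zero movement input never runs.
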(event Ability|EventActivateAbility
  (Ability|CommitAbility)
  (|PlayMontageandWaitProxy "None" "/Game/Animation/MC/Locomotion/AM_Dash.AM_Dash" 1.0 "None" true 1.0 0.0 false
    (:then
      (Class|BPIGAS|GASAddAtkMove(Message) (Ability|GetAvatarActorfromActorInfo) 5e+01)
      (Ability|CommitAbilityCooldown false)
      (Ability|Tasks|WaitGameplayEvent "(TagName=\"Ability.Dash.End\")" 0
        (:EventReceived
          (Ability|EndAbility))))
    (:OnInterrupted
      (Ability|EndAbility :!label _label))
    (:OnCancelled
      (goto _label))))

(event Ability|EventOnEndAbility
  (params (bWasCancelled :type Boolean))
  (bind _returnvalue (Ability|GetAvatarActorfromActorInfo))
  (Class|BPIGAS|GASStopDashMovement(Message) _returnvalue)
  (Class|BPIGAS|GASResetDashFov(Message) _returnvalue))