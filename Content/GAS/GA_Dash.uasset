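; Gameplay ability that makes the avatar dash forward when moving, or step back when standing still.
; Both branches commit the ability, play their montage and apply a constant root motion force along the actor's forward axis.
; The dash is a short, strong burst that restores prior velocity; the step back is weaker, longer and reversed.
; The ability ends when the force finishes, independent of montage completion.
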(event Ability|EventActivateAbility
  (bind _returnvalue (Ability|GetAvatarActorfromActorInfo))
  (if (> (Math|Vector|VectorLength (Transformation|GetVelocity (Ability|GetAvatarActorfromActorInfo))) 0.0)
    (Ability|CommitAbility)
    (|PlayMontageandWaitProxy "None" "/Game/VW/Anim/dash.dash" 1.0 "None" true 1.0 0.0 false
      (:then
        (Ability|Tasks|ApplyRootMotionConstantForce "None" (Transformation|GetActorForwardVector _returnvalue) 4e+03 0.2 false 0 "SetVelocity" (Transformation|GetVelocity _returnvalue)
          (:OnFinish
            (Ability|EndAbility)))))
    (else
      (Ability|CommitAbility)
      (|PlayMontageandWaitProxy "None" "/Game/VW/Anim/AM_StepBack.AM_StepBack" 1.0 "None" true 1.0 0.0 false
        (:then
          (Ability|Tasks|ApplyRootMotionConstantForce "None" (* (Transformation|GetActorForwardVector (Ability|GetAvatarActorfromActorInfo)) -1.0) 3e+02 0.8 false 0 "SetVelocity"
            (:OnFinish
              (Ability|EndAbility))))))))

(event Ability|EventOnEndAbility
  (params (bWasCancelled :type Boolean)))