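; GA_JumpBoost is a gameplay ability that launches the player character straight up in a boosted jump.
; On activation it commits, plays the jump boost montage, sets the character's JumpBoost flag, applies a vertical launch and registers a combo.
; A looping timer at frame interval polls the falling state and ends the ability once the character is no longer falling, clearing the flag and timer.
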(event Custom|StopTimer
  (Utilities|Time|ClearandInvalidateTimerbyHandle (stale Ability|EventActivateAbility _returnvalue)))

(event Custom|StartTimer
  (bind _mc (Class|BPIGAS|GASGetMcRef(Message) (Ability|GetAvatarActorfromActorInfo)))
  (bind _isfalling (Class|BPIGAS|GASGetIsFalling(Message) _mc))
  (if (not _isfalling)
    (Ability|EndAbility)))

(event Ability|EventOnEndAbility
  (params (bWasCancelled :type Boolean))
  (bind _mc (Class|BPIGAS|GASGetMcRef(Message) (Ability|GetAvatarActorfromActorInfo)))
  (Variables|/Game/ThirdPerson/Blueprints/Player/BP_MC.BP_MC_C|SetbJumpBoost _mc false)
  (CallFunction|StopTimer))

(event Ability|EventActivateAbility
  (Ability|CommitAbility)
  (bind (_mc _gas _targeting _actioncam _combocounter) (Class|BPIGAS|GASGetMcRef(Message) (Ability|GetAvatarActorfromActorInfo)))
  (|PlayMontageandWaitProxy "None" "/Game/Characters/Megan/Anim/Locomotion/AM_JumpBoost.AM_JumpBoost" 1.0 "None" true 1.0 0.0 false
    (:then
      (Variables|/Game/ThirdPerson/Blueprints/Player/BP_MC.BP_MC_C|SetbJumpBoost _mc true)
      (Character|LaunchCharacter _mc "0.000000,0.000000,2000.000000" false true)
      (Default|RegisterCombo _combocounter)
      (bind _returnvalue (Utilities|Time|SetTimerbyEvent (delegate Custom|StartTimer) (Utilities|Time|GetWorldDeltaSeconds) true)))
    (:OnCancelled
      (Ability|EndAbility))))