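; GA_PerfectDash is a gameplay ability for a perfect dash that registers a combo and slows the world around the character.
; It plays a dash montage, adds attack movement, applies GE_Dash and ignores Pawn collision.
; Global time dilation drops while the character's custom dilation rises to compensate, keeping the player at normal speed.
; A dash-end event or montage end finishes the ability, restoring time and collision and removing the effect.
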(event Ability|EventActivateAbility
  (Ability|CommitAbility)
  (|PlayMontageandWaitProxy "None" "/Game/Characters/Megan/Anim/Locomotion/AM_Dash_Megan.AM_Dash_Megan" 1.0 "None" true 1.0 0.0 false
    (:then
      (bind (_mc _gas _targeting _actioncam _combocounter) (Class|BPIGAS|GASGetMcRef(Message) (Ability|GetAvatarActorfromActorInfo)))
      (Ability|GameplayEffect|RemoveLooseGameplayTags _mc (Variables|Default|GetComboStarterTag))
      (Default|RegisterCombo _combocounter)
      (Class|BPIGAS|GASAddAtkMove(Message) _mc 2e+01)
      (Utilities|Time|SetGlobalTimeDilation 0.2)
      (Variables|/Script/Engine.Actor|SetCustomTimeDilation _mc 5.0)
      (Collision|SetCollisionResponsetoChannel (Variables|/Script/Engine.Character|GetCapsuleComponent _mc) "ECC_Pawn" "ECR_Ignore")
      (bind _returnvalue (Ability|ApplyGameplayEffectToOwner "/Game/GAS/Locomotion/Cue-n-Effect/GE_Dash.GE_Dash_C"))
      (Variables|Default|SetActiveEffect _returnvalue)
      (Ability|Tasks|WaitGameplayEvent "(TagName=\"Ability.Dash.End\")" 0
        (:EventReceived
          (Ability|EndAbility))))
    (:OnCompleted
      (Ability|EndAbility :!label _label))
    (:OnInterrupted
      (goto _label))
    (:OnCancelled
      (goto _label))))

(event Ability|EventOnEndAbility
  (params (bWasCancelled :type Boolean))
  (Class|BPIGAS|GASStopDashMovement(Message) (Ability|GetAvatarActorfromActorInfo))
  (Ability|RemoveGameplayEffectFromOwnerWithHandle (Variables|Default|GetActiveEffect))
  (Collision|SetCollisionResponsetoChannel (Variables|/Script/Engine.Character|GetCapsuleComponent (stale Ability|EventActivateAbility _mc)) "ECC_Pawn" "ECR_Block")
  (Utilities|Time|SetGlobalTimeDilation 1.0)
  (Variables|/Script/Engine.Actor|SetCustomTimeDilation (stale Ability|EventActivateAbility _mc) 1.0))