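; GA_DoubleJump is a Gameplay Ability that performs the character's double jump.
; On activation it plays a jump sound, commits, removes the loose DoubleJumpTag and gets the main character through a GAS message call.
; It plays the double jump montage while setting the DoubleJump flag, launching the character upward with a Z override and registering a combo.
; The ability ends when the montage finishes, is interrupted or cancelled, clearing the flag on end.
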(event Ability|EventActivateAbility
  (Audio|PlaySound2D "/Game/SFX/SoundCue/SC_Jump.SC_Jump" 1.0 1.0 0.0 0 0)
  (Ability|CommitAbility)
  (Ability|GameplayEffect|RemoveLooseGameplayTags (Ability|GetAvatarActorfromActorInfo) (Variables|Default|GetDoubleJumpTag))
  (bind (_mc _gas _targeting _actioncam _combocounter) (Class|BPIGAS|GASGetMcRef(Message) (Ability|GetAvatarActorfromActorInfo)))
  (|PlayMontageandWaitProxy "None" "/Game/Characters/Mel/Anim/Locomotion/AM_JumpDouble1.AM_JumpDouble1" 1.0 "None" true 1.0 0.0 false
    (:then
      (Variables|/Game/ThirdPerson/Blueprints/Player/BP_MC.BP_MC_C|SetbDoubleJump _mc true)
      (Character|LaunchCharacter _mc "0.000000,0.000000,1000.000000" false true)
      (Default|RegisterCombo _combocounter))
    (:OnCompleted
      (Ability|EndAbility :!label _label))
    (:OnInterrupted
      (goto _label))
    (:OnCancelled
      (goto _label))))

(event Ability|EventOnEndAbility
  (params (bWasCancelled :type Boolean))
  (bind _mc (Class|BPIGAS|GASGetMcRef(Message) (Ability|GetAvatarActorfromActorInfo)))
  (Variables|/Game/ThirdPerson/Blueprints/Player/BP_MC.BP_MC_C|SetbDoubleJump _mc false))