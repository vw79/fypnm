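; GA_Jump is a Gameplay Ability that makes the main character jump and counts the jump toward combos.
; On activation it plays the jump sound, commits, and adds a local double-jump tag to the avatar.
; An interface message supplies the character and its combo counter, so it removes the combo-starter tag, calls Jump and registers the combo.
; The ability ends immediately, without waiting for landing.
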(event Ability|EventActivateAbility
  (Audio|PlaySound2D "/Game/SFX/SoundCue/SC_Jump.SC_Jump" 1.0 1.0 0.0 0 0)
  (Ability|CommitAbility)
  (Ability|GameplayEffect|AddLooseGameplayTags (Ability|GetAvatarActorfromActorInfo) (Variables|Default|GetDoubleJumpTag))
  (bind (_mc _gas _targeting _actioncam _combocounter) (Class|BPIGAS|GASGetMcRef(Message) (Ability|GetAvatarActorfromActorInfo)))
  (Ability|GameplayEffect|RemoveLooseGameplayTags _mc (Variables|Default|GetComboStarterTag))
  (Character|Jump _mc)
  (Default|RegisterCombo _combocounter)
  (Ability|EndAbility))