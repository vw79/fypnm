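; Gameplay ability for the character's dash, choosing a dash with movement input or a back dash without it.
; Each plays its montage and sends an attack-move message, while the back dash also unequips the weapon and adds an upward launch.
; Both clear the combo starter tag, register a combo and apply GE_Dash.
; The montage finishing or an Ability.Dash.End event ends the ability, which stops dash movement and removes the effect.
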(event Ability|EventActivateAbility
  (bind _returnvalue (Ability|GetAvatarActorfromActorInfo))
  (Ability|CommitAbility)
  (bind _mc (Class|BPIGAS|GASGetMcRef(Message) (Ability|GetAvatarActorfromActorInfo)))
  (if (!= (Math|Vector|VectorLength (Class|Pawn|GetLastMovementInputVector _mc)) 0.0)
    (|PlayMontageandWaitProxy "None" "/Game/Characters/Megan/Anim/Locomotion/AM_Dash.AM_Dash" 1.0 "None" true 1.0 0.0 false
      (:then
        (Class|BPIGAS|GASAddAtkMove(Message) _returnvalue 5e+01)
        (bind (_mc_2 _gas _targeting _actioncam _combocounter) (Class|BPIGAS|GASGetMcRef(Message) _returnvalue :!label _label))
        (Ability|GameplayEffect|RemoveLooseGameplayTags _mc_2 (Variables|Default|GetComboStarterTag))
        (Default|RegisterCombo _combocounter)
        (bind _returnvalue_2 (Ability|ApplyGameplayEffectToOwner "/Game/GAS/Locomotion/Cue-n-Effect/GE_Dash.GE_Dash_C"))
        (Variables|Default|SetActiveEffect _returnvalue_2)
        (Ability|Tasks|WaitGameplayEvent "(TagName=\"Ability.Dash.End\")" 0
          (:EventReceived
            (Ability|EndAbility))))
      (:OnCompleted
        (Ability|EndAbility :!label _label_2))
      (:OnInterrupted
        (goto _label_2))
      (:OnCancelled
        (goto _label_2)))
    (else
      ;[1 1 1] Dash Back
      (bind _mc_3 (Class|BPIGAS|GASGetMcRef(Message) (Ability|GetAvatarActorfromActorInfo)))
      (Default|UnequipWeapon (Variables|/Game/ThirdPerson/Blueprints/Player/BP_MC.BP_MC_C|GetWeaponRef _mc_3))
      (|PlayMontageandWaitProxy "None" "/Game/Characters/Megan/Anim/Locomotion/AM_DashBack.AM_DashBack" 1.0 "None" true 1.0 0.0 false
        (:then
          (Class|BPIGAS|GASAddAtkMove(Message) (Ability|GetAvatarActorfromActorInfo) -1e+01)
          (Character|LaunchCharacter _mc_3 "0.000000,0.000000,150.000000" false false)
          (goto _label))
        (:OnCompleted
          _)
        (:OnInterrupted
          _)
        (:OnCancelled
          _))
      (Ability|EndAbility))))

(event Ability|EventOnEndAbility
  (params (bWasCancelled :type Boolean))
  (Class|BPIGAS|GASStopDashMovement(Message) (Ability|GetAvatarActorfromActorInfo))
  (Ability|RemoveGameplayEffectFromOwnerWithHandle (Variables|Default|GetActiveEffect)))