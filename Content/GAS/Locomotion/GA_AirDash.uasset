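; GA_AirDash is a gameplay ability that performs the character's air dash.
; After commit it plays a dash montage, adds attack movement, applies a VFX effect, removes the combo starter tag, registers a combo and starts wall-run.
; A per-frame looping timer ends the ability once the character stops falling or is on a wall, as does the montage finishing or being interrupted.
; Ending stops dash movement, removes the effect and clears the timer.
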(event Custom|StopTimer
  (Utilities|Time|ClearandInvalidateTimerbyHandle (stale Ability|EventActivateAbility _returnvalue_2)))

(event Custom|StartTimer
  (bind _mc (Class|BPIGAS|GASGetMcRef(Message) (Ability|GetAvatarActorfromActorInfo)))
  (bind _isfalling (Class|BPIGAS|GASGetIsFalling(Message) _mc))
  (if (or (not _isfalling) (Variables|/Game/ThirdPerson/Blueprints/Player/BP_MC.BP_MC_C|GetOnWall? _mc))
    (Ability|EndAbility)))

(event Ability|EventActivateAbility
  (Ability|CommitAbility)
  (|PlayMontageandWaitProxy "None" "/Game/Characters/Mel/Anim/Locomotion/AM_DashAir_Mel.AM_DashAir_Mel" 1.0 "None" true 1.0 0.0 false
    (:then
      (Class|BPIGAS|GASAddAtkMove(Message) (Ability|GetAvatarActorfromActorInfo) 5e+01)
      (bind _returnvalue (Ability|ApplyGameplayEffectToOwner "/Game/GAS/Locomotion/Cue-n-Effect/GE_AirDashVFX.GE_AirDashVFX_C"))
      (Variables|Default|SetActiveEffect _returnvalue)
      (bind (_mc _gas _targeting _actioncam _combocounter) (Class|BPIGAS|GASGetMcRef(Message) (Ability|GetAvatarActorfromActorInfo)))
      (Ability|GameplayEffect|RemoveLooseGameplayTags _mc (Variables|Default|GetComboStarterTag))
      (Default|RegisterCombo _combocounter)
      (Default|StartWallRun _mc)
      (bind _returnvalue_2 (Utilities|Time|SetTimerbyEvent (delegate Custom|StartTimer) (Utilities|Time|GetWorldDeltaSeconds) true)))
    (:OnCompleted
      (Ability|EndAbility :!label _label))
    (:OnInterrupted
      (goto _label))
    (:OnCancelled
      (goto _label))))

(event Ability|EventOnEndAbility
  (params (bWasCancelled :type Boolean))
  (Class|BPIGAS|GASStopDashMovement(Message) (Ability|GetAvatarActorfromActorInfo))
  (Ability|RemoveGameplayEffectFromOwnerWithHandle (Variables|Default|GetActiveEffect))
  (CallFunction|StopTimer))