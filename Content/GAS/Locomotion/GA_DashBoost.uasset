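; GA_DashBoost is a Gameplay Ability that performs the avatar's dash boost.
; Activation commits, plays the boost montage, sends an attack-move message, adds a small upward launch, registers a combo and applies GE_DashBoost.
; An Ability.Dash.End event or the montage finishing, interrupting or cancelling ends it.
; OnEndAbility stops dash movement, removes the effect and, if movement input exists, sets velocity forward to carry momentum.
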(event Ability|EventActivateAbility
  (bind _returnvalue (Ability|GetAvatarActorfromActorInfo))
  (Ability|CommitAbility)
  (bind _mc (Class|BPIGAS|GASGetMcRef(Message) (Ability|GetAvatarActorfromActorInfo)))
  (|PlayMontageandWaitProxy "None" "/Game/Characters/Megan/Anim/Locomotion/AM_DashBoost_Megan.AM_DashBoost_Megan" 1.0 "None" true 1.0 0.0 false
    (:then
      (Class|BPIGAS|GASAddAtkMove(Message) _returnvalue 1e+02)
      (Development|PrintString "boost")
      (Character|LaunchCharacter _mc "0.000000,0.000000,150.000000" false false)
      (bind _combocounter (Class|BPIGAS|GASGetMcRef(Message) _returnvalue))
      (Default|RegisterCombo _combocounter)
      (bind _returnvalue_2 (Ability|ApplyGameplayEffectToOwner "/Game/GAS/Locomotion/Cue-n-Effect/GE_DashBoost.GE_DashBoost_C"))
      (Variables|Default|SetActiveEffect _returnvalue_2)
      (Ability|Tasks|WaitGameplayEvent "(TagName=\"Ability.Dash.End\")" 0
        (:EventReceived
          (Ability|EndAbility))))
    (:OnCompleted
      (Ability|EndAbility :!label _label))
    (:OnInterrupted
      (goto _label))
    (:OnCancelled
      (goto _label))))

(event Ability|EventOnEndAbility
  (params (bWasCancelled :type Boolean))
  (Class|BPIGAS|GASStopDashMovement(Message) (Ability|GetAvatarActorfromActorInfo))
  (Ability|RemoveGameplayEffectFromOwnerWithHandle (Variables|Default|GetActiveEffect))
  (bind (_mc _gas _targeting _actioncam _combocounter _weapon_collision _movement) (Class|BPIGAS|GASGetMcRef(Message) (Ability|GetAvatarActorfromActorInfo)))
  (if (> (Math|Vector|VectorLength (Class|Pawn|GetLastMovementInputVector _mc)) 0.1)
    (Variables|/Script/Engine.MovementComponent|SetVelocity _movement (* (Transformation|GetActorForwardVector _mc) 1e+03))))