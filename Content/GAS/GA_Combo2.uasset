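; GA_Combo2 is a Gameplay Ability for the second slash in a combo, playing a sped-up montage on activation.
; Gameplay events mark the combo window: opening swaps the avatar's loose ComboOpen1 tag for ComboOpen2, and closing removes ComboOpen2 and ends the ability.
; Montage completion also ends the ability, but that path clears no tags, and interruption or cancellation is not handled.
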(event Ability|EventActivateAbility
  (bind _returnvalue (Ability|GetAvatarActorfromActorInfo))
  (Ability|CommitAbility)
  (|PlayMontageandWaitProxy "None" "/Game/VW/Slash/AM_Slash2.AM_Slash2" 1.3 "None" true 1.0 0.0 false
    (:then
      (Ability|Tasks|WaitGameplayEvent "(TagName=\"Event.ComboWindowOpen\")" 0
        (:then
          (Ability|Tasks|WaitGameplayEvent "(TagName=\"Event.ComboWindowEnd\")" 0
            (:EventReceived
              (Ability|GameplayEffect|RemoveLooseGameplayTags (Ability|GetAvatarActorfromActorInfo) (Variables|Default|GetComboOpen2))
              (Ability|EndAbility))))
        (:EventReceived
          (Ability|GameplayEffect|RemoveLooseGameplayTags _returnvalue (Variables|Default|GetComboOpen1))
          (Ability|GameplayEffect|AddLooseGameplayTags _returnvalue (Variables|Default|GetComboOpen2)))))
    (:OnCompleted
      (Ability|EndAbility))))

(event Ability|EventOnEndAbility
  (params (bWasCancelled :type Boolean)))