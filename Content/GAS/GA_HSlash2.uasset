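; GA_HSlash2 is a Gameplay Ability for the second heavy slash in a melee combo.
; It commits, plays AM_HSlash2 sped up and starts attack movement on the avatar.
; The combo window open event swaps the ComboOpen1 tag for ComboOpen2 and messages the player controller to save heavy attack input.
; The window end event clears the tag, resets attack state, stops movement and ends the ability, as does montage completion.
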(event Ability|EventActivateAbility
  (bind _returnvalue (Game|GetPlayerController 0))
  (bind _returnvalue_2 (Ability|GetAvatarActorfromActorInfo))
  (Ability|CommitAbility)
  (|PlayMontageandWaitProxy "None" "/Game/VW/Slash/AM_HSlash2.AM_HSlash2" 1.5 "None" true 1.0 0.0 false
    (:then
      (Class|BPIGAS|AddAtkMove(Message) (Ability|GetAvatarActorfromActorInfo) 5.0)
      (Ability|Tasks|WaitGameplayEvent "(TagName=\"Event.ComboWindowOpen\")" 0
        (:then
          (Ability|Tasks|WaitGameplayEvent "(TagName=\"Event.ComboWindowEnd\")" 0
            (:EventReceived
              (Ability|GameplayEffect|RemoveLooseGameplayTags (Ability|GetAvatarActorfromActorInfo) (Variables|Default|GetComboOpen2))
              (Class|BPIInputBuffer|IBResetAttackState(Message) _returnvalue)
              (Class|BPIGAS|StopAtkMove(Message) (Ability|GetAvatarActorfromActorInfo))
              (Ability|EndAbility))))
        (:EventReceived
          (Ability|GameplayEffect|RemoveLooseGameplayTags _returnvalue_2 (Variables|Default|GetComboOpen1))
          (Ability|GameplayEffect|AddLooseGameplayTags _returnvalue_2 (Variables|Default|GetComboOpen2))
          (Class|BPIInputBuffer|IBSaveHeavyAttack(Message) _returnvalue))))
    (:OnCompleted
      (Ability|EndAbility))))

(event Ability|EventOnEndAbility
  (params (bWasCancelled :type Boolean)))