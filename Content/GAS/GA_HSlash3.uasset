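; Gameplay Ability for the HSlash3 attack, apparently the third slash of a combo.
; It commits, plays the slash montage slightly sped up and starts attack movement on the avatar.
; A ComboWindowEnd gameplay event removes the combo-open loose tag, stops that movement and ends the ability.
; Montage completion also ends the ability but skips that cleanup, and other montage outcomes are unhandled.
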(event Ability|EventActivateAbility
  (Ability|CommitAbility)
  (|PlayMontageandWaitProxy "None" "/Game/VW/Slash/AM_HSlash3.AM_HSlash3" 1.3 "None" true 1.0 0.0 false
    (:then
      (Class|BPIGAS|AddAtkMove(Message) (Ability|GetAvatarActorfromActorInfo) 1e+01)
      (Ability|Tasks|WaitGameplayEvent "(TagName=\"Event.ComboWindowEnd\")" 0
        (:EventReceived
          (Ability|GameplayEffect|RemoveLooseGameplayTags (Ability|GetAvatarActorfromActorInfo) (Variables|Default|GetComboOpenTag))
          (Class|BPIGAS|StopAtkMove(Message) (Ability|GetAvatarActorfromActorInfo))
          (Ability|EndAbility))))
    (:OnCompleted
      (Ability|EndAbility))))

(event Ability|EventOnEndAbility
  (params (bWasCancelled :type Boolean)))