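; Gameplay ability for the second H slash of a melee combo: commits, sends its attack index to the player controller and plays the HSlash2 montage slightly sped up.
; Once the montage starts, it messages the avatar to add attack movement and listens for combo window events.
; Window open swaps loose tag ComboOpen1 for ComboOpen2; window end removes it, stops movement and ends the ability.
; Montage completion or cancellation also ends it, and OnEndAbility clears ComboOpen2.
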(event Ability|EventActivateAbility
  (bind _returnvalue (Ability|GetAvatarActorfromActorInfo))
  (Ability|CommitAbility)
  (Class|BPIGAS|GASSetHAttackIndex(Message) (Game|GetPlayerController 0) (Variables|Default|GetHIndex))
  (|PlayMontageandWaitProxy "None" "/Game/Animation/MC/Slash/AM_HSlash2.AM_HSlash2" 1.3 "None" true 1.0 0.0 false
    (:then
      (Class|BPIGAS|GASAddAtkMove(Message) (Ability|GetAvatarActorfromActorInfo) 5.0)
      (Ability|Tasks|WaitGameplayEvent "(TagName=\"Event.ComboWindowOpen\")" 0
        (:then
          (Ability|Tasks|WaitGameplayEvent "(TagName=\"Event.ComboWindowEnd\")" 0
            (:EventReceived
              (Ability|GameplayEffect|RemoveLooseGameplayTags (Ability|GetAvatarActorfromActorInfo) (Variables|Default|GetComboOpen2))
              (Class|BPIGAS|GASStopAtkMove(Message) (Ability|GetAvatarActorfromActorInfo))
              (Ability|EndAbility))))
        (:EventReceived
          (Ability|GameplayEffect|RemoveLooseGameplayTags _returnvalue (Variables|Default|GetComboOpen1))
          (Ability|GameplayEffect|AddLooseGameplayTags _returnvalue (Variables|Default|GetComboOpen2)))))
    (:OnCompleted
      (Ability|EndAbility :!label _label))
    (:OnCancelled
      (goto _label))))

(event Ability|EventOnEndAbility
  (params (bWasCancelled :type Boolean))
  (Ability|GameplayEffect|RemoveLooseGameplayTags (Ability|GetAvatarActorfromActorInfo) (Variables|Default|GetComboOpen2)))