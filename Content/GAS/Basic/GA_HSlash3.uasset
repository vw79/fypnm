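; Gameplay Ability for the third H-slash attack in a combo chain.
; On activation it commits, reports its attack index to the player controller, plays the AM_HSlash3 montage slightly sped up and starts attack movement on the avatar.
; A ComboWindowEnd gameplay event stops that movement, removes the combo-open tag and ends the ability.
; Montage completion or cancellation also ends it, and OnEndAbility always clears the tag.
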(event Ability|EventActivateAbility
  (Ability|CommitAbility)
  (Class|BPIGAS|GASSetHAttackIndex(Message) (Game|GetPlayerController 0) (Variables|Default|GetHIndex))
  (|PlayMontageandWaitProxy "None" "/Game/Animation/MC/Slash/AM_HSlash3.AM_HSlash3" 1.3 "None" true 1.0 0.0 false
    (:then
      (Class|BPIGAS|GASAddAtkMove(Message) (Ability|GetAvatarActorfromActorInfo) 1e+01)
      (Ability|Tasks|WaitGameplayEvent "(TagName=\"Event.ComboWindowEnd\")" 0
        (:EventReceived
          (Ability|GameplayEffect|RemoveLooseGameplayTags (Ability|GetAvatarActorfromActorInfo) (Variables|Default|GetComboOpenTag))
          (Class|BPIGAS|GASStopAtkMove(Message) (Ability|GetAvatarActorfromActorInfo))
          (Ability|EndAbility))))
    (:OnCompleted
      (Ability|EndAbility :!label _label))
    (:OnCancelled
      (goto _label))))

(event Ability|EventOnEndAbility
  (params (bWasCancelled :type Boolean))
  (Ability|GameplayEffect|RemoveLooseGameplayTags (Ability|GetAvatarActorfromActorInfo) (Variables|Default|GetComboOpenTag)))