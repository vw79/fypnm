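; Gameplay ability for the third light slash, which commits and plays AM_Lslash3 at increased rate while starting attack movement on the avatar.
; The combo-window-open event removes ComboOpenTag and sends a save-light-attack message to the player controller.
; The combo-window-end event removes the tag again, resets attack state, stops attack movement and ends the ability.
; Montage completion or interruption only ends the ability, without that cleanup.
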(event Ability|EventActivateAbility
  (bind _returnvalue (Game|GetPlayerController 0))
  (Ability|CommitAbility)
  (|PlayMontageandWaitProxy "None" "/Game/Animation/MC/Slash/AM_Lslash3.AM_Lslash3" 2.0 "None" true 1.0 0.0 false
    (:then
      (Class|BPIGAS|AddAtkMove(Message) (Ability|GetAvatarActorfromActorInfo) 1e+01)
      (Ability|Tasks|WaitGameplayEvent "(TagName=\"Event.ComboWindowOpen\")" 0
        (:then
          (Ability|Tasks|WaitGameplayEvent "(TagName=\"Event.ComboWindowEnd\")" 0
            (:EventReceived
              (Ability|GameplayEffect|RemoveLooseGameplayTags (Ability|GetAvatarActorfromActorInfo) (Variables|Default|GetComboOpenTag))
              (Class|BPIInputBuffer|IBResetAttackState(Message) _returnvalue)
              (Class|BPIGAS|StopAtkMove(Message) (Ability|GetAvatarActorfromActorInfo))
              (Ability|EndAbility))))
        (:EventReceived
          (Ability|GameplayEffect|RemoveLooseGameplayTags (Ability|GetAvatarActorfromActorInfo) (Variables|Default|GetComboOpenTag))
          (Class|BPIInputBuffer|IBSaveLightAttack(Message) _returnvalue))))
    (:OnCompleted
      (Ability|EndAbility :!label _label))
    (:OnInterrupted
      (goto _label))))