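; Gameplay ability for a combo chain attack that plays the AM_ComboChain1 montage, starts attack movement and launches BP_MC upward in Falling mode.
; The ComboWindowOpen event swaps loose tag ChainCW1 for ChainCW2.
; ComboWindowEnd removes ChainCW2, stops attack movement and ends the ability.
; Montage completion or cancellation also ends it, and OnEndAbility clears the ResetTag tags.
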(event Ability|EventActivateAbility
  (bind _returnvalue (Ability|GetAvatarActorfromActorInfo))
  (Ability|CommitAbility)
  (|PlayMontageandWaitProxy "None" "/Game/Animation/MC/Slash/AM_ComboChain1.AM_ComboChain1" 1.0 "None" true 1.0 0.0 false
    (:then
      (Class|BPIGAS|GASAddAtkMove(Message) (Ability|GetAvatarActorfromActorInfo) 1e+01)
      (bind _asbp_mc (Utilities|Casting|CastToBP_MC (Ability|GetAvatarActorfromActorInfo)))
      (Pawn|Components|CharacterMovement|SetMovementMode (Variables|/Script/Engine.Character|GetCharacterMovement _asbp_mc) "MOVE_Falling" 0)
      (Character|LaunchCharacter _asbp_mc "0.000000,0.000000,300.000000" false false)
      (Ability|Tasks|WaitGameplayEvent "(TagName=\"Event.ComboWindowOpen\")" 0
        (:then
          (Ability|Tasks|WaitGameplayEvent "(TagName=\"Event.ComboWindowEnd\")" 0
            (:EventReceived
              (Ability|GameplayEffect|RemoveLooseGameplayTags (Ability|GetAvatarActorfromActorInfo) (Variables|Default|GetChainCW2))
              (Class|BPIGAS|GASStopAtkMove(Message) (Ability|GetAvatarActorfromActorInfo))
              (Ability|EndAbility))))
        (:EventReceived
          (Ability|GameplayEffect|RemoveLooseGameplayTags _returnvalue (Variables|Default|GetChainCW1))
          (Ability|GameplayEffect|AddLooseGameplayTags _returnvalue (Variables|Default|GetChainCW2)))))
    (:OnCompleted
      (Ability|EndAbility :!label _label))
    (:OnCancelled
      (goto _label))))

(event Ability|EventOnEndAbility
  (params (bWasCancelled :type Boolean))
  (Ability|GameplayEffect|RemoveLooseGameplayTags (Ability|GetAvatarActorfromActorInfo) (Variables|Default|GetResetTag)))