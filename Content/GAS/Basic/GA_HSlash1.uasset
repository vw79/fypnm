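; GA_HSlash1 is a Gameplay Ability for the first HSlash attack in a melee combo.
; It commits, sends the H-attack index to the player controller, plays AM_HSlash1 slightly sped up and starts attack movement on the avatar.
; Combo window events add and remove a loose ComboWindowOpen tag; the end event also stops movement and ends the ability.
; Montage completion or cancellation also ends it, and OnEndAbility clears the tag.
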(event Ability|EventActivateAbility
  (Ability|CommitAbility)
  (Class|BPIGAS|GASSetHAttackIndex(Message) (Game|GetPlayerController 0) (Variables|Default|GetHIndex))
  (|PlayMontageandWaitProxy "None" "/Game/Animation/MC/Slash/AM_HSlash1.AM_HSlash1" 1.1 "None" true 1.0 0.0 false
    (:then
      (Class|BPIGAS|GASAddAtkMove(Message) (Ability|GetAvatarActorfromActorInfo) 1e+01)
      (Ability|Tasks|WaitGameplayEvent "(TagName=\"Event.ComboWindowOpen\")" 0
        (:then
          (Ability|Tasks|WaitGameplayEvent "(TagName=\"Event.ComboWindowEnd\")" 0
            (:EventReceived
              (Ability|GameplayEffect|RemoveLooseGameplayTags (Ability|GetAvatarActorfromActorInfo) (Variables|Default|GetComboWindowOpen))
              (Class|BPIGAS|GASStopAtkMove(Message) (Ability|GetAvatarActorfromActorInfo))
              (Ability|EndAbility))))
        (:EventReceived
          (Ability|GameplayEffect|AddLooseGameplayTags (Ability|GetAvatarActorfromActorInfo) (Variables|Default|GetComboWindowOpen)))))
    (:OnCompleted
      (Ability|EndAbility :!label _label))
    (:OnCancelled
      (goto _label))))

(event Ability|EventOnEndAbility
  (params (bWasCancelled :type Boolean))
  (Ability|GameplayEffect|RemoveLooseGameplayTags (Ability|GetAvatarActorfromActorInfo) (Variables|Default|GetComboWindowOpen)))