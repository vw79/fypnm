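; GA_LSlash1 is a Gameplay Ability for a light slash attack, apparently the first step of a combo.
; On activation it commits, reports its attack index to the player controller, plays the slash montage sped up and starts attack movement on the avatar.
; Gameplay events open and close a combo window via a loose tag; closing also stops movement and ends the ability.
; Montage completion or cancellation also ends it, and ending always clears the tag.
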(event Ability|EventActivateAbility
  (Ability|CommitAbility)
  (Class|BPIGAS|GASSetLAttackIndex(Message) (Game|GetPlayerController 0) (Variables|Default|GetLIndex))
  (|PlayMontageandWaitProxy "None" "/Game/Animation/MC/Slash/AM_Lslash1.AM_Lslash1" 1.5 "None" true 1.0 0.0 false
    (:then
      (Class|BPIGAS|GASAddAtkMove(Message) (Ability|GetAvatarActorfromActorInfo) 2.0)
      (Ability|Tasks|WaitGameplayEvent "(TagName=\"Event.ComboWindowOpen\")" 0
        (:then
          (Ability|Tasks|WaitGameplayEvent "(TagName=\"Event.ComboWindowEnd\")" 0
            (:EventReceived
              (Ability|GameplayEffect|RemoveLooseGameplayTags (Ability|GetAvatarActorfromActorInfo) (Variables|Default|GetComboWindowOpen))
              (Class|BPIGAS|GASStopAtkMove(Message) (Ability|GetAvatarActorfromActorInfo))
              (Ability|EndAbility))))
        (:EventReceived
          (Ability|GameplayEffect|AddLooseGameplayTags (Ability|GetAvatarActorfromActorInfo) (Variables|Default|GetComboWindowOpen)))))
    (:OnCompleted
      (Ability|EndAbility :!label _label))
    (:OnCancelled
      (goto _label))))

(event Ability|EventOnEndAbility
  (params (bWasCancelled :type Boolean))
  (Ability|GameplayEffect|RemoveLooseGameplayTags (Ability|GetAvatarActorfromActorInfo) (Variables|Default|GetComboWindowOpen)))