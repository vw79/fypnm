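; Action camera component on BP_MC that briefly cuts to a cinematic side shot of the player and an enemy.
; ToggleActionCam places the level's cine camera beside their midpoint, perpendicular to the line between them, choosing the side from the follow camera's facing via a dot product.
; It blends to that camera aimed slightly above the enemy, disables move and look input, then blends back after a one-second delay.
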(event Custom|ToggleActionCam
  (params (Enemy :type Actor%20Object%20Reference))
  (CallFunction|DisableInput)
  (CallFunction|CalculateNewCamPostoSide Enemy)
  (CallFunction|ChooseSideBaseonOriCam)
  (CallFunction|SwitchCam Enemy)
  (Utilities|FlowControl|Delay 1.0)
  (Game|Player|SetViewTargetwithBlend (Variables|References|GetMcControllerRef) (Variables|References|GetCamChildActorRef) 0.3 "VTBlend_Linear" 0.3 false)
  (CallFunction|EnableInput))

(event EventBeginPlay
  (bind _asbp_mc (Utilities|Casting|CastToBP_MC (Components|GetOwner)))
  (Variables|References|SetMcRef _asbp_mc)
  (bind _asbp_mccontroller (Utilities|Casting|CastToBP_MCController (Game|GetPlayerController 0)))
  (Variables|References|SetMcControllerRef _asbp_mccontroller)
  (bind _returnvalue (Actor|GetActorOfClass "/Game/VW/BP_CineCameraActor.BP_CineCameraActor_C"))
  (Variables|References|SetCineCamRef _returnvalue)
  (Variables|References|SetFollowCamRef (Variables|/Game/ThirdPerson/Blueprints/Player/BP_MC.BP_MC_C|GetFollowCamera (Variables|References|GetMcRef)))
  (Variables|References|SetCamChildActorRef (Variables|/Script/Engine.ChildActorComponent|GetChildActor (Variables|/Game/ThirdPerson/Blueprints/Player/BP_MC.BP_MC_C|GetCamChildActor (Variables|References|GetMcRef)))))

(fn DisableInput
  (bind _mccontrollerref (Variables|References|GetMcControllerRef))
  (Input|DisableInput _mccontrollerref _mccontrollerref)
  (Input|SetIgnoreLookInput _mccontrollerref true))

(fn EnableInput
  (bind _mccontrollerref (Variables|References|GetMcControllerRef))
  (Input|EnableInput (Variables|References|GetMcRef) _mccontrollerref)
  (Input|SetIgnoreLookInput _mccontrollerref false))

(fn CalculateNewCamPostoSide
  (params (Enemy :type Actor%20Object%20Reference))
  (Variables|Calculation|SetMidpoint (/ (+ (Transformation|GetActorLocation (Variables|References|GetMcRef)) (Transformation|GetActorLocation Enemy)) 2.0))
  (Variables|Calculation|SetForwardDirection (Math|Vector|Normalize (- (Transformation|GetActorLocation (Variables|References|GetMcRef)) (Transformation|GetActorLocation Enemy))))
  ;[1 1 1] Get Perpendicular
  (Variables|Calculation|SetRightVector (Math|Vector|CrossProduct (Variables|Calculation|GetForwardDirection) "0.000000,0.000000,1.000000")))

(fn ChooseSideBaseonOriCam
  (if (> (Math|Vector|DotProduct (Math|Vector|GetForwardVector (Variables|References|GetFollowCamRef)) (Variables|Calculation|GetRightVector)) 0.0)
    (Variables|Calculation|SetNewCamPosition (+ (- (Variables|Calculation|GetMidpoint) (* (Variables|Calculation|GetRightVector) (Variables|Default|GetCamSideOffset))) (* (Math|Vector|VectorUp) (Variables|Default|GetCamHeightOfftset))))
    (else
      (Variables|Calculation|SetNewCamPosition (+ (+ (Variables|Calculation|GetMidpoint) (* (Variables|Calculation|GetRightVector) (Variables|Default|GetCamSideOffset))) (* (Math|Vector|VectorUp) (Variables|Default|GetCamHeightOfftset)))))))

(fn SwitchCam
  (params (Enemy :type Actor%20Object%20Reference))
  (bind _returnvalue (Transformation|GetActorLocation Enemy))
  (bind _cinecamref (Variables|References|GetCineCamRef))
  (Transformation|SetActorLocation _cinecamref (Variables|Calculation|GetNewCamPosition) false false)
  (Transformation|SetActorRotation _cinecamref (Math|Rotator|FindLookatRotation (Variables|Calculation|GetNewCamPosition) (+ (Math|Vector|MakeVector (.x _returnvalue) (.y _returnvalue) (+ (.z _returnvalue) 5e+01)) (Transformation|GetActorForwardVector Enemy))))
  (Game|Player|SetViewTargetwithBlend (Variables|References|GetMcControllerRef) _cinecamref 0.3 "VTBlend_Cubic" 0.3 false))