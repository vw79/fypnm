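; Gameplay Ability for the first light slash, which commits, plays its montage at increased rate and starts attack movement on the avatar.
; Gameplay events open and close a combo window, toggling a loose tag and messaging the player controller's input buffer to save light attack or reset attack state.
; Window end also stops attack movement and ends the ability; montage completion or interruption only ends it.
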(event Ability|EventActivateAbility
  (bind _returnvalue (Game|GetPlayerController 0))
  (Ability|CommitAbility)
  (|PlayMontageandWaitProxy "None" "/Game/VW/Slash/AM_Lslash1.AM_Lslash1" 2.0 "None" true 1.0 0.0 false
    (:then
      (Class|BPIGAS|AddAtkMove(Message) (Ability|GetAvatarActorfromActorInfo) 2.0)
      (Ability|Tasks|WaitGameplayEvent "(TagName=\"Event.ComboWindowOpen\")" 0
        (:then
          (Ability|Tasks|WaitGameplayEvent "(TagName=\"Event.ComboWindowEnd\")" 0
            (:EventReceived
              (Ability|GameplayEffect|RemoveLooseGameplayTags (Ability|GetAvatarActorfromActorInfo) (Variables|Default|GetComboWindowOpen))
              (Class|BPIInputBuffer|IBResetAttackState(Message) _returnvalue)
              (Class|BPIGAS|StopAtkMove(Message) (Ability|GetAvatarActorfromActorInfo))
              (Ability|EndAbility))))
        (:EventReceived
          (Ability|GameplayEffect|AddLooseGameplayTags (Ability|GetAvatarActorfromActorInfo) (Variables|Default|GetComboWindowOpen))
          (Class|BPIInputBuffer|IBSaveLightAttack(Message) _returnvalue))))
    (:OnCompleted
      (Ability|EndAbility :!label _label))
    (:OnInterrupted
      (goto _label))))

(event Ability|EventOnEndAbility
  (params (bWasCancelled :type Boolean))
  (if bWasCancelled
    (Development|PrintString "cancel")))