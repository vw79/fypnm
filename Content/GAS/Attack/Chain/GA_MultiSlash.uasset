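; GA_MultiSlash is a Gameplay Ability for a melee multi-slash step in an attack chain.
; On activation it boosts post-process intensity, starts the slash Niagara effect, plays a montage and adds attack movement.
; Gameplay events toggle the weapon and swap combo tag ChainCW1 for ChainCW2, with window end stopping movement and the ability.
; Ending resets post-process settings, deactivates the effect and clears ChainCW2.
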(event Ability|EventActivateAbility
  (bind _returnvalue (Ability|GetAvatarActorfromActorInfo))
  (Ability|CommitAbility)
  (bind _mc (Class|BPIGAS|GASGetMcRef(Message) (Ability|GetAvatarActorfromActorInfo)))
  (Variables|/Script/Engine.PostProcessComponent|SetSettings (Variables|/Game/ThirdPerson/Blueprints/Player/BP_MC.BP_MC_C|GetPP%20Volume _mc) (Utilities|Struct|MakePostProcessSettings 2.0 1.0))
  (Components|Activation|Activate (Variables|/Game/ThirdPerson/Blueprints/Player/BP_MC.BP_MC_C|GetNS_MultiSlash _mc) false)
  (|PlayMontageandWaitProxy "None" "/Game/Characters/Mel/Anim/Attack/Chain/AM_Combo1_Mel.AM_Combo1_Mel" 1.0 "None" true 1.0 0.0 false
    (:then
      (Ability|Tasks|WaitGameplayEvent "(TagName=\"Event.EquipWeapon\")" 0
        (:then
          (Class|BPIGAS|GASAddAtkMove(Message) (Ability|GetAvatarActorfromActorInfo) 2e+01)
          (Ability|Tasks|WaitGameplayEvent "(TagName=\"Event.ComboWindowOpen\")" 0
            (:then
              (Ability|Tasks|WaitGameplayEvent "(TagName=\"Event.UnequipWeapon\")" 0
                (:then
                  (Ability|Tasks|WaitGameplayEvent "(TagName=\"Event.ComboWindowEnd\")" 0
                    (:EventReceived
                      (Ability|GameplayEffect|RemoveLooseGameplayTags (Ability|GetAvatarActorfromActorInfo) (Variables|Default|GetChainCW2))
                      (Class|BPIGAS|GASStopAtkMove(Message) (Ability|GetAvatarActorfromActorInfo))
                      (Ability|EndAbility))))
                (:EventReceived
                  (bind _mc_2 (Class|BPIGAS|GASGetMcRef(Message) (Ability|GetAvatarActorfromActorInfo)))
                  (Default|UnequipWeapon (Variables|/Game/ThirdPerson/Blueprints/Player/BP_MC.BP_MC_C|GetWeaponRef _mc_2)))))
            (:EventReceived
              (Ability|GameplayEffect|AddLooseGameplayTags _returnvalue (Variables|Default|GetChainCW2))
              (Ability|GameplayEffect|RemoveLooseGameplayTags _returnvalue (Variables|Default|GetChainCW1)))))
        (:EventReceived
          (Default|EquipWeapon (Variables|/Game/ThirdPerson/Blueprints/Player/BP_MC.BP_MC_C|GetWeaponRef _mc)))))
    (:OnCompleted
      (Ability|EndAbility :!label _label))
    (:OnInterrupted
      (goto _label))
    (:OnCancelled
      (goto _label))))

(event Ability|EventOnEndAbility
  (params (bWasCancelled :type Boolean))
  (Variables|/Script/Engine.PostProcessComponent|SetSettings (Variables|/Game/ThirdPerson/Blueprints/Player/BP_MC.BP_MC_C|GetPP%20Volume (stale Ability|EventActivateAbility _mc)) (Utilities|Struct|MakePostProcessSettings 0.0))
  (Ability|GameplayEffect|RemoveLooseGameplayTags (Ability|GetAvatarActorfromActorInfo) (Variables|Default|GetChainCW2))
  (Components|Activation|Deactivate (Variables|/Game/ThirdPerson/Blueprints/Player/BP_MC.BP_MC_C|GetNS_MultiSlash (stale Ability|EventActivateAbility _mc))))