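; Gameplay ability that starts a melee combo chain by playing the combo-start montage.
; Parallel gameplay-event waits let the montage unequip the character's weapon through an interface reference and open the combo window.
; The window opening adds a non-replicated ChainCW1 loose tag, and its closing removes the tag and ends the ability.
; Montage completion, interruption or cancellation also ends it, with OnEndAbility clearing the tag as cleanup.
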(event Ability|EventActivateAbility
  (Ability|CommitAbility)
  (|PlayMontageandWaitProxy "None" "/Game/Characters/Mel/Anim/Attack/Chain/AM_ComboStart_Mel.AM_ComboStart_Mel" 1.2 "None" true 1.0 0.0 false
    (:then
      (Ability|Tasks|WaitGameplayEvent "(TagName=\"Event.UnequipWeapon\")" 0
        (:then
          (Ability|Tasks|WaitGameplayEvent "(TagName=\"Event.ComboWindowOpen\")" 0
            (:then
              (Ability|Tasks|WaitGameplayEvent "(TagName=\"Event.ComboWindowEnd\")" 0
                (:EventReceived
                  (Ability|GameplayEffect|RemoveLooseGameplayTags (Ability|GetAvatarActorfromActorInfo) (Variables|Default|GetChainCW1))
                  (Ability|EndAbility))))
            (:EventReceived
              (Ability|GameplayEffect|AddLooseGameplayTags (Ability|GetAvatarActorfromActorInfo) (Variables|Default|GetChainCW1)))))
        (:EventReceived
          (bind _mc (Class|BPIGAS|GASGetMcRef(Message) (Ability|GetAvatarActorfromActorInfo)))
          (Default|UnequipWeapon (Variables|/Game/ThirdPerson/Blueprints/Player/BP_MC.BP_MC_C|GetWeaponRef _mc)))))
    (:OnCompleted
      (Ability|EndAbility :!label _label))
    (:OnInterrupted
      (goto _label))
    (:OnCancelled
      (goto _label))))

(event Ability|EventOnEndAbility
  (params (bWasCancelled :type Boolean))
  (Ability|GameplayEffect|RemoveLooseGameplayTags (Ability|GetAvatarActorfromActorInfo) (Variables|Default|GetChainCW1)))