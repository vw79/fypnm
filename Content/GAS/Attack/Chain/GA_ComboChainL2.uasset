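; Gameplay ability for a melee combo chain attack that plays the Combo2 montage with a sword slash effect.
; On activation it raises post-process intensities, adds attack movement, spawns the slash and starts listening for montage-phase gameplay events.
; Those events equip and unequip the weapon, and the combo-window end clears reset tags, stops movement and ends the ability.
; Montage completion or interruption also ends it; ending resets post-processing and tags.
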(event Ability|EventActivateAbility
  (Ability|CommitAbility)
  (|PlayMontageandWaitProxy "None" "/Game/Characters/Mel/Anim/Attack/Chain/AM_Combo2_Mel.AM_Combo2_Mel" 1.0 "None" true 1.0 0.0 false
    (:then
      (bind _mc (Class|BPIGAS|GASGetMcRef(Message) (Ability|GetAvatarActorfromActorInfo)))
      (Variables|/Script/Engine.PostProcessComponent|SetSettings (Variables|/Game/ThirdPerson/Blueprints/Player/BP_MC.BP_MC_C|GetPP%20Volume _mc) (Utilities|Struct|MakePostProcessSettings 2.0 1.0))
      (Ability|Tasks|WaitGameplayEvent "(TagName=\"Event.EquipWeapon\")" 0
        (:then
          (Class|BPIGAS|GASAddAtkMove(Message) (Ability|GetAvatarActorfromActorInfo) 3e+01)
          (Niagara|SpawnSystematLocation "/Game/Roi/VFX/NS_SwordSlash.NS_SwordSlash" (+ (Transformation|GetActorLocation _mc) (Math|Vector|MakeVector 5e+01 0.0 0.0)) (Transformation|GetActorRotation _mc))
          (Ability|Tasks|WaitGameplayEvent "(TagName=\"Event.UnequipWeapon\")" 0
            (:then
              (Ability|Tasks|WaitGameplayEvent "(TagName=\"Event.ComboWindowEnd\")" 0
                (:EventReceived
                  (Ability|GameplayEffect|RemoveLooseGameplayTags (Ability|GetAvatarActorfromActorInfo) (Variables|Default|GetResetTag))
                  (Class|BPIGAS|GASStopAtkMove(Message) (Ability|GetAvatarActorfromActorInfo))
                  (Ability|EndAbility))))
            (:EventReceived
              (Default|UnequipWeapon (Variables|/Game/ThirdPerson/Blueprints/Player/BP_MC.BP_MC_C|GetWeaponRef _mc)))))
        (:EventReceived
          (Default|EquipWeapon (Variables|/Game/ThirdPerson/Blueprints/Player/BP_MC.BP_MC_C|GetWeaponRef _mc)))))
    (:OnCompleted
      (Ability|EndAbility :!label _label))
    (:OnInterrupted
      (goto _label))
    (:OnCancelled
      (goto _label))))

(event Ability|EventOnEndAbility
  (params (bWasCancelled :type Boolean))
  (Variables|/Script/Engine.PostProcessComponent|SetSettings (Variables|/Game/ThirdPerson/Blueprints/Player/BP_MC.BP_MC_C|GetPP%20Volume (stale Ability|EventActivateAbility _mc)) (Utilities|Struct|MakePostProcessSettings 0.0))
  (Ability|GameplayEffect|RemoveLooseGameplayTags (Ability|GetAvatarActorfromActorInfo) (Variables|Default|GetResetTag)))