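; Gameplay ability that starts the MultiSlash chain attack by playing the melee combo-start montage on the avatar.
; On activation it commits, flags ability-or-rage use on the main character, then listens for gameplay event tags while the montage plays.
; The unequip event unequips the weapon, combo-window open calls MultiSlash on the player controller, and combo-window end ends the ability.
; Montage completion, interruption or cancellation also ends it.
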(event Ability|EventActivateAbility
  (Ability|CommitAbility)
  (bind _mc (Class|BPIGAS|GASGetMcRef(Message) (Ability|GetAvatarActorfromActorInfo)))
  (Default|AbilityorRageUsed _mc true)
  (|PlayMontageandWaitProxy "None" "/Game/Characters/Mel/Anim/Attack/Chain/AM_ComboStart_Mel.AM_ComboStart_Mel" 1.2 "None" true 1.0 0.0 false
    (:then
      (Ability|Tasks|WaitGameplayEvent "(TagName=\"Event.UnequipWeapon\")" 0
        (:then
          (Ability|Tasks|WaitGameplayEvent "(TagName=\"Event.ComboWindowOpen\")" 0
            (:then
              (Ability|Tasks|WaitGameplayEvent "(TagName=\"Event.ComboWindowEnd\")" 0
                (:EventReceived
                  (Ability|EndAbility))))
            (:EventReceived
              (bind _mccontroller (Class|BPIGAS|GASGetMcControllerRef(Message) (Game|GetPlayerController 0)))
              (Default|MultiSlash _mccontroller))))
        (:EventReceived
          (bind _mc_2 (Class|BPIGAS|GASGetMcRef(Message) (Ability|GetAvatarActorfromActorInfo)))
          (Default|UnequipWeapon (Variables|/Game/ThirdPerson/Blueprints/Player/BP_MC.BP_MC_C|GetWeaponRef _mc_2)))))
    (:OnCompleted
      (Ability|EndAbility :!label _label))
    (:OnInterrupted
      (goto _label))
    (:OnCancelled
      (goto _label))))