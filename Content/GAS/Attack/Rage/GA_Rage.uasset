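; GA_Rage is a gameplay ability that puts the player character into a timed rage mode.
; Activation commits, plays a sound and montage, notifies the character of rage use, raises the combo counter's TweakFactor and applies GE_Rage.
; A looping one-second timer counts RageDuration up to the effect's rounded remaining duration, then lowers TweakFactor and ends the ability.
; Montage completion, interruption or cancellation also ends the ability, without resetting TweakFactor.
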(event Custom|RageMode
  (if (< (Variables|Default|GetRageDuration) (Math|Float|Round (stale Ability|EventActivateAbility _returnvalue_2)))
    (bind _result (Math|Integer|IncrementInt (Variables|Default|GetRageDuration))
      (:%20%20
        (Development|PrintString (Utilities|String|Append "Rage Timer" " " (Utilities|String|ToString(Integer) _result)))))
    (else
      (CallFunction|StopRageTimer))))

(event Custom|StopRageTimer
  (Utilities|Time|ClearandInvalidateTimerbyHandle (stale Ability|EventActivateAbility _returnvalue_3))
  (bind _combocounter (Class|BPIGAS|GASGetMcRef(Message) (Ability|GetAvatarActorfromActorInfo)))
  (Variables|/Game/GAS/BPC_ComboCounter.BPC_ComboCounter_C|SetTweakFactor _combocounter 0.8)
  (Development|PrintString "rage reset")
  (Ability|EndAbility))

(event Ability|EventActivateAbility
  (Audio|PlaySound2D "/Game/SFX/Rage.Rage" 1.0 1.0 0.0 0 0)
  (Ability|CommitAbility)
  (|PlayMontageandWaitProxy "None" "/Game/Characters/Mel/Anim/Attack/AM_Rage_Mel.AM_Rage_Mel" 1.3 "None" true 1.0 0.0 false
    (:then
      (bind (_mc _gas _targeting _actioncam _combocounter) (Class|BPIGAS|GASGetMcRef(Message) (Ability|GetAvatarActorfromActorInfo)))
      (Default|AbilityorRageUsed _mc false) ; This is Rage
      (Variables|/Game/GAS/BPC_ComboCounter.BPC_ComboCounter_C|SetTweakFactor _combocounter 1.2)
      (bind _returnvalue (Ability|ApplyGameplayEffectToOwner "/Game/GAS/Attack/Rage/GE_Rage.GE_Rage_C"))
      (bind _structout (Utilities|Struct|SetmembersinActiveGameplayEffectHandle _returnvalue))
      (bind _returnvalue_2 (Ability|GameplayEffect|GetActiveGameplayEffectRemainingDuration _structout))
      (bind _returnvalue_3 (Utilities|Time|SetTimerbyEvent (delegate Custom|RageMode) 1.0 true)))
    (:OnCompleted
      (Ability|EndAbility :!label _label))
    (:OnInterrupted
      (goto _label))
    (:OnCancelled
      (goto _label))))