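; Gameplay ability that handles the main character's reaction to being hurt.
; On activation it commits, fetches the character and combo counter through an avatar message, triggers the hurt cue, grants brief invincibility and drops the combo rank.
; It then plays a directional hit montage chosen by the character's hit direction, ending the ability when the montage blends out or is interrupted.
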(event Ability|EventActivateAbility
  (Ability|CommitAbility)
  (bind (_mc _gas _targeting _actioncam _combocounter) (Class|BPIGAS|GASGetMcRef(Message) (Ability|GetAvatarActorfromActorInfo)))
  (Default|HurtGameplayCue _mc)
  (Default|InvinciblewithDelay _mc 2.0)
  (Default|DropRank _combocounter)
  (switch Utilities|FlowControl|Switch|SwitchonE_DirectionalHit (Variables|/Game/ThirdPerson/Blueprints/Player/BP_MC.BP_MC_C|GetHit%20Direction _mc)
    (:NewEnumerator0
      (|PlayMontageandWaitProxy "None" (Utilities|Array|Get(acopy) (Variables|Default|GetHitAnimation)) 1.2 "None" true 1.0 0.0 false
        (:OnBlendOut
          _)
        (:OnInterrupted
          _)))
    (:NewEnumerator1
      (|PlayMontageandWaitProxy "None" (Utilities|Array|Get(acopy) (Variables|Default|GetHitAnimation) 1) 1.2 "None" true 1.0 0.0 false
        (:OnBlendOut
          _)
        (:OnInterrupted
          _)))
    (:NewEnumerator2
      (|PlayMontageandWaitProxy "None" (Utilities|Array|Get(acopy) (Variables|Default|GetHitAnimation) 2) 1.2 "None" true 1.0 0.0 false
        (:OnBlendOut
          _)
        (:OnInterrupted
          _)))
    (:NewEnumerator3
      (|PlayMontageandWaitProxy "None" (Utilities|Array|Get(acopy) (Variables|Default|GetHitAnimation) 3) 1.2 "None" true 1.0 0.0 false
        (:OnBlendOut
          _)
        (:OnInterrupted
          _))))
  (Ability|EndAbility))