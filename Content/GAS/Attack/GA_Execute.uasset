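; Gameplay ability for the main character's execution attack on the hard-locked target, which also heals the character.
; It plays the execute montage, motion-warps to just in front of the target with yaw toward it, and ignores Pawn collision meanwhile.
; Global time slows while the character's custom dilation compensates, keeping them at normal speed.
; The ability ends with the montage, restoring collision and both time dilations.
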(event Ability|EventActivateAbility
  (Ability|CommitAbility)
  (|PlayMontageandWaitProxy "None" "/Game/Animation/MC/AM_Execute.AM_Execute" 1.0 "None" true 1.0 0.0 false
    (:then
      (bind (_mc _gas _targeting) (Class|BPIGAS|GASGetMcRef(Message) (Ability|GetAvatarActorfromActorInfo)))
      (Utilities|Time|SetGlobalTimeDilation 0.2)
      (Variables|/Script/Engine.Actor|SetCustomTimeDilation _mc 5.0)
      (Collision|SetCollisionResponsetoChannel (Variables|/Script/Engine.Character|GetCapsuleComponent _mc) "ECC_Pawn" "ECR_Ignore")
      (Class|MotionWarpingComponent|AddorUpdateWarpTargetfromLocationandRotation (Variables|/Game/ThirdPerson/Blueprints/Player/BP_MC.BP_MC_C|GetMotionWarping _mc) "Execute" (+ (Transformation|GetActorLocation (Variables|/Game/Blueprints/Component/BPC_TargetingSystem.BPC_TargetingSystem_C|GetHardLockedOnActor _targeting)) (* (Transformation|GetActorForwardVector (Variables|/Game/Blueprints/Component/BPC_TargetingSystem.BPC_TargetingSystem_C|GetHardLockedOnActor _targeting)) 1.2e+02)) (Math|Rotator|MakeRotator (.roll (Transformation|GetActorRotation _mc)) (.pitch (Transformation|GetActorRotation _mc)) (.yaw (Math|Rotator|FindLookatRotation (Transformation|GetActorLocation _mc) (Transformation|GetActorLocation (Variables|/Game/Blueprints/Component/BPC_TargetingSystem.BPC_TargetingSystem_C|GetHardLockedOnActor _targeting))))))
      (Default|HealMc _mc))
    (:OnCompleted
      (Ability|EndAbility :!label _label))
    (:OnInterrupted
      (goto _label))
    (:OnCancelled
      (goto _label))))

(event Ability|EventOnEndAbility
  (params (bWasCancelled :type Boolean))
  (bind _mc (Class|BPIGAS|GASGetMcRef(Message) (Ability|GetAvatarActorfromActorInfo)))
  (Collision|SetCollisionResponsetoChannel (Variables|/Script/Engine.Character|GetCapsuleComponent _mc) "ECC_Pawn" "ECR_Block")
  (Utilities|Time|SetGlobalTimeDilation 1.0)
  (Variables|/Script/Engine.Actor|SetCustomTimeDilation _mc 1.0))