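; Gameplay ability for the second light slash of an air combo.
; On activation it commits, plays the air slash montage sped up and messages the avatar to start attack movement.
; Gameplay events for combo window open and end swap loose tags from AirComboWindow1 to AirComboWindow2, then clear it, stop movement and end the ability.
; Montage completion or interruption also ends it, with tag cleanup on end.
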(event Ability|EventActivateAbility
  (bind _returnvalue (Ability|GetAvatarActorfromActorInfo))
  (Ability|CommitAbility)
  (|PlayMontageandWaitProxy "None" "/Game/Animation/MC/Slash/AM_Air_Lslash2.AM_Air_Lslash2" 1.5 "None" true 1.0 0.0 false
    (:then
      (Class|BPIGAS|GASAddAtkMove(Message) (Ability|GetAvatarActorfromActorInfo) 2.0)
      (Ability|Tasks|WaitGameplayEvent "(TagName=\"Event.ComboWindowOpen\")" 0
        (:then
          (Ability|Tasks|WaitGameplayEvent "(TagName=\"Event.ComboWindowEnd\")" 0
            (:EventReceived
              (Ability|GameplayEffect|RemoveLooseGameplayTags (Ability|GetAvatarActorfromActorInfo) (Variables|Default|GetAirComboWindow2))
              (Class|BPIGAS|GASStopAtkMove(Message) (Ability|GetAvatarActorfromActorInfo))
              (Ability|EndAbility))))
        (:EventReceived
          (Ability|GameplayEffect|RemoveLooseGameplayTags _returnvalue (Variables|Default|GetAirComboWindow1))
          (Ability|GameplayEffect|AddLooseGameplayTags _returnvalue (Variables|Default|GetAirComboWindow2)))))
    (:OnCompleted
      (Ability|EndAbility :!label _label))
    (:OnInterrupted
      (goto _label))
    (:OnCancelled
      (goto _label))))

(event Ability|EventOnEndAbility
  (params (bWasCancelled :type Boolean))
  (Ability|GameplayEffect|RemoveLooseGameplayTags (Ability|GetAvatarActorfromActorInfo) (Variables|Default|GetAirComboWindow2)))