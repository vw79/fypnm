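; GA_Launch is a Gameplay Ability for a launcher attack that sends the player and the hard-locked enemy into a launch.
; On activation it equips the weapon and plays the launch montage, then waits for the combo-window gameplay event.
; If the locked enemy is valid, alive, among the weapon's traced hits and not a BP_Titan, it messages the avatar to launch both and ends.
; Otherwise the ability ends with the montage.
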(event Ability|EventActivateAbility
  (Ability|CommitAbility)
  (bind _mc (Class|BPIGAS|GASGetMcRef(Message) (Ability|GetAvatarActorfromActorInfo)))
  (Default|EquipWeapon (Variables|/Game/ThirdPerson/Blueprints/Player/BP_MC.BP_MC_C|GetWeaponRef _mc))
  (|PlayMontageandWaitProxy "None" "/Game/Characters/Megan/Anim/Attack/Air/AM_Launch_Megan.AM_Launch_Megan" 1.0 "None" true 1.0 0.0 false
    (:then
      (Ability|Tasks|WaitGameplayEvent "(TagName=\"Event.ComboWindowOpen\")" 0
        (:EventReceived
          (bind (_mc_2 _gas _targeting _actioncam _combocounter _weapon_collision) (Class|BPIGAS|GASGetMcRef(Message) (Ability|GetAvatarActorfromActorInfo)))
          (bind (_demonbase _isdead) (Default|GetHardLockEnemy _targeting))
          (if (Math|Boolean|ANDBoolean (Utilities|IsValid _demonbase) (not _isdead) (Utilities|Array|ContainsItem (Variables|/Game/GAS/BPC_WeaponCollision.BPC_WeaponCollision_C|GetTracedEnemies _weapon_collision) _demonbase) (not (== (Utilities|GetClass _demonbase) "/Game/AI/Blueprints/Titan/BP_Titan.BP_Titan_C")))
            (Class|BPIGAS|GASLaunchPlayer&Enemy(Message) (Ability|GetAvatarActorfromActorInfo))
            (Ability|EndAbility)))))
    (:OnCompleted
      (Ability|EndAbility :!label _label))
    (:OnInterrupted
      (goto _label))
    (:OnCancelled
      (goto _label))))