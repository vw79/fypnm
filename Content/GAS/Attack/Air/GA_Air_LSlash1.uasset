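; GA_Air_LSlash1 is a Gameplay Ability for an airborne slash attack, apparently the first of an air combo.
; On activation it commits, equips the weapon, plays the air attack montage and starts attack movement on the avatar.
; Montage gameplay events add and remove the AirComboWindow tag, with window end also stopping movement and ending the ability.
; A looping timer at frame-delta interval polls IsFalling to end it upon landing.
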(event Custom|StartAirAtkTimer
  (if (not (AI|Components|NavMovement|IsFalling (stale Ability|EventActivateAbility _movement)))
    (CallFunction|StopAirAtkTimer)))

(event Custom|StopAirAtkTimer
  (Utilities|Time|ClearandInvalidateTimerbyHandle (stale Ability|EventActivateAbility _returnvalue))
  (Ability|EndAbility)
  (Development|PrintString "aa1"))

(event Ability|EventActivateAbility
  (Ability|CommitAbility)
  (bind (_mc _gas _targeting _actioncam _combocounter _weapon_collision _movement) (Class|BPIGAS|GASGetMcRef(Message) (Ability|GetAvatarActorfromActorInfo)))
  (Default|EquipWeapon (Variables|/Game/ThirdPerson/Blueprints/Player/BP_MC.BP_MC_C|GetWeaponRef _mc))
  (bind _returnvalue (Utilities|Time|SetTimerbyEvent (delegate Custom|StartAirAtkTimer) (Utilities|Time|GetWorldDeltaSeconds) true))
  (|PlayMontageandWaitProxy "None" "/Game/Characters/Megan/Anim/Attack/Air/AM_AirAttack1_Megan.AM_AirAttack1_Megan" 1.5 "None" true 1.0 0.0 false
    (:then
      (Class|BPIGAS|GASAddAtkMove(Message) (Ability|GetAvatarActorfromActorInfo) 2.0)
      (Ability|Tasks|WaitGameplayEvent "(TagName=\"Event.ComboWindowOpen\")" 0
        (:then
          (Ability|Tasks|WaitGameplayEvent "(TagName=\"Event.ComboWindowEnd\")" 0
            (:EventReceived
              (Ability|GameplayEffect|RemoveLooseGameplayTags (Ability|GetAvatarActorfromActorInfo) (Variables|Default|GetAirComboWindow))
              (Class|BPIGAS|GASStopAtkMove(Message) (Ability|GetAvatarActorfromActorInfo))
              (Ability|EndAbility))))
        (:EventReceived
          (Ability|GameplayEffect|AddLooseGameplayTags (Ability|GetAvatarActorfromActorInfo) (Variables|Default|GetAirComboWindow)))))
    (:OnCompleted
      (Ability|EndAbility :!label _label))
    (:OnInterrupted
      (goto _label))
    (:OnCancelled
      (goto _label))))

(event Ability|EventOnEndAbility
  (params (bWasCancelled :type Boolean))
  (Ability|GameplayEffect|RemoveLooseGameplayTags (Ability|GetAvatarActorfromActorInfo) (Variables|Default|GetAirComboWindow)))