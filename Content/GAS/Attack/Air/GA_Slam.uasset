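; GA_Slam is a Gameplay Ability for an aerial slam attack that drives the player, and an airborne locked-on demon, downward.
; It commits and plays AM_Slam, then on the ComboWindowOpen event sets the controller's IsSlam flag and launches both characters straight down.
; The ability ends on ComboWindowEnd or montage completion or interruption, removing the ResetTag loose tags and clearing IsSlam.
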(event Ability|EventActivateAbility
  (Ability|CommitAbility)
  (|PlayMontageandWaitProxy "None" "/Game/Animation/MC/Slash/AM_Slam.AM_Slam" 1.0 "None" true 1.0 0.0 false
    (:then
      (Ability|Tasks|WaitGameplayEvent "(TagName=\"Event.ComboWindowOpen\")" 0
        (:then
          (Ability|Tasks|WaitGameplayEvent "(TagName=\"Event.ComboWindowEnd\")" 0
            (:EventReceived
              (Ability|EndAbility))))
        (:EventReceived
          (bind _asbp_mccontroller (Utilities|Casting|CastToBP_MCController (Game|GetPlayerController 0)))
          (Variables|/Game/Blueprints/BP_MCController.BP_MCController_C|SetisSlam _asbp_mccontroller true)
          (bind _asbp_mc (Utilities|Casting|CastToBP_MC (Ability|GetAvatarActorfromActorInfo)))
          (Character|LaunchCharacter _asbp_mc "0.000000,0.000000,-1500.000000" true true)
          (bind _asbp_demon_base (Utilities|Casting|CastToBP_Demon_Base (Variables|/Game/Blueprints/Component/BPC_TargetingSystem.BPC_TargetingSystem_C|GetHardLockedOnActor (Variables|/Game/ThirdPerson/Blueprints/Player/BP_MC.BP_MC_C|GetBPC_TargetingSystem _asbp_mc))))
          (if (AI|Components|NavMovement|IsFalling (Variables|/Script/Engine.Character|GetCharacterMovement _asbp_demon_base))
            (Character|LaunchCharacter _asbp_demon_base "0.000000,0.000000,-1500.000000" true true)))))
    (:OnCompleted
      (Ability|EndAbility :!label _label))
    (:OnInterrupted
      (goto _label))))

(event Ability|EventOnEndAbility
  (params (bWasCancelled :type Boolean))
  (Ability|GameplayEffect|RemoveLooseGameplayTags (Ability|GetAvatarActorfromActorInfo) (Variables|Default|GetResetTag))
  (bind _asbp_mccontroller (Utilities|Casting|CastToBP_MCController (Game|GetPlayerController 0)))
  (Variables|/Game/Blueprints/BP_MCController.BP_MCController_C|SetisSlam _asbp_mccontroller false))