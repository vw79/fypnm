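; GA_Satanic is a gameplay ability that applies the GE_Satanic effect to its owner for a timed Satanic state.
; On activation it commits, calls AbilityUsed on the avatar's MC reference and reads the applied effect's remaining duration.
; A looping one-second timer increments SatanicDuration until it reaches that rounded duration, then clears itself and ends the ability.
; SatanicDuration is never reset in this graph.
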(event Custom|SatanicTimer
  (if (< (Variables|Default|GetSatanicDuration) (Math|Float|Round (stale Ability|EventActivateAbility _returnvalue_2)))
    (bind _result (Math|Integer|IncrementInt (Variables|Default|GetSatanicDuration)))
    (else
      (CallFunction|StopSatanicTimer))))

(event Custom|StopSatanicTimer
  (Utilities|Time|ClearandInvalidateTimerbyHandle (stale Ability|EventActivateAbility _returnvalue_3))
  (Development|PrintString "satanic end")
  (Ability|EndAbility))

(event Ability|EventActivateAbility
  (Ability|CommitAbility)
  (bind _mc (Class|BPIGAS|GASGetMcRef(Message) (Ability|GetAvatarActorfromActorInfo)))
  (Default|AbilityUsed _mc)
  (bind _returnvalue (Ability|ApplyGameplayEffectToOwner "/Game/GAS/Attack/Ability/GE_Satanic.GE_Satanic_C"))
  (bind _structout (Utilities|Struct|SetmembersinActiveGameplayEffectHandle _returnvalue))
  (bind _returnvalue_2 (Ability|GameplayEffect|GetActiveGameplayEffectRemainingDuration _structout))
  (bind _returnvalue_3 (Utilities|Time|SetTimerbyEvent (delegate Custom|SatanicTimer) 1.0 true)))