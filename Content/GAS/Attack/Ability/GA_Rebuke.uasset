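; Gameplay ability for the player's Rebuke attack, which damages and knocks back nearby enemies.
; On activation it commits, notifies the MC and plays the 360 attack montage, immediately sphere-tracing a short distance forward for Enemy-tagged pawns.
; Each unique hit takes damage, shows its health bar and is launched along a fixed world-space vector rather than away from the player.
; Montage completion, interruption or cancellation ends the ability, hiding those health bars.
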(event Ability|EventActivateAbility
  (bind _returnvalue (Ability|GetAvatarActorfromActorInfo))
  (Ability|CommitAbility)
  (bind _mc (Class|BPIGAS|GASGetMcRef(Message) (Ability|GetAvatarActorfromActorInfo)))
  (Default|AbilityUsed _mc)
  (Utilities|Array|Clear (Variables|Default|GetEnemies))
  (|PlayMontageandWaitProxy "None" "/Game/AI/Animations/Animation_Sequence/Manny/AM_360Attack.AM_360Attack" 1.0 "None" true 1.0 0.0 false
    (:then
      (bind _mc_2 (Class|BPIGAS|GASGetMcRef(Message) _returnvalue))
      (bind (_outhits _returnvalue_2) (Collision|MultiSphereTraceForObjects (Transformation|GetActorLocation _mc_2) (+ (Transformation|GetActorLocation _mc_2) (* (Math|Vector|GetForwardVector (Transformation|GetActorRotation _mc_2)) 1.3e+02)) 125.0 (Utilities|Array|MakeArray "ObjectTypeQuery3") false (Utilities|Array|MakeArray _returnvalue) "None"))
      (for _array_element _outhits
        (if _returnvalue_2
          (if (Actor|ActorHasTag (.HitActor (Collision|BreakHitResult _array_element)) "Enemy")
            (if (not (Utilities|Array|ContainsItem (Variables|Default|GetEnemies) (.HitActor (Collision|BreakHitResult _array_element))))
              (Utilities|Array|AddUnique (Variables|Default|GetEnemies) (.HitActor (Collision|BreakHitResult _array_element)))
              (Default|DamageEnemy _mc_2 (.HitActor (Collision|BreakHitResult _array_element)) 25.0)
              (bind _enemy (Class|BPIDemon|GetDemonRef(Message) (.HitActor (Collision|BreakHitResult _array_element))))
              (Rendering|SetVisibility (Variables|/Game/AI/Blueprints/BP_Demon_Base.BP_Demon_Base_C|GetHealth%20Bar%20Widget _enemy) true false)
              (Character|LaunchCharacter _enemy "1000.000000,1000.000000,0.000000" true true))))))
    (:OnCompleted
      (Ability|EndAbility :!label _label))
    (:OnInterrupted
      (goto _label))
    (:OnCancelled
      (goto _label))))

(event Ability|EventOnEndAbility
  (params (bWasCancelled :type Boolean))
  (for _array_element (Variables|Default|GetEnemies)
    (bind _enemy (Class|BPIDemon|GetDemonRef(Message) _array_element))
    (Rendering|SetVisibility (Variables|/Game/AI/Blueprints/BP_Demon_Base.BP_Demon_Base_C|GetHealth%20Bar%20Widget _enemy) false false)))