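; GA_HSlash3 is a gameplay ability for the third heavy slash attack of a combo.
; On activation it commits, plays the AM_HSlash3 montage slightly sped up, and tells the avatar to start attack movement.
; A ComboWindowEnd gameplay event removes the HeavyComboOpen tag, stops that movement and ends the ability.
; Montage completion, interruption or cancellation also ends it, and OnEndAbility clears the tag again as cleanup.
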(event Ability|EventActivateAbility
  (Ability|CommitAbility)
  ;[0 0.06125 1] Heavy Attack 3
  (|PlayMontageandWaitProxy "None" "/Game/Animation/MC/Slash/AM_HSlash3.AM_HSlash3" 1.3 "None" true 1.0 0.0 false
    (:then
      (Class|BPIGAS|GASAddAtkMove(Message) (Ability|GetAvatarActorfromActorInfo) 1e+01)
      ;[0.06848 1 0] CleanUp
      (Ability|Tasks|WaitGameplayEvent "(TagName=\"Event.ComboWindowEnd\")" 0
        (:EventReceived
          (Ability|GameplayEffect|RemoveLooseGameplayTags (Ability|GetAvatarActorfromActorInfo) (Variables|Default|GetHeavyComboOpen))
          (Class|BPIGAS|GASStopAtkMove(Message) (Ability|GetAvatarActorfromActorInfo))
          (Ability|EndAbility))))
    (:OnCompleted
      (Ability|EndAbility :!label _label))
    (:OnInterrupted
      (goto _label))
    (:OnCancelled
      (goto _label))))

(event Ability|EventOnEndAbility
  (params (bWasCancelled :type Boolean))
  (Ability|GameplayEffect|RemoveLooseGameplayTags (Ability|GetAvatarActorfromActorInfo) (Variables|Default|GetHeavyComboOpen)))