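; Gameplay ability for the second light attack in the combo, playing a Megan montage sped up with an attack-movement message to the avatar.
; The ComboWindowOpen event swaps the LightComboOpen1 loose tag for LightComboOpen2.
; ComboWindowEnd removes that tag, stops attack movement and ends the ability, as does montage completion, interruption or cancellation.
; On end it clears LightComboOpen2 and resets the controller's IsAttack, unless flagged as interrupted.
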(event Ability|EventActivateAbility
  (bind _returnvalue (Ability|GetAvatarActorfromActorInfo))
  (Ability|CommitAbility)
  ;[0 0.9387 1] Light Attack 2
  (|PlayMontageandWaitProxy "None" "/Game/Characters/Megan/Anim/Attack/AM_LAttack2_Megan.AM_LAttack2_Megan" 1.4 "None" true 1.0 0.0 false
    (:then
      (Class|BPIGAS|GASAddAtkMove(Message) (Ability|GetAvatarActorfromActorInfo) 5.0)
      (Ability|Tasks|WaitGameplayEvent "(TagName=\"Event.ComboWindowOpen\")" 0
        (:then
          ;[0.06848 1 0] CleanUp
          (Ability|Tasks|WaitGameplayEvent "(TagName=\"Event.ComboWindowEnd\")" 0
            (:EventReceived
              (Ability|GameplayEffect|RemoveLooseGameplayTags (Ability|GetAvatarActorfromActorInfo) (Variables|Default|GetLightComboOpen2))
              (Class|BPIGAS|GASStopAtkMove(Message) (Ability|GetAvatarActorfromActorInfo))
              (Ability|EndAbility))))
        (:EventReceived
          (Ability|GameplayEffect|RemoveLooseGameplayTags _returnvalue (Variables|Default|GetLightComboOpen1))
          (Ability|GameplayEffect|AddLooseGameplayTags _returnvalue (Variables|Default|GetLightComboOpen2)))))
    (:OnCompleted
      (Ability|EndAbility :!label _label))
    (:OnInterrupted
      (Variables|Default|SetisInterrupt true)
      (goto _label))
    (:OnCancelled
      (goto _label))))

(event Ability|EventOnEndAbility
  (params (bWasCancelled :type Boolean))
  (Ability|GameplayEffect|RemoveLooseGameplayTags (Ability|GetAvatarActorfromActorInfo) (Variables|Default|GetLightComboOpen2))
  (if (not (Variables|Default|GetisInterrupt))
    (bind _mccontroller (Class|BPIGAS|GASGetMcControllerRef(Message) (Game|GetPlayerController 0)))
    (Variables|/Game/Blueprints/BP_MCController.BP_MCController_C|SetisAttack _mccontroller false)
    (Variables|Default|SetisInterrupt false)))