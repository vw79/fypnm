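; GA_LSlash3 is a Gameplay Ability for the third light slash attack.
; On activation it commits, plays the slash montage at increased rate and messages the avatar to add attack movement.
; A ComboWindowEnd gameplay event removes the LightComboOpen tag, stops attack movement and ends the ability.
; Montage completion, interruption or cancellation also ends it, and OnEndAbility clears the combo tag without stopping movement.
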(event Ability|EventActivateAbility
  (Ability|CommitAbility)
  ;[0 0.9387 1] Light Attack 3
  (|PlayMontageandWaitProxy "None" "/Game/Animation/MC/Slash/AM_Lslash3.AM_Lslash3" 1.5 "None" true 1.0 0.0 false
    (:then
      (Class|BPIGAS|GASAddAtkMove(Message) (Ability|GetAvatarActorfromActorInfo) 1e+01)
      ;[0.06848 1 0] CleanUp
      (Ability|Tasks|WaitGameplayEvent "(TagName=\"Event.ComboWindowEnd\")" 0
        (:EventReceived
          (Ability|GameplayEffect|RemoveLooseGameplayTags (Ability|GetAvatarActorfromActorInfo) (Variables|Default|GetLightComboOpen))
          (Class|BPIGAS|GASStopAtkMove(Message) (Ability|GetAvatarActorfromActorInfo))
          (Ability|EndAbility))))
    (:OnCompleted
      (Ability|EndAbility :!label _label))
    (:OnInterrupted
      (goto _label))
    (:OnCancelled
      (goto _label))))

(event Ability|EventOnEndAbility
  (params (bWasCancelled :type Boolean))
  (Ability|GameplayEffect|RemoveLooseGameplayTags (Ability|GetAvatarActorfromActorInfo) (Variables|Default|GetLightComboOpen)))