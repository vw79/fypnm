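; Gameplay Ability for the first light slash attack, which becomes a combo starter when the avatar has the Attack.Combo.Start tag.
; Each branch plays its montage and sends attack-movement messages to the avatar.
; Montage gameplay events open and close the combo window by toggling non-replicated loose tags for chain or light follow-ups.
; The window's close or the montage's finish ends the ability, which clears a reset tag.
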(event Ability|EventActivateAbility
  (Ability|CommitAbility)
  (bind _returnvalue (GameplayTags|HasMatchingGameplayTag(Message) (Ability|GetAbilitySystemComponent (Ability|GetAvatarActorfromActorInfo)) "(TagName=\"Attack.Combo.Start\")"))
  (if _returnvalue
    ;[0.3768 0 1] Combo Starter
    (|PlayMontageandWaitProxy "None" "/Game/Animation/MC/Slash/AM_ComboStart.AM_ComboStart" 1.0 "None" true 1.0 0.0 false
      (:then
        (Class|BPIGAS|GASAddAtkMove(Message) (Ability|GetAvatarActorfromActorInfo) 1e+01)
        (Ability|Tasks|WaitGameplayEvent "(TagName=\"Event.ComboWindowOpen\")" 0
          (:then
            ;[0.06848 1 0] CleanUp
            (Ability|Tasks|WaitGameplayEvent "(TagName=\"Event.ComboWindowEnd\")" 0
              (:EventReceived
                (Ability|GameplayEffect|RemoveLooseGameplayTags (Ability|GetAvatarActorfromActorInfo) (Variables|Default|GetChainComboOpen))
                (Class|BPIGAS|GASStopAtkMove(Message) (Ability|GetAvatarActorfromActorInfo))
                (Ability|EndAbility))))
          (:EventReceived
            (Ability|GameplayEffect|RemoveLooseGameplayTags (Ability|GetAvatarActorfromActorInfo) (Variables|Default|GetComboStarterTag))
            (Ability|GameplayEffect|AddLooseGameplayTags (Ability|GetAvatarActorfromActorInfo) (Variables|Default|GetChainComboOpen)))))
      (:OnCompleted
        (Ability|EndAbility :!label _label))
      (:OnCancelled
        (goto _label)))
    (else
      ;[0 0.9387 1] Light Attack 1
      (|PlayMontageandWaitProxy "None" "/Game/Animation/MC/Slash/AM_Lslash1.AM_Lslash1" 1.5 "None" true 1.0 0.0 false
        (:then
          (Class|BPIGAS|GASAddAtkMove(Message) (Ability|GetAvatarActorfromActorInfo) 5.0)
          (Ability|Tasks|WaitGameplayEvent "(TagName=\"Event.ComboWindowOpen\")" 0
            (:then
              ;[0.06848 1 0] CleanUp
              (Ability|Tasks|WaitGameplayEvent "(TagName=\"Event.ComboWindowEnd\")" 0
                (:EventReceived
                  (Ability|GameplayEffect|RemoveLooseGameplayTags (Ability|GetAvatarActorfromActorInfo) (Variables|Default|GetLightComboOpen))
                  (Class|BPIGAS|GASStopAtkMove(Message) (Ability|GetAvatarActorfromActorInfo))
                  (Ability|EndAbility))))
            (:EventReceived
              (Ability|GameplayEffect|AddLooseGameplayTags (Ability|GetAvatarActorfromActorInfo) (Variables|Default|GetLightComboOpen)))))
        (:OnCompleted
          (Ability|EndAbility :!label _label_2))
        (:OnInterrupted
          (goto _label_2))
        (:OnCancelled
          (goto _label_2))))))

(event Ability|EventOnEndAbility
  (params (bWasCancelled :type Boolean))
  (Ability|GameplayEffect|RemoveLooseGameplayTags (Ability|GetAvatarActorfromActorInfo) (Variables|Default|GetResetTag)))