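; GA_HSlash2 is a Gameplay Ability for the second heavy slash in a melee combo.
; It commits, plays the AM_HSlash2 montage slightly sped up and tells the avatar to add attack movement.
; Combo window gameplay events swap the HeavyComboOpen1 loose tag for HeavyComboOpen2, then remove it, stop the movement and end the ability.
; Montage completion or interruption also ends it, and OnEndAbility always clears HeavyComboOpen2.
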(event Ability|EventActivateAbility
  (bind _returnvalue (Ability|GetAvatarActorfromActorInfo))
  (Ability|CommitAbility)
  ;[0 0.06125 1] Heavy Attack 2
  (|PlayMontageandWaitProxy "None" "/Game/Animation/MC/Slash/AM_HSlash2.AM_HSlash2" 1.3 "None" true 1.0 0.0 false
    (:then
      (Class|BPIGAS|GASAddAtkMove(Message) (Ability|GetAvatarActorfromActorInfo) 5.0)
      (Ability|Tasks|WaitGameplayEvent "(TagName=\"Event.ComboWindowOpen\")" 0
        (:then
          ;[0.06848 1 0] CleanUp
          (Ability|Tasks|WaitGameplayEvent "(TagName=\"Event.ComboWindowEnd\")" 0
            (:EventReceived
              (Ability|GameplayEffect|RemoveLooseGameplayTags (Ability|GetAvatarActorfromActorInfo) (Variables|Default|GetHeavyComboOpen2))
              (Class|BPIGAS|GASStopAtkMove(Message) (Ability|GetAvatarActorfromActorInfo))
              (Ability|EndAbility))))
        (:EventReceived
          (Ability|GameplayEffect|RemoveLooseGameplayTags _returnvalue (Variables|Default|GetHeavyComboOpen1))
          (Ability|GameplayEffect|AddLooseGameplayTags _returnvalue (Variables|Default|GetHeavyComboOpen2)))))
    (:OnCompleted
      (Ability|EndAbility :!label _label))
    (:OnInterrupted
      (goto _label))
    (:OnCancelled
      (goto _label))))

(event Ability|EventOnEndAbility
  (params (bWasCancelled :type Boolean))
  (Ability|GameplayEffect|RemoveLooseGameplayTags (Ability|GetAvatarActorfromActorInfo) (Variables|Default|GetHeavyComboOpen2)))