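; GA_HSlash1 is a Gameplay Ability for the first heavy slash of a melee combo.
; It plays the slash montage with attack movement, first running an equip montage if the weapon is not equipped.
; Montage gameplay events open the combo window by adding starter and heavy-combo tags, then close it by removing the heavy tag, stopping movement and ending the ability.
; Ending the ability also clears a reset tag.
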(event Ability|EventActivateAbility
  (Ability|CommitAbility)
  (bind _mc (Class|BPIGAS|GASGetMcRef(Message) (Ability|GetAvatarActorfromActorInfo)))
  (if (Variables|/Game/Blueprints/BP_Weapon.BP_Weapon_C|GetisEquip (Variables|/Game/ThirdPerson/Blueprints/Player/BP_MC.BP_MC_C|GetWeaponRef _mc))
    _
    (else
      (|PlayMontageandWaitProxy "None" "/Game/Characters/Megan/Anim/Attack/Basic/AM_EquipMegan.AM_EquipMegan" 1.5 "None" true 1.0 0.0 false
        (:OnBlendOut
          (Default|EquipWeapon (Variables|/Game/ThirdPerson/Blueprints/Player/BP_MC.BP_MC_C|GetWeaponRef _mc))))))
  ;[0 0.06125 1] Heavy Attack 1
  (|PlayMontageandWaitProxy "None" "/Game/Animation/MC/Slash/AM_HSlash1.AM_HSlash1" 1.1 "None" true 1.0 0.0 false
    (:then
      (Class|BPIGAS|GASAddAtkMove(Message) (Ability|GetAvatarActorfromActorInfo) 1e+01)
      (Ability|Tasks|WaitGameplayEvent "(TagName=\"Event.ComboWindowOpen\")" 0
        (:then
          ;[0.06848 1 0] CleanUp
          (Ability|Tasks|WaitGameplayEvent "(TagName=\"Event.ComboWindowEnd\")" 0
            (:EventReceived
              (Ability|GameplayEffect|RemoveLooseGameplayTags (Ability|GetAvatarActorfromActorInfo) (Variables|Default|GetHeavyComboOpen))
              (Class|BPIGAS|GASStopAtkMove(Message) (Ability|GetAvatarActorfromActorInfo))
              (Ability|EndAbility))))
        (:EventReceived
          (bind _returnvalue (GameplayTags|HasMatchingGameplayTag(Message) (Ability|GetAbilitySystemComponent (Ability|GetAvatarActorfromActorInfo)) "(TagName=\"Attack.Combo.Start\")"))
          (if _returnvalue
            (Ability|GameplayEffect|RemoveLooseGameplayTags (Ability|GetAvatarActorfromActorInfo) (Variables|Default|GetComboStarterTag)))
          (Ability|GameplayEffect|AddLooseGameplayTags (Ability|GetAvatarActorfromActorInfo) (Variables|Default|GetComboStarterTag))
          (Ability|GameplayEffect|AddLooseGameplayTags (Ability|GetAvatarActorfromActorInfo) (Variables|Default|GetHeavyComboOpen)))))
    (:OnCompleted
      (Ability|EndAbility :!label _label))
    (:OnInterrupted
      (goto _label))
    (:OnCancelled
      (goto _label))))

(event Ability|EventOnEndAbility
  (params (bWasCancelled :type Boolean))
  (Ability|GameplayEffect|RemoveLooseGameplayTags (Ability|GetAvatarActorfromActorInfo) (Variables|Default|GetResetTag)))