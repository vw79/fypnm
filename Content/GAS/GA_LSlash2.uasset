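; Gameplay Ability for the second light slash in a combo.
; On activation it commits, plays the slash montage at double speed and starts attack movement on the avatar.
; The combo-window open event swaps loose tag ComboOpen1 for ComboOpen2 and messages the player controller to save the light attack.
; The window end event clears ComboOpen2, resets attack state, stops movement and ends the ability; montage completion only ends it.
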(event Ability|EventActivateAbility
  (bind _returnvalue (Ability|GetAvatarActorfromActorInfo))
  (bind _returnvalue_2 (Game|GetPlayerController 0))
  (Ability|CommitAbility)
  (|PlayMontageandWaitProxy "None" "/Game/VW/Slash/AM_Lslash2.AM_Lslash2" 2.0 "None" true 1.0 0.0 false
    (:then
      (Class|BPIGAS|AddAtkMove(Message) (Ability|GetAvatarActorfromActorInfo) 2.0)
      (Ability|Tasks|WaitGameplayEvent "(TagName=\"Event.ComboWindowOpen\")" 0
        (:then
          (Ability|Tasks|WaitGameplayEvent "(TagName=\"Event.ComboWindowEnd\")" 0
            (:EventReceived
              (Ability|GameplayEffect|RemoveLooseGameplayTags (Ability|GetAvatarActorfromActorInfo) (Variables|Default|GetComboOpen2))
              (Class|BPIInputBuffer|IBResetAttackState(Message) _returnvalue_2)
              (Class|BPIGAS|StopAtkMove(Message) (Ability|GetAvatarActorfromActorInfo))
              (Ability|EndAbility))))
        (:EventReceived
          (Ability|GameplayEffect|RemoveLooseGameplayTags _returnvalue (Variables|Default|GetComboOpen1))
          (Ability|GameplayEffect|AddLooseGameplayTags _returnvalue (Variables|Default|GetComboOpen2))
          (Class|BPIInputBuffer|IBSaveLightAttack(Message) _returnvalue_2))))
    (:OnCompleted
      (Ability|EndAbility))))