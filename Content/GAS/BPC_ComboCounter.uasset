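; Combo counter component that tracks hit count, move variety, a score multiplier and a style rank.
; RegisterCombo maps the owner's GAS tags to attack categories via DT_ParentTag, rewarding categories absent from a short recent-move list.
; The multiplier combines hits, variety and exponential time falloff, selecting rank by threshold and playing rank-change sounds.
; After a timeout, looping decay applies per-rank penalties and updates the HUD until reset; DropRank demotes one rank.
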(event Custom|DropRank
  (CallFunction|StartDecayTimer)
  (if (Utilities|Enum|Equal(Enum) (Variables|Result|GetRank) "NewEnumerator0")
    (CallFunction|StopDecayTimer)
    (CallFunction|ResetCounter)
    (elif (.ReturnValue (Utilities|Map|Find (Variables|Default|GetCountPenalty) (Variables|Result|GetRank)))
      (Variables|Result|SetCurrentHitCount (Math|Float|Round (- (* (Variables|Result|GetCurrentHitCount) (- 1 (.Value (Utilities|Map|Find (Variables|Default|GetCountPenalty) (Variables|Result|GetRank))))) (.Value (Utilities|Map|Find (Variables|Default|GetFixedReduction) (Variables|Result|GetRank))))))
      (bind _keys (Utilities|Map|Keys (Variables|Default|GetReComboThresholds)))
      (Class|KismetArrayLibrary|SortByteArray _keys)
      (bind (_array_element _array_index) (Utilities|Array|ForEachLoopwithBreak _keys :!label _label)
        (:LoopBody
          (if (Utilities|Enum|Equal(Enum) _array_element (Variables|Result|GetRank))
            (Variables|Result|SetRank (Utilities|Array|Get(acopy) _keys (- _array_index 1)))
            (goto _label Break)))
        (:Completed
          (Variables|Result|SetComboMultiplier (- (Variables|Result|GetComboMultiplier) (* 0.3 (.Value (Utilities|Map|Find (Variables|Default|GetReComboThresholds) (Variables|Result|GetRank))))))
          (CallFunction|UpdateComboUI))))))

(event Custom|StopDecayTimer
  (Utilities|Time|ClearandInvalidateTimerbyHandle (stale Custom|StartDecayTimer _returnvalue)))

(event Custom|DecayTimer
  (if (> (Variables|Result|GetComboMultiplier) 1.0)
    (Utilities|Array|Clear (Variables|Style|GetUniqueTag))
    (Variables|Style|SetUniqueMove (Math|Integer|Max(Integer) (Math|Float|Round (* (Variables|Style|GetUniqueMove) (Class|KismetMathLibrary|Exp (* (.Value (Utilities|Map|Find (Variables|Default|GetCountPenalty) (Variables|Result|GetRank))) -1.0))))))
    (Variables|Result|SetCurrentHitCount (Math|Float|Round (* (Variables|Result|GetCurrentHitCount) (Class|KismetMathLibrary|Exp (* (.Value (Utilities|Map|Find (Variables|Default|GetCountPenalty) (Variables|Result|GetRank))) -1.0)))))
    (CallFunction|UpdateMultiplier)
    (if (< (Variables|Result|GetComboMultiplier) 1.0)
      (Variables|Result|SetComboMultiplier 1.0))
    (bind _rank (CallFunction|GetClosestRank (Variables|Default|GetComboThresholds)))
    (Variables|Result|SetRank _rank)
    (CallFunction|UpdateComboUI)
    (else
      (CallFunction|ResetCounter)
      (CallFunction|StopDecayTimer))))

(event Custom|StartDecayTimer
  (CallFunction|StopDecayTimer)
  (Utilities|FlowControl|Delay (Variables|Timeout|GetTimeout))
  (bind _returnvalue (Utilities|Time|SetTimerbyEvent (delegate Custom|DecayTimer) 1.0 true)))

(event EventBeginPlay
  (bind (_mc _gas) (Class|BPIGAS|GASGetMcRef(Message) (Components|GetOwner)))
  (Variables|Ref|SetMcRef _mc)
  (Variables|Ref|SetGasRef _gas)
  (bind (_mccontroller _hud) (Class|BPIGAS|GASGetMcControllerRef(Message) (Game|GetPlayerController 0)))
  (Variables|Ref|SetMcControllerRef _mccontroller)
  (Variables|Ref|SetHUDRef _hud)
  (bind _outrownames (DataTable|GetDataTableRowNames "/Game/GAS/DT_ParentTag.DT_ParentTag"))
  (for _array_element _outrownames
    (bind _returnvalue (Utilities|GetDataTableRow "/Game/GAS/DT_ParentTag.DT_ParentTag" _array_element)
      (:then
        (Utilities|Map|Add (Variables|Style|GetParentTag) (.GasTag (Utilities|Struct|BreakParentTag _returnvalue)) (.ParentTag (Utilities|Struct|BreakParentTag _returnvalue)))))))

(fn RegisterCombo
  (bind _uniquetag (Variables|Style|GetUniqueTag))
  (Variables|Style|SetCurrentTag "")
  (bind _array_element (Utilities|Array|ForEachLoopwithBreak (GameplayTags|BreakGameplayTagContainer (GameplayTags|GetOwnedGameplayTags (Variables|Ref|GetGasRef) :!class /Script/GameplayTags.GameplayTagAssetInterface)) :!label _label)
    (:LoopBody
      (bind _parenttag (CallFunction|GetAttackCategory _array_element))
      (if (== _parenttag "")
        (Development|PrintString "no con tag")
        (else
          (Variables|Style|SetCurrentTag _parenttag)
          (goto _label Break))))
    (:Completed
      (Math|Integer|IncrementInt (Variables|Result|GetCurrentHitCount)
        (:%20%20
          (if (Utilities|Array|ContainsItem (Variables|Style|GetUniqueTag) (Variables|Style|GetCurrentTag))
            _
            (else
              (Utilities|Array|Add _uniquetag (Variables|Style|GetCurrentTag))
              (Math|Integer|IncrementInt (Variables|Style|GetUniqueMove)
                (:%20%20
                  (if (> (Utilities|Array|Length _uniquetag) 3)
                    (Utilities|Array|RemoveIndex (Variables|Style|GetUniqueTag)))))))
          (CallFunction|UpdateMultiplier)
          (bind _rank (CallFunction|GetClosestRank (Variables|Default|GetComboThresholds)))
          (bind _output_get (Variables|Result|SetRank _rank))
          (if (Utilities|Enum|NotEqual(Enum) _output_get (Variables|SFX|GetPreviousRank))
            (Audio|PlaySound2D (.Value (Utilities|Map|Find (Variables|SFX|GetComboSounds) _output_get)) 1.0 1.0 0.0 0 0)
            (Variables|SFX|SetPreviousRank _output_get))
          (CallFunction|StartDecayTimer)
          (return (Variables|Result|GetCurrentHitCount) (Variables|Result|GetRank) (Variables|Result|GetComboMultiplier)))))))

(fn GetClosestRank
  (params (TargetMap :type Map%20of%20Floats%20%28double-precision%29%20to%20Bytes))
  (LocalVariables|SetClosestThreshold 0.0)
  (bind _keys (Utilities|Map|Keys TargetMap))
  (Class|KismetArrayLibrary|SortFloatArray _keys false "Descending")
  (bind _array_element (Utilities|Array|ForEachLoopwithBreak _keys :!label _label)
    (:LoopBody
      (if (<= _array_element (Variables|Result|GetComboMultiplier))
        (LocalVariables|SetClosestThreshold _array_element)
        (goto _label Break)))
    (:Completed
      (if (.ReturnValue (Utilities|Map|Find TargetMap (LocalVariables|GetClosestThreshold)))
        (return (.Value (Utilities|Map|Find TargetMap (LocalVariables|GetClosestThreshold))))))))

(fn ResetCounter
  (Default|HideCombo (Variables|Ref|GetHUDRef))
  (Variables|Result|SetCurrentHitCount 0)
  (Variables|Result|SetComboMultiplier 1.0)
  (Variables|Result|SetRank "NewEnumerator0"))

(fn GetAttackCategory
  (params (GasTag :type Gameplay%20Tag%20Structure))
  (bind _parenttag (Variables|Style|GetParentTag))
  (bind (_value _returnvalue) (Utilities|Map|Find _parenttag GasTag))
  (if _returnvalue
    (return _value)
    (else
      (Development|PrintString "Unknown Tag Map"))))

(fn UpdateComboUI
  (Default|UpdateComboText (Variables|/Game/Widgets/AWB/AWB_HUD.AWB_HUD_C|GetCounterWidget (Variables|Ref|GetHUDRef)) (Variables|Result|GetCurrentHitCount) (Variables|Result|GetRank) (Variables|Result|GetComboMultiplier)))

(fn Roundto2DP
  (params (Float :type Float%20%28double-precision%29))
  (return (/ (Math|Float|Round (* Float 1e+02)) 100)))

(fn UpdateMultiplier
  (Variables|Result|SetComboMultiplier (CallFunction|Roundto2DP (* (* (+ 1.0 (* 0.05 (Variables|Result|GetCurrentHitCount))) (+ 1.0 (* 0.15 (Variables|Style|GetUniqueMove)))) (Class|KismetMathLibrary|Exp (* -0.05 (Variables|Style|GetTimeSinceLastHit)))))) ; M=(1 + 0.1𝑁) * (1 + 0.2𝑉) * e^-0.1𝑇\n\n𝑁 = Combo Count\n𝑉 = Unique Moves Used\n𝑇 = Seconds Since Last Hit Taken
)